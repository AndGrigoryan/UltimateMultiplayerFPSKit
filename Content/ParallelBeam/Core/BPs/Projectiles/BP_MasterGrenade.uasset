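; BP_MasterGrenade is a fused grenade projectile, named as a master Blueprint, that explodes after a set time.
; On BeginPlay only the authority starts the fuse timer, which calls Explode to apply full radial damage credited to the owner and instigator.
; Explode then calls ApplyEffect to spawn a pooled Niagara system, fed the impact position through an array parameter, plus a sound, before destroying the actor.
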(event `self.ReceiveBeginPlay`
  (`/Engine/EditorBlueprintResources/ActorMacros.Switch Has Authority`
    (:`Authority`
      (`KismetSystemLibrary.K2_SetTimerDelegate` (delegate `Explode`) (`self.FuseTime`)))))

(event `Explode`
  (bind _returnvalue (`self.K2_GetActorLocation`))
  (`GameplayStatics.ApplyRadialDamage` :`BaseDamage` (`self.Base Damage`) :`Origin` _returnvalue :`DamageRadius` (`self.Damage Radius`) :`DamageTypeClass` (`self.Damage Type Class`) :`DamageCauser` (`self.GetOwner`) :`InstigatedByController` (`self.GetInstigatorController`) :`bDoFullDamage` true)
  (`self.ApplyEffect` _returnvalue)
  (`self.K2_DestroyActor`))

(event `ApplyEffect`
  (params (Location :type "Vector Structure"))
  (bind _returnvalue (`NiagaraFunctionLibrary.SpawnSystemAtLocation` (`self.TriggerParticles`) Location (struct) (1.0 1.0 1.0) true true "AutoRelease"))
  (`GameplayStatics.SpawnSoundAtLocation` (`self.TriggerSound`) Location (struct) 1.0 1.0 0.0 null null)
  (`NiagaraDataInterfaceArrayFunctionLibrary.SetNiagaraArrayPosition` _returnvalue "User.ImpactPositions" (`|MakeArray` Location)))

(fn `UserConstructionScript`)