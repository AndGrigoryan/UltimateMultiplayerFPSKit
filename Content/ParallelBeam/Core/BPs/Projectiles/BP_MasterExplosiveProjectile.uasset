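; Base explosive projectile that detonates on every terminal hit, penetration and ricochet.
; Each of these events applies radial damage with falloff at the hit point, then spawns pooled Niagara and sound effects, passing the impact position to the particle system.
; BeginPlay randomly attaches a delayed trail effect.
; CalculateDamage scales weapon damage by bone, climbing parent bones before falling back to Base, but the explosion logic does not call it.
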(event `self.ReceiveBeginPlay`
  (if (`KismetMathLibrary.RandomBoolWithWeight` (`self.TrailChance`))
    (`KismetSystemLibrary.Delay` (`self.TrailDelay`))
    (`NiagaraFunctionLibrary.SpawnSystemAttached` (`self.TrailEffect`) (`self.Sphere`) "None" (0.0 0.0 0.0) (struct) "SnapToTarget" true true "AutoRelease")))

(event `self.OnProjectileTerminalHit`
  (params (InHitResult :type "HitResult Structure (by ref)"))
  (`self.ApplyDamage` InHitResult)
  (`self.HitEffects` InHitResult))

(event `self.OnProjectilePenetrated`
  (params (InVelocity :type "Vector Structure (by ref)") (InEntryHitResult :type "HitResult Structure (by ref)") (InPenetrationResult :type "AGR_PenetrationResult Structure (by ref)"))
  (`self.ApplyDamage` InEntryHitResult)
  (`self.HitEffects` InEntryHitResult))

(event `self.OnProjectileRicocheted`
  (params (InVelocity :type "Vector Structure (by ref)") (InHitResult :type "HitResult Structure (by ref)") (InBounces :type Integer) (InRicochetResult :type "AGR_RicochetResult Structure (by ref)") (InHitTransform :type "Transform Structure (by ref)") (InBounceTransform :type "Transform Structure (by ref)"))
  (`self.ApplyDamage` InHitResult)
  (`self.HitEffects` InHitResult))

(event `HitEffects`
  (params (Hit :type "HitResult Structure (by ref)"))
  (`self.ApplyEffect` (`.Location` (`GameplayStatics.BreakHitResult` Hit))))

(event `ApplyDamage`
  (params (HitResult :type "HitResult Structure"))
  (`GameplayStatics.ApplyRadialDamageWithFalloff` :`BaseDamage` 500.0 :`MinimumDamage` 50.0 :`Origin` (`.Location` (`GameplayStatics.BreakHitResult` HitResult)) :`DamageInnerRadius` 100.0 :`DamageOuterRadius` 200.0 :`DamageTypeClass` (`self.Damage Type Class`) :`DamageCauser` (`self.GetOwner`) :`InstigatedByController` (`self.GetInstigatorController`)))

(event `ApplyEffect`
  (params (Location :type "Vector Structure"))
  (bind _returnvalue (`NiagaraFunctionLibrary.SpawnSystemAtLocation` (`self.TriggerParticles`) Location (struct) (1.0 1.0 1.0) true true "AutoRelease"))
  (`GameplayStatics.SpawnSoundAtLocation` (`self.TriggerSound`) Location (struct) 1.0 1.0 0.0 null null)
  (`NiagaraDataInterfaceArrayFunctionLibrary.SetNiagaraArrayPosition` _returnvalue "User.ImpactPositions" (`|MakeArray` Location)))

(fn `CalculateDamage`
  (params (BoneName :type "Name (by ref)") (HitComponent :type "PrimitiveComponent Object Reference"))
  (returns (ReturnValue :type "Float (double-precision)"))
  (locals (Loc_bone :type Name))
  (bind (_value _returnvalue) (`BlueprintMapLibrary.Map_Find` (`self.DamageValues`) (`local.Loc_bone`)))
  (bind _asskeletal_mesh_component (cast `SkeletalMeshComponent` HitComponent)
    (:`then`
      (`|ExecutionSequence`
        (:`then_0`
          (set `local.Loc_bone` BoneName)
          (if _returnvalue :!label _label
            (return (* _value (`self.WeaponDamage`)))
            (else
              (set `local.Loc_bone` (`SkinnedMeshComponent.GetParentBone` _asskeletal_mesh_component (`local.Loc_bone`)))
              (`/Engine/EditorBlueprintResources/StandardMacros.Do N` 5
                (:`Exit`
                  (goto _label))))))
        (:`then_1`
          _)))
    (:`CastFailed`
      _))
  (return (* (`BlueprintMapLibrary.Map_Find` (`self.DamageValues`) "Base") (`self.WeaponDamage`))))

(fn `UserConstructionScript`)