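; Base projectile that applies point damage and requests surface-based impact effects from its owner on terminal hits, penetrations and ricochets.
; Damage comes from the owner's MSK projectile launcher component using the hit bone and component.
; A weighted random roll spawns a delayed, pooled trail that is manually released on destruction.
; Its own CalculateDamage, uncalled here, climbs parent bones a few times for a multiplier, falling back to "Base".
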(event `self.ReceiveDestroyed`
  (bind _trail (`self.Trail`)
    (:`then`
      (`FXSystemComponent.ReleaseToPool` _trail)
      (`ActorComponent.K2_DestroyComponent` _trail))
    (:`else`)))

(event `self.ReceiveBeginPlay`
  (if (`KismetMathLibrary.RandomBoolWithWeight` (`self.TrailChance`))
    (`KismetSystemLibrary.Delay` (`self.TrailDelay`))
    (bind _returnvalue (`NiagaraFunctionLibrary.SpawnSystemAttached` (`self.TrailEffect`) (`self.Sphere`) "None" (0.0 0.0 0.0) (struct) "SnapToTarget" true true "ManualRelease"))
    (set `self.Trail` _returnvalue)))

(event `self.OnProjectileTerminalHit`
  (params (InHitResult :type "HitResult Structure (by ref)"))
  (`self.ApplyDamage` InHitResult)
  (`self.HitEffects` InHitResult))

(event `self.OnProjectilePenetrated`
  (params (InVelocity :type "Vector Structure (by ref)") (InEntryHitResult :type "HitResult Structure (by ref)") (InPenetrationResult :type "AGR_PenetrationResult Structure (by ref)"))
  (`self.ApplyDamage` InEntryHitResult)
  (`self.HitEffects` InEntryHitResult))

(event `self.OnProjectileRicocheted`
  (params (InVelocity :type "Vector Structure (by ref)") (InHitResult :type "HitResult Structure (by ref)") (InBounces :type Integer) (InRicochetResult :type "AGR_RicochetResult Structure (by ref)") (InHitTransform :type "Transform Structure (by ref)") (InBounceTransform :type "Transform Structure (by ref)"))
  (`self.ApplyDamage` InHitResult)
  (`self.HitEffects` InHitResult))

(event `HitEffects`
  (params (Hit :type "HitResult Structure (by ref)"))
  (bind (_bblockinghit _binitialoverlap _time _distance _location _impactpoint _normal _impactnormal _physmat) (`GameplayStatics.BreakHitResult` Hit))
  (bind _returnvalue (`self.GetOwner`))
  (`/Engine/EditorBlueprintResources/StandardMacros.IsValid` _returnvalue
    (:`Is Valid`
      (message `/Game/ParallelBeam/Core/BPs/Interfaces/BPI_Weapon.SpawnHitEffect` _returnvalue _location _impactnormal (`PhysicalMaterial.SurfaceType` _physmat)))))

(event `ApplyDamage`
  (params (HitResult :type "HitResult Structure"))
  (bind (_bblockinghit _binitialoverlap _time _distance _location _impactpoint _normal _impactnormal _physmat _hitactor _hitcomponent _hitbonename) (`GameplayStatics.BreakHitResult` HitResult))
  (bind _returnvalue (`/Game/ParallelBeam/Core/BPs/Components/BP_MSK_ProjectileLauncher.CalculateDamage` (`/Game/ParallelBeam/Core/BPs/FunctionLib/BFL_MSK.GetMSKProjectileLauncherComponent` (`self.GetOwner`)) _hitbonename _hitcomponent))
  (`GameplayStatics.ApplyPointDamage` _hitactor _returnvalue _impactnormal HitResult (`self.GetInstigatorController`) (`self.GetOwner`) (`self.Damage Type Class`)))

(fn `CalculateDamage`
  (params (BoneName :type "Name (by ref)") (HitComponent :type "PrimitiveComponent Object Reference"))
  (returns (ReturnValue :type "Float (double-precision)"))
  (locals (Loc_bone :type Name))
  (bind (_value _returnvalue) (`BlueprintMapLibrary.Map_Find` (`self.DamageValues`) (`local.Loc_bone`)))
  (bind _asskeletal_mesh_component (cast `SkeletalMeshComponent` HitComponent)
    (:`then`
      (`|ExecutionSequence`
        (:`then_0`
          (set `local.Loc_bone` BoneName)
          (if _returnvalue :!label _label
            (return (* _value (`self.WeaponDamage`)))
            (else
              (set `local.Loc_bone` (`SkinnedMeshComponent.GetParentBone` _asskeletal_mesh_component (`local.Loc_bone`)))
              (`/Engine/EditorBlueprintResources/StandardMacros.Do N` 5
                (:`Exit`
                  (goto _label))))))
        (:`then_1`
          _)))
    (:`CastFailed`
      _))
  (return (* (`BlueprintMapLibrary.Map_Find` (`self.DamageValues`) "Base") (`self.WeaponDamage`))))

(fn `UserConstructionScript`)