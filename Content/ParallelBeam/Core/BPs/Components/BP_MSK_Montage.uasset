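; Component that plays and ends replicated action montages on its owner and the weapon actor.
; Calls run locally, then optionally relay through server to multicast, normally skipping the locally controlled client unless forced or server-initiated.
; Montages come from the weapon interface or default data, using dual-wield state and modifier-scaled speed.
; Playback targets arm-specific linked anim graphs, falling back to the main instance; vaults add RootMesh, and ending routes to "End" sections.
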(event `PlayMontage`
  (params (SelfOnly :type Boolean) (ForcePlayOnOwner :type Boolean) (Actor :type "Actor Object Reference") (Action :type "GameplayTag Structure"))
  ;[0 0 0] Montages
  ;;[1 1 1] Play Montage
  (if (not SelfOnly)
    (`self.SVR_PlayMontage` Actor Action ForcePlayOnOwner))
  (`self.Montage` Action Actor))

(event `SVR_PlayMontage`
  (params (Actor :type "Actor Object Reference") (Action :type "GameplayTag Structure") (ForcePlayOnOwner :type Boolean))
  ;[0 0 0] Montages
  ;;[1 1 1] Play Montage
  (`self.MLT_PlayMontage` Actor Action ForcePlayOnOwner))

(event `MLT_PlayMontage`
  (params (Actor :type "Actor Object Reference") (Action :type "GameplayTag Structure") (ForcePlayOnOwner :type Boolean))
  ;[0 0 0] Montages
  ;;[1 1 1] Play Montage
  (if ForcePlayOnOwner
    (`self.Montage` Action Actor :!label _label)
    (elif (not (`Pawn.IsLocallyControlled` (`Actor.Instigator` (`self.GetOwner`))))
      (goto _label))))

(event `EndMontage`
  (params (SelfOnly :type Boolean) (Actor :type "Actor Object Reference"))
  ;[0 0 0] Montages
  ;;[1 1 1] End Montage
  (if (not SelfOnly)
    (`self.SVR_EndMontage` (`KismetSystemLibrary.IsServer`) Actor))
  (`self.End Montage` Actor))

(event `SVR_EndMontage`
  (params (CalledByServer :type Boolean) (Actor :type "Actor Object Reference"))
  ;[0 0 0] Montages
  ;;[1 1 1] End Montage
  (`self.MLT_EndMontage` CalledByServer Actor))

(event `MLT_EndMontage`
  (params (CalledByServer :type Boolean) (Actor :type "Actor Object Reference"))
  ;[0 0 0] Montages
  ;;[1 1 1] End Montage
  (if (`Pawn.IsLocallyControlled` (`Actor.Instigator` (`self.GetOwner`)))
    (if CalledByServer
      (`self.End Montage` Actor :!label _label_2))
    (else
      (goto _label_2))))

(fn `End Montage`
  (params (Actor :type "Actor Object Reference"))
  (locals (Loc_AnimGraphTag :type Name))
  (bind _actor (`local.Actor`))
  (bind _output (`|GetArrayItem` (`Actor.GetComponentsByTag` (`self.GetOwner`) "/Script/Engine.SkeletalMeshComponent" "MainMesh")))
  (bind _output_2 (`|GetArrayItem` (`Actor.GetComponentsByTag` (`local.Actor`) "/Script/Engine.SkeletalMeshComponent" "MainMesh")))
  (bind _returnvalue (`SkeletalMeshComponent.GetAnimInstance` _output_2))
  (bind _returnvalue_2 (`AnimInstance.GetCurrentActiveMontage` _returnvalue))
  (bind _returnvalue_3 (`AnimInstance.GetLinkedAnimGraphInstanceByTag` (`SkeletalMeshComponent.GetLinkedAnimGraphInstanceByTag` _output "Weapon") (`local.Loc_AnimGraphTag`)))
  (bind _returnvalue_4 (select `bool` (`KismetSystemLibrary.IsValid` _returnvalue_3) :`false` (`SkeletalMeshComponent.GetAnimInstance` _output) :`true` _returnvalue_3))
  (bind _returnvalue_5 (`AnimInstance.GetCurrentActiveMontage` _returnvalue_4))
  (`|ExecutionSequence`
    (:`then_0`
      (if (`KismetSystemLibrary.DoesImplementInterface` Actor "/Game/ParallelBeam/Core/BPs/Interfaces/BPI_Weapon.BPI_Weapon_C")
        (bind _return_value (message `/Game/ParallelBeam/Core/BPs/Interfaces/BPI_Weapon.GetIsOnWeaponLayer` _actor))
        (if _return_value
          (bind _return_value_2 (message `/Game/ParallelBeam/Core/BPs/Interfaces/BPI_Weapon.GetIsRightHanded` _actor))
          (if _return_value_2
            (set `local.Loc_AnimGraphTag` "RightArm")
            (else
              (set `local.Loc_AnimGraphTag` "LeftArm"))))))
    (:`then_1`
      (if (== (`AnimInstance.Montage_GetCurrentSection` _returnvalue_4 _returnvalue_5) "Loop")
        (`AnimInstance.Montage_JumpToSection` _returnvalue_4 "End" _returnvalue_5)
        (else
          (`AnimInstance.Montage_SetNextSection` _returnvalue_4 "Start" "End" _returnvalue_5)))
      (`/Engine/EditorBlueprintResources/StandardMacros.IsValid` _output_2
        (:`Is Valid`
          (if (== (`AnimInstance.Montage_GetCurrentSection` _returnvalue _returnvalue_2) "Loop")
            (`AnimInstance.Montage_JumpToSection` _returnvalue "End" _returnvalue_2)
            (else
              (`AnimInstance.Montage_SetNextSection` _returnvalue "Start" "End" _returnvalue_2))))))))

(fn `Montage`
  (params (Action :type "GameplayTag Structure") (Actor :type "Actor Object Reference"))
  (locals (LOC_AnimData :type "/Game/ParallelBeam/Core/BPs/Data/DTA_WeaponAnimation Object Reference" :default null) (Loc_AnimGraphTag :type Name :default "None") (LOC_CharacterMontage :type "AnimMontage Object Reference") (LOC_WeaponMontage :type "AnimMontage Object Reference") (Loc_IsDuelWelding :type Boolean :default false) (Loc_MontageSpeed :type "Float (single-precision)" :default 1.0))
  (bind _actor (`local.Actor`))
  (bind _loc_montagespeed (`local.Loc_MontageSpeed`))
  (bind (_character _weapon) (`/Game/ParallelBeam/Core/BPs/Data/DTA_WeaponAnimation.GetActionMontage` (`local.LOC_AnimData`) (`local.Action`) (`local.Loc_IsDuelWelding`)))
  (bind _return_value (`/Game/ParallelBeam/Core/BPs/FunctionLib/BFL_MSK.GetMSKLocomotionComponent` (`self.GetOwner`)))
  (bind (_found_value _floatvalue) (`/Game/ParallelBeam/Core/BPs/Components/BP_MSK_Locomotion.Get Action Modifier Value` _return_value (`local.Action`)))
  (bind _returnvalue (+ _floatvalue 1.0))
  (`|ExecutionSequence`
    (:`then_0`
      (`/Engine/EditorBlueprintResources/StandardMacros.IsValid` _return_value
        (:`Is Valid`
          (if _found_value
            (if (!= _returnvalue 0.0)
              (set `local.Loc_MontageSpeed` (`KismetMathLibrary.Abs` _returnvalue))
              (set `local.Loc_IsDuelWelding` (`/Game/ParallelBeam/Core/BPs/Components/BP_MSK_Locomotion.IsDuelWelding` _return_value)))))))
    (:`then_1`
      (if (`KismetSystemLibrary.DoesImplementInterface` (`local.Actor`) "/Game/ParallelBeam/Core/BPs/Interfaces/BPI_Weapon.BPI_Weapon_C")
        (bind _return_value_2 (message `/Game/ParallelBeam/Core/BPs/Interfaces/BPI_Weapon.GetIsOnWeaponLayer` _actor))
        (if _return_value_2
          (bind _return_value_3 (message `/Game/ParallelBeam/Core/BPs/Interfaces/BPI_Weapon.GetIsRightHanded` _actor))
          (if _return_value_3
            (set `local.Loc_AnimGraphTag` "RightArm")
            (else
              (set `local.Loc_AnimGraphTag` "LeftArm"))))
        (bind (_character_2 _weapon_2) (message `/Game/ParallelBeam/Core/BPs/Interfaces/BPI_Weapon.GetActionMontage` (`local.Actor`) (`local.Action`) (`local.Loc_IsDuelWelding`)))
        (set `local.LOC_CharacterMontage` _character_2)
        (set `local.LOC_WeaponMontage` _weapon_2)
        (else
          (set `local.LOC_AnimData` (`self.DefaultCharacterAnimationData`))
          (set `local.LOC_CharacterMontage` _character)
          (set `local.LOC_WeaponMontage` _weapon))))
    (:`then_2`
      (for _array_element (select `bool` (`BlueprintGameplayTagLibrary.MatchesAnyTags` Action (`BlueprintGameplayTagLibrary.MakeLiteralGameplayTagContainer` (struct :`GameplayTags` (struct :`(TagName` "Actions.Vault") :`(TagName` "Actions.Ladder"))))) :`false` (`|MakeArray` "MainMesh" :!type "Name") :`true` (`|MakeArray` "MainMesh" "RootMesh" :!type "Name"))
        (bind _output (`|GetArrayItem` (`Actor.GetComponentsByTag` (`self.GetOwner`) "/Script/Engine.SkeletalMeshComponent" _array_element)))
        (`/Engine/EditorBlueprintResources/StandardMacros.IsValid` _output
          (:`Is Valid`
            (bind _returnvalue_2 (`SkeletalMeshComponent.GetLinkedAnimGraphInstanceByTag` _output "Weapon"))
            (`/Engine/EditorBlueprintResources/StandardMacros.IsValid` _returnvalue_2
              (:`Is Valid`
                (bind _returnvalue_3 (`AnimInstance.GetLinkedAnimGraphInstanceByTag` _returnvalue_2 (`local.Loc_AnimGraphTag`)))
                (`/Engine/EditorBlueprintResources/StandardMacros.IsValid` _returnvalue_3
                  (:`Is Valid`
                    (`AnimInstance.Montage_Play` _returnvalue_3 (`local.LOC_CharacterMontage`) _loc_montagespeed "Duration" 0.0 true)
                    (bind _actor_2 (`local.Actor`)
                      (:`then`
                        (bind _returnvalue_4 (`SkeletalMeshComponent.GetAnimInstance` (`|GetArrayItem` (`Actor.GetComponentsByTag` _actor_2 "/Script/Engine.SkeletalMeshComponent" "MainMesh"))))
                        (`/Engine/EditorBlueprintResources/StandardMacros.IsValid` _returnvalue_4
                          (:`Is Valid`
                            (`AnimInstance.Montage_Play` _returnvalue_4 (`local.LOC_WeaponMontage`) (`local.Loc_MontageSpeed`) "Duration" 0.0 true))))
                      (:`else`)))
                  (:`Is Not Valid`
                    (`AnimInstance.Montage_Play` (`SkeletalMeshComponent.GetAnimInstance` _output) (`local.LOC_CharacterMontage`) _loc_montagespeed "MontageLength" 0.0 true :!label _label))))
              (:`Is Not Valid`
                (goto _label)))))))))