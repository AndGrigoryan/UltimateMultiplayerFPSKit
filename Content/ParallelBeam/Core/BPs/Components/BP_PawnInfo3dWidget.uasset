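; BP_PawnInfo3dWidget is a widget component that briefly shows a WB_PawnInfo widget for its owning pawn.
; The widget starts collapsed, and each Show call makes it visible and restarts a half-second retriggerable delay that collapses it again.
; A DoOnce passes the pawn to UpdatePlayerState only on the first Show of each visible period, resetting when the widget hides.
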(event `self.ReceiveBeginPlay`
  (`Widget.SetVisibility` (`self.GetWidget`) "Collapsed"))

(event `Show`
  (bind _returnvalue (`self.GetWidget`))
  (`|ExecutionSequence`
    (:`then_0`
      (`Widget.SetVisibility` _returnvalue "Visible")
      (`KismetSystemLibrary.RetriggerableDelay` 0.5)
      (`Widget.SetVisibility` _returnvalue "Collapsed")
      (goto _label :!via `Reset`))
    (:`then_1`
      (`/Engine/EditorBlueprintResources/StandardMacros.DoOnce` false :!label _label
        (:`Completed`
          (bind _aspawn (cast `Pawn` (`self.GetOwner`)))
          (bind _aswb_pawn_info (cast `/Game/ParallelBeam/Core/Widgets/Game/Elements/WB_PawnInfo` (`self.GetWidget`)))
          (`/Game/ParallelBeam/Core/Widgets/Game/Elements/WB_PawnInfo.UpdatePlayerState` _aswb_pawn_info _aspawn))))))