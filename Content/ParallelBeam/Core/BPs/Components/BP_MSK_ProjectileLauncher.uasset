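; Weapon launcher component that fires semi-auto, full-auto and burst shots, with ammo use, curve-driven recoil, muzzle, shell, audio and impact effects.
; Replicates only firing start/stop, so each machine runs its own shot timer and effects.
; Shots use penetrating line traces weakened by material strength, falling back to physical projectiles on a miss or without trace range.
; Clients predict hit effects, while the server re-traces reported hits before applying bone-based damage.
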(event `self.ReceiveBeginPlay`
  (bind _returnvalue (`self.GetOwner`))
  (set `self.SkeletalMesh` (`|GetArrayItem` (`Actor.GetComponentsByTag` _returnvalue "/Script/Engine.SkeletalMeshComponent" "MainMesh")))
  (set `self.Audio` (`|GetArrayItem` (`Actor.GetComponentsByTag` _returnvalue "/Script/Engine.AudioComponent" "MainAudio")))
  (bind _dt_animation (message `/Game/ParallelBeam/Core/BPs/Interfaces/BPI_Weapon.GetAnimationData` (`self.GetOwner`)))
  (`/Engine/EditorBlueprintResources/StandardMacros.IsValid` _dt_animation
    (:`Is Valid`
      (set `self.DT_Anims` _dt_animation))
    (:`Is Not Valid`
      _))
  (bind _ammotype (`self.AmmoType`)
    (:`then`
      (set `self.AmmoType` _ammotype))
    (:`else`)))

(event `AttemptFire`
  (params (Trigger :type Boolean))
  ;[0 0 0] shooting attempt
  (`self.CLT_StartFiring` Trigger))

(event `MLT_HitEffects`
  (params (Location :type "Vector Structure") (`Impact Normals` :type "Vector Structure") (SurfaceType :type "EPhysicalSurface Enum" :default "SurfaceType_Default"))
  ;[0 0 0] Spawn and activate Weapon Impact system
  (if (not (`self.IsLocalPlayer`))
    (`self.HitEffect` Location `Impact Normals` SurfaceType)))

(event `StartFiring`
  (params (Start :type Boolean))
  (bind _returnvalue (`self.GetFireMode`))
  ;[0 0 0] Actual part where we start the process of firing, checking if we can fire and then starting the firing sequence
  (bind _ownerpawn (`self.OwnerPawn`)
    (:`then`
      (set `self.IsLocalPlayer` (and (`Pawn.IsLocallyControlled` _ownerpawn) (`Pawn.IsPlayerControlled` _ownerpawn))))
    (:`else`
      _))
  (set `self.Effect_Ammo_Local` (`self.GetAmmoCount`))
  (if Start
    (if (`self.CanFire`)
      (`/Engine/EditorBlueprintResources/StandardMacros.DoOnce` false :!label _label
        (:`Completed`
          (switch `EAGR_FireMode` _returnvalue
            (:`SemiAuto`
              (`self.ShootBullet`))
            (:`FullAuto`
              (bind _returnvalue_2 (`KismetSystemLibrary.K2_SetTimerDelegate` (`|CreateDelegate` :!event `ShootBullet`) (`self.FireInterval`) true :!label _label_2))
              (set `self.FiringTimer` _returnvalue_2)
              (`self.ShootBullet`))
            (:`Burst`
              (goto _label_2))
            (:`InterruptibleBurst`
              (goto _label_2)))))
      (else
        (`self.StopFiring` :!label _label_3)))
    (else
      (switch `EAGR_FireMode` _returnvalue
        (:`SemiAuto`
          (goto _label_3))
        (:`FullAuto`
          (goto _label_3))
        (:`InterruptibleBurst`
          (goto _label_3))))))

(event `ResetFiring`
  ;[0 0 0] Actual part where we start the process of firing, checking if we can fire and then starting the firing sequence
  (goto _label :!via `Reset`))

(event `HitEffect`
  (params (ImpactPositions :type "Vector Structure") (`Impact Normals` :type "Vector Structure") (ImpactSurfaceTypes :type "EPhysicalSurface Enum" :default "SurfaceType_Default"))
  ;[0 0 0] Spawn and activate Weapon Impact system
  (`/Engine/EditorBlueprintResources/StandardMacros.IsValid` (`self.Weapon Impacts`)
    (:`Is Valid`
      _)
    (:`Is Not Valid`
      (bind _returnvalue (`|SpawnActorFromClass` (`self.HitEffectClass`) (`KismetMathLibrary.MakeTransform` (0.0 0.0 0.0)) "Undefined" "OverrideRootScale" null null))
      (bind _output_get (set `self.Weapon Impacts` _returnvalue))
      (`Actor.K2_AttachToComponent` _output_get (`self.SkeletalMesh`) "None" "KeepRelative" "KeepRelative" "KeepRelative" true)))
  (set `/Game/ParallelBeam/Core/BPs/Actors/BP_WepEffectManager.ImpactPositions` (`|MakeArray` ImpactPositions) (`self.Weapon Impacts`))
  (set `/Game/ParallelBeam/Core/BPs/Actors/BP_WepEffectManager.ImpactNormals` (`|MakeArray` `Impact Normals`) (`self.Weapon Impacts`))
  (set `/Game/ParallelBeam/Core/BPs/Actors/BP_WepEffectManager.ImpactSurfaceTypes` (`|MakeArray` ImpactSurfaceTypes) (`self.Weapon Impacts`))
  (set `/Game/ParallelBeam/Core/BPs/Actors/BP_WepEffectManager.MuzzlePosition` (+ (`self.GetSocketLocation` (`self.SkeletalMesh`) "Muzzle_socket") (`self.MuzzleOffset`)) (`self.Weapon Impacts`))
  (`/Game/ParallelBeam/Core/BPs/Actors/BP_WepEffectManager.Fire` (`self.Weapon Impacts`)))

(event `MLT_ContinueFiringEffect`
  (params (Start :type Boolean))
  ;[0 0 0] Replication of firing
  ; replicationg of firing event for everyone by the client
  ; instead of replicating each time we shoot , we simple replicate start and stop of shooting so its cheaper on network
  (`self.StartFiring` Start))

(event `SVR_StartFiring`
  (params (Start :type Boolean))
  ;[0 0 0] Replication of firing
  ; replicationg of firing event for everyone by the client
  ; instead of replicating each time we shoot , we simple replicate start and stop of shooting so its cheaper on network
  (`self.StartFiring` Start)
  (`self.MLT_ContinueFiringEffect` Start))

(event `StopFiring`
  (bind _burstcooldown (`self.BurstCooldown`))
  (bind _fireinterval (`self.FireInterval`))
  ;[0 0 0] Stoping the firing sequence, callled when run out of ammo, brust count and when player leaves input
  ; then reseting the firing sequence with a proper delay so we can begin firing again
  (`KismetSystemLibrary.K2_ClearAndInvalidateTimerHandle` (`self.FiringTimer`))
  (set `self.CurrentShot` 0)
  (`self.firingEffect` false)
  (`KismetSystemLibrary.Delay` (select `EAGR_FireMode` (`self.GetFireMode`) :`SemiAuto` _fireinterval :`FullAuto` _fireinterval :`Burst` _burstcooldown :`InterruptibleBurst` _burstcooldown :`Custom` _fireinterval))
  (`self.ResetFiring`)
  (goto _label_5 :!via `Reset`))

(event `CLT_StartFiring`
  (params (Start :type Boolean))
  ;[0 0 0] Replication of firing
  ; replicationg of firing event for everyone by the client
  ; instead of replicating each time we shoot , we simple replicate start and stop of shooting so its cheaper on network
  (`self.StartFiring` Start)
  (`self.SVR_StartFiring` Start))

(event `ShootBullet`
  (bind _returnvalue (`self.GetFireMode`))
  ;[0 0 0] Part where we do shoot the bullet and process the hit
  (if (`self.CanFire`)
    (`/Engine/EditorBlueprintResources/StandardMacros.IncrementInt` (`self.CurrentShot`)
      (:`  `
        (if (or (`|EnumEquality` _returnvalue "Burst") (`|EnumEquality` _returnvalue "InterruptibleBurst"))
          (if (<= (`self.CurrentShot`) (`self.BurstCount`))
            (`self.ConsumeAmmo` :!label _label_4)
            (`|ExecutionSequence`
              (:`then_0`
                (if (`self.IsLocalPlayer`)
                  ;[0 0 0] Building ignore list for the line traces on the first shot
                  (`/Engine/EditorBlueprintResources/StandardMacros.DoOnce` false :!label _label_5
                    (:`Completed`
                      (set `self.IgnoreList` (`self.BuildIgnoreActorList`))))))
              (:`then_1`
                (for _ (range 1 (+ (`self.ProjectileSpawnAmount`) 1))
                  (if (not (`self.IsLocalPlayer`))
                    (`/Engine/EditorBlueprintResources/ActorComponentMacros.Switch Has Authority`
                      (:`Authority`
                        _)))
                  ;;[0 0 0] Checking if  the weapon even wants to do a line trace shoot
                  (if (> (`self.LineTraceDistance`) 0.0)
                    (bind _hits (`self.PenetrationTrace`))
                    ;;[0 0 0] If line trace did not hit anyhting then we resort to firing a projectile on the server
                    (if (`KismetArrayLibrary.Array_IsNotEmpty` _hits)
                      (if (`self.IsLocalPlayer`)
                        (`self.SVR_ValidateHits` _hits)
                        (`/Engine/EditorBlueprintResources/ActorComponentMacros.Switch Has Authority`
                          (:`Remote`
                            (for _array_element _hits
                              (`self.OnObjectHit` _array_element)))))
                      (else
                        (if (`self.CanUsePhysicalProjectiles`) :!label _label_6
                          (`self.SpawnProjectile`))))
                    (else
                      (goto _label_6)))))
              (:`then_2`
                (`self.firingEffect` true)
                (set `self.Effect_Ammo_Local` (- (`self.Effect_Ammo_Local`) (`self.AmmoConsumptionPerShot`)))))
            (else
              (`self.StopFiring` :!label _label_7)))
          (else
            (goto _label_4)))))
    (else
      (goto _label_7))))

(event `SVR_ValidateHits`
  (params (Hits :type "Array of HitResult Structure"))
  ;[0 0 0] Client asks server to validate its hits an do the damge
  (`self.ValidateHits` Hits))

(event `OnObjectHit`
  (params (Hit :type "HitResult Structure"))
  (bind (_bblockinghit _binitialoverlap _time _distance _location _impactpoint _normal _impactnormal _physmat _hitactor _hitcomponent _hitbonename _bonename) (`GameplayStatics.BreakHitResult` Hit))
  (bind _surfacetype (`PhysicalMaterial.SurfaceType` _physmat))
  ;[0 0 0] On hitting the object we damage it and spaown the ffects
  ; local clients also call it to get quick feedback of thier hits but dosent deal damage
  (bind _returnvalue (`self.CalculateDamage` _bonename _hitcomponent))
  (`self.MLT_HitEffects` _location _impactnormal _surfacetype)
  (`GameplayStatics.ApplyPointDamage` _hitactor _returnvalue _impactnormal Hit (`Actor.GetInstigatorController` (`self.OwnerPawn`)) (`self.GetOwner`) (`.DamageType` (defaults `Object` (`self.AmmoType`))))
  (if (`self.IsLocalPlayer`)
    (`self.HitEffect` _location _impactnormal _surfacetype)))

(event `firingEffect`
  (params (Start :type Boolean))
  (bind _ns_muzzleflash (`self.NS_MuzzleFlash`))
  (bind _dt_anims (`self.DT_Anims`))
  (bind _ns_shelleject (`self.NS_ShellEject`))
  (bind _shellejection_system (`self.ShellEjection System`))
  (bind _ns_shelleject_2 (`self.NS_ShellEject`))
  (bind _audio (`self.Audio`))
  (bind _return_value (`/Game/ParallelBeam/Core/BPs/FunctionLib/BFL_MSK.GetMSKLocomotionComponent` (`Actor.GetOwner` (`self.GetOwner`))))
  ;[0 0 0] Firing effects that are called by everyone to show weapon is firing
  ; For local player also manages the recoil and such effects
  (if Start
    (`/Engine/EditorBlueprintResources/StandardMacros.IsValid` (`self.GetOwner`)
      (:`Is Valid`
        (`|ExecutionSequence`
          (:`then_0`
            (bind _montagecomponent (`self.MontageComponent`)
              (:`then`
                (`/Game/ParallelBeam/Core/BPs/Components/BP_MSK_Montage.PlayMontage` _montagecomponent true false (`self.GetOwner`) (select `bool` (> (`self.Effect_Ammo_Local`) 1) :`false` (struct :`TagName` "Actions.FireEmpty") :`true` (struct :`TagName` "Actions.Fire") :!type "GameplayTag Structure")))
              (:`else`
                _))
            (set `self.Muzzle Flash Trigger` (not (`self.Muzzle Flash Trigger`)))
            (`self.Recoil` true)
            (if (not (`KismetSystemLibrary.IsDedicatedServer`))
              (`|ExecutionSequence`
                (:`then_0`
                  (message `/Game/ParallelBeam/Core/BPs/Interfaces/BPI_HUD.UpdateGameUIValues` (`/Game/ParallelBeam/Core/BPs/FunctionLib/BFL_MSK.GetMSK_HUD` (`self.GetOwner`))))
                (:`then_1`
                  (`/Engine/EditorBlueprintResources/StandardMacros.IsValid` (`self.NS_MuzzleFlash`)
                    (:`Is Valid`
                      _)
                    (:`Is Not Valid`
                      (bind _returnvalue (`NiagaraFunctionLibrary.SpawnSystemAttached` (`self.Muzzle Flash System`) (`self.SkeletalMesh`) "Muzzle_socket" (`self.MuzzleOffset`) (struct :`Yaw` 90.0) "KeepRelativeOffset" true true "ManualRelease"))
                      (set `self.NS_MuzzleFlash` _returnvalue)))
                  (`NiagaraComponent.SetVariableBool` (`self.NS_MuzzleFlash`) "User.Trigger" (`self.Muzzle Flash Trigger`)))
                (:`then_2`
                  (if (not (`AudioComponent.IsPlaying` _audio))
                    (`AudioComponent.Play` _audio 0.0))
                  (`AudioParameterControllerInterface.SetIntParameter` _audio "MagazineAmmo" (`self.GetAmmoCount`))
                  (`AudioParameterControllerInterface.SetTriggerParameter` (`self.Audio`) "Fire"))
                (:`then_3`
                  (`/Engine/EditorBlueprintResources/StandardMacros.IsValid` _shellejection_system
                    (:`Is Valid`
                      (`/Engine/EditorBlueprintResources/StandardMacros.IsValid` (`self.NS_ShellEject`)
                        (:`Is Valid`
                          _)
                        (:`Is Not Valid`
                          (bind _returnvalue_2 (`NiagaraFunctionLibrary.SpawnSystemAttached` _shellejection_system (`self.SkeletalMesh`) "Shell_Eject" (0.0 0.0 0.0) (struct) "KeepRelativeOffset" true true "ManualRelease"))
                          (set `self.NS_ShellEject` _returnvalue_2)
                          (`NiagaraComponent.SetVariableStaticMesh` _ns_shelleject "ShellEjectStaticMesh" (defaults `Object` (`self.AmmoType`)))))
                      (`NiagaraComponent.SetVariableBool` _ns_shelleject "User.Trigger" (`self.Muzzle Flash Trigger`)))))
                (:`then_4`
                  (`KismetSystemLibrary.RetriggerableDelay` 0.5)
                  (`FXSystemComponent.ReleaseToPool` _ns_muzzleflash)
                  (`self.K2_DestroyComponent` _ns_muzzleflash)
                  (set `self.Muzzle Flash Trigger` false)
                  (set `self.NS_MuzzleFlash` null)
                  (`/Engine/EditorBlueprintResources/StandardMacros.IsValid` _ns_shelleject_2
                    (:`Is Valid`
                      (`FXSystemComponent.ReleaseToPool` _ns_shelleject_2)
                      (`self.K2_DestroyComponent` _ns_shelleject_2))
                    (:`Is Not Valid`
                      _))
                  (set `self.NS_ShellEject` null)))))
          (:`then_1`
            (goto _label_8 :!via `Open`)))))
    (else
      (if (<= (`self.Effect_Ammo_Local`) 0)
        (`AudioParameterControllerInterface.SetTriggerParameter` (`self.Audio`) "DryClick"))
      (`|ExecutionSequence`
        (:`then_0`
          (`/Engine/EditorBlueprintResources/StandardMacros.Gate` true :!label _label_8
            (:`Exit`
              (`KismetSystemLibrary.RetriggerableDelay` (`self.Recoil Time to Complete`))
              (`/Engine/EditorBlueprintResources/StandardMacros.IsValid` _return_value
                (:`Is Valid`
                  (`/Game/ParallelBeam/Core/BPs/Components/BP_MSK_Locomotion.StopRecoil` _return_value (`self.Recoil Time to Reset`))
                  (set `/Game/ParallelBeam/Core/BPs/Data/DTA_WeaponAnimation.IsFiring` false (`self.DT_Anims`))
                  (set `/Game/ParallelBeam/Core/BPs/Data/DTA_WeaponAnimation.RecoilLocation` (0.0 0.0 0.0) _dt_anims)
                  (set `/Game/ParallelBeam/Core/BPs/Data/DTA_WeaponAnimation.RecoilRotation` (struct) _dt_anims))
                (:`Is Not Valid`
                  _))
              (`KismetSystemLibrary.RetriggerableDelay` 0.5)
              (`self.Recoil` false))))
        (:`then_1`
          (goto _label_8 :!via `Close`))))))

(event `self.SpawnProjectile`
  (bind _returnvalue (`self.K2_GetComponentLocation`))
  (`|SpawnActorFromClass` (`|GetArrayItem` (`self.GetAmmoSequence`)) (`KismetMathLibrary.MakeTransform` _returnvalue (`KismetMathLibrary.FindLookAtRotation` _returnvalue (+ _returnvalue (* (`KismetMathLibrary.GetForwardVector` (`KismetMathLibrary.ComposeRotators` (`self.CalculateFireSpread`) (`self.K2_GetComponentRotation`))) (`self.ClientAimTraceDistance`))))) "AdjustIfPossibleButAlwaysSpawn" "MultiplyWithRoot" (`self.GetOwner`) (`self.ProjectileInitialSpeed`) (`self.bDebug`) (`self.DebugDuration`) (`self.IgnoreList`) (`self.WeaponTags`) (`self.WeaponDamage`) (`self.OwnerPawn`)))

(fn `CalculateAnimRecoil`
  (params (IsAiming :type Boolean))
  (bind _dt_anims (`self.DT_Anims`))
  (bind (_minincrease _maxincrease _recoilcap) (break `/Game/ParallelBeam/Core/BPs/Data/Structures/S_Recoil` (select `bool` (`local.IsAiming`) :`false` (`self.Anim_Recoil`) :`true` (`self.Anim_Recoil_Aiming`))))
  (set `/Game/ParallelBeam/Core/BPs/Data/DTA_WeaponAnimation.RecoilLocation` (`KismetMathLibrary.MakeVector` (`KismetMathLibrary.FClamp` (.x (+ (`/Game/ParallelBeam/Core/BPs/Data/DTA_WeaponAnimation.RecoilLocation` (`self.DT_Anims`)) (`KismetMathLibrary.MakeVector` (`KismetMathLibrary.RandomFloatInRange` (.x (.location _minincrease)) (.x (.location _maxincrease))) (`KismetMathLibrary.RandomFloatInRange` (.y (.location _minincrease)) (.y (.location _maxincrease))) (`KismetMathLibrary.RandomFloatInRange` (.z (.location _minincrease)) (.z (.location _maxincrease)))))) (* (.x (.location _recoilcap)) -1.0) (.x (.location _recoilcap))) (`KismetMathLibrary.FClamp` (.y (+ (`/Game/ParallelBeam/Core/BPs/Data/DTA_WeaponAnimation.RecoilLocation` (`self.DT_Anims`)) (`KismetMathLibrary.MakeVector` (`KismetMathLibrary.RandomFloatInRange` (.x (.location _minincrease)) (.x (.location _maxincrease))) (`KismetMathLibrary.RandomFloatInRange` (.y (.location _minincrease)) (.y (.location _maxincrease))) (`KismetMathLibrary.RandomFloatInRange` (.z (.location _minincrease)) (.z (.location _maxincrease)))))) (* (.y (.location _recoilcap)) -1.0) (.y (.location _recoilcap))) (`KismetMathLibrary.FClamp` (.z (+ (`/Game/ParallelBeam/Core/BPs/Data/DTA_WeaponAnimation.RecoilLocation` (`self.DT_Anims`)) (`KismetMathLibrary.MakeVector` (`KismetMathLibrary.RandomFloatInRange` (.x (.location _minincrease)) (.x (.location _maxincrease))) (`KismetMathLibrary.RandomFloatInRange` (.y (.location _minincrease)) (.y (.location _maxincrease))) (`KismetMathLibrary.RandomFloatInRange` (.z (.location _minincrease)) (.z (.location _maxincrease)))))) (* (.z (.location _recoilcap)) -1.0) (.z (.location _recoilcap)))) _dt_anims)
  (set `/Game/ParallelBeam/Core/BPs/Data/DTA_WeaponAnimation.RecoilRotation` (`KismetMathLibrary.MakeRotator` (`KismetMathLibrary.FClamp` (.roll (`KismetMathLibrary.MakeRotator` (`KismetMathLibrary.RandomFloatInRange` (.roll (.rotation _minincrease)) (.roll (.rotation _maxincrease))) (`KismetMathLibrary.RandomFloatInRange` (.pitch (.rotation _minincrease)) (.pitch (.rotation _maxincrease))) (`KismetMathLibrary.RandomFloatInRange` (.yaw (.rotation _minincrease)) (.yaw (.rotation _maxincrease))))) (* (.roll (.rotation _recoilcap)) -1.0) (.roll (.rotation _recoilcap))) (`KismetMathLibrary.FClamp` (.pitch (`KismetMathLibrary.MakeRotator` (`KismetMathLibrary.RandomFloatInRange` (.roll (.rotation _minincrease)) (.roll (.rotation _maxincrease))) (`KismetMathLibrary.RandomFloatInRange` (.pitch (.rotation _minincrease)) (.pitch (.rotation _maxincrease))) (`KismetMathLibrary.RandomFloatInRange` (.yaw (.rotation _minincrease)) (.yaw (.rotation _maxincrease))))) (* (.pitch (.rotation _recoilcap)) -1.0) (.pitch (.rotation _recoilcap))) (`KismetMathLibrary.FClamp` (.yaw (`KismetMathLibrary.MakeRotator` (`KismetMathLibrary.RandomFloatInRange` (.roll (.rotation _minincrease)) (.roll (.rotation _maxincrease))) (`KismetMathLibrary.RandomFloatInRange` (.pitch (.rotation _minincrease)) (.pitch (.rotation _maxincrease))) (`KismetMathLibrary.RandomFloatInRange` (.yaw (.rotation _minincrease)) (.yaw (.rotation _maxincrease))))) (* (.yaw (.rotation _recoilcap)) -1.0) (.yaw (.rotation _recoilcap)))) _dt_anims)
  (set `/Game/ParallelBeam/Core/BPs/Data/DTA_WeaponAnimation.IsFiring` true (`self.DT_Anims`)))

(fn `CalculateDamage`
  (params (BoneName :type "Name (by ref)") (HitComponent :type "PrimitiveComponent Object Reference"))
  (returns (ReturnValue :type "Float (double-precision)"))
  (locals (Loc_bone :type Name))
  (bind _damage_values (`self.Damage Values`))
  (bind (_value _returnvalue) (`BlueprintMapLibrary.Map_Find` _damage_values (`local.Loc_bone`)))
  (bind _asskeletal_mesh_component (cast `SkeletalMeshComponent` HitComponent)
    (:`then`
      (`|ExecutionSequence`
        (:`then_0`
          (set `local.Loc_bone` BoneName)
          (if _returnvalue :!label _label
            (return (* _value (`self.WeaponDamage`)))
            (else
              (set `local.Loc_bone` (`SkinnedMeshComponent.GetParentBone` _asskeletal_mesh_component (`local.Loc_bone`)))
              (`/Engine/EditorBlueprintResources/StandardMacros.Do N` 5
                (:`Exit`
                  (goto _label))))))
        (:`then_1`
          _)))
    (:`CastFailed`
      _))
  (return (* (`BlueprintMapLibrary.Map_Find` _damage_values "Base") (`self.WeaponDamage`))))

(fn `OnRep_AmmoType`
  (bind _ammotype (`self.AmmoType`)
    (:`then`
      (bind (_casingmesh _damagevalues _projectiletype) (defaults `Object` _ammotype))
      (set `self.Damage Values` _damagevalues)
      (`self.SetAmmoSequence` (`|MakeArray` _projectiletype)))
    (:`else`)))

(fn `PenetrationTrace`
  (returns (Hits :type "Array of HitResult Structure"))
  (locals (LOC_TraceStartLocation :type "Vector Structure") (LOCForwardVector :type "Vector Structure") (LOC_PenetrationStrength :type "Float (single-precision)" :default 200.0) (LOC_Hits :type "Array of HitResult Structure"))
  (bind _ownerpawn (`self.OwnerPawn`))
  (bind _loc_tracestartlocation (`local.LOC_TraceStartLocation`))
  (`|ExecutionSequence`
    (:`then_0`
      (`/Engine/EditorBlueprintResources/StandardMacros.IsValid` _ownerpawn
        (:`Is Valid`
          (set `local.LOC_TraceStartLocation` (`self.K2_GetComponentLocation`))
          (set `local.LOCForwardVector` (`KismetMathLibrary.GetForwardVector` (`KismetMathLibrary.ComposeRotators` (`self.CalculateFireSpread`) (`Pawn.GetControlRotation` _ownerpawn))))
          (`/Engine/EditorBlueprintResources/StandardMacros.Do N` 10 :!label _label
            (:`Exit`
              (bind _outhit (`KismetSystemLibrary.LineTraceSingle` _loc_tracestartlocation (+ _loc_tracestartlocation (* (`local.LOCForwardVector`) (`self.ClientAimTraceDistance`))) "TraceTypeQuery3" false (`self.IgnoreList`)))
              (bind (_bblockinghit _binitialoverlap _time _distance _location _impactpoint _normal _impactnormal _physmat _hitactor _hitcomponent) (`GameplayStatics.BreakHitResult` _outhit))
              (if _bblockinghit
                (`KismetArrayLibrary.Array_Add` (`local.LOC_Hits`) _outhit)
                (bind (_outhits _returnvalue) (`KismetSystemLibrary.SphereTraceMulti` (+ _location (* (`local.LOCForwardVector`) 50.0)) _location 2.0 "TraceTypeQuery3" false (`self.IgnoreList`)))
                (if _returnvalue
                  (for _array_element _outhits
                    (bind (_bblockinghit_2 _binitialoverlap_2 _time_2 _distance_2 _location_2 _impactpoint_2 _normal_2 _impactnormal_2 _physmat_2 _hitactor_2 _hitcomponent_2) (`GameplayStatics.BreakHitResult` _array_element))
                    (if (and _bblockinghit_2 (== _hitcomponent _hitcomponent_2))
                      (`|ExecutionSequence`
                        (:`then_0`
                          (break))
                        (:`then_1`
                          (bind _output_get (set `local.LOC_PenetrationStrength` (- (`local.LOC_PenetrationStrength`) (* (`KismetMathLibrary.Vector_Distance` _location_2 _location) (`.ShearStrength` (break `PhysicalMaterialStrength` (`PhysicalMaterial.Strength` _physmat)))))))
                          (if (> _output_get 0.0)
                            (set `local.LOC_TraceStartLocation` (+ _location_2 (* (`local.LOCForwardVector`) 1.0)))
                            (set `local.LOCForwardVector` (+ (`local.LOCForwardVector`) (0.0 0.0 -0.002)))
                            (goto _label)))))))))))))
    (:`then_1`
      (return (`local.LOC_Hits`)))))

(fn `Recoil`
  (params (Start :type Boolean))
  (locals (LOC_Aiming :type Boolean :default false))
  (bind _recoilcurve (`self.RecoilCurve`))
  (bind _return_value (`/Game/ParallelBeam/Core/BPs/FunctionLib/BFL_MSK.GetMSKLocomotionComponent` (`self.OwnerPawn`)))
  (bind _returnvalue (`KismetMathLibrary.Conv_IntToDouble` (`self.RecoilCount`)))
  (`/Engine/EditorBlueprintResources/StandardMacros.IsValid` _return_value
    (:`Is Valid`
      (set `local.LOC_Aiming` (`/Game/ParallelBeam/Core/BPs/Components/BP_MSK_Locomotion.IsAiming` _return_value))
      (if (`self.IsLocalPlayer`)
        (if (> _returnvalue (`.MaxTime` (`CurveBase.GetTimeRange` _recoilcurve)))
          (set `self.RecoilCount` 0))
        (if Start
          (`/Engine/EditorBlueprintResources/StandardMacros.IsValid` _return_value
            (:`Is Valid`
              (`/Game/ParallelBeam/Core/BPs/Components/BP_MSK_Locomotion.AddRecoil` _return_value (`KismetMathLibrary.MakeVector2D` (* (`self.VerticalRecoilMultiplier`) (.y (* (`CurveVector.GetVectorValue` _recoilcurve _returnvalue) (select `bool` (`local.LOC_Aiming`) :`false` (`self.RecoilMultiplier`) :`true` (`self.AimingRecoilMultiplier`))))) (* (`self.HorizonalRecoilMultiplier`) (.x (* (`CurveVector.GetVectorValue` _recoilcurve _returnvalue) (select `bool` (`local.LOC_Aiming`) :`false` (`self.RecoilMultiplier`) :`true` (`self.AimingRecoilMultiplier`)))))) (`self.Recoil Time to Complete`)))
            (:`Is Not Valid`
              _))
          (message `/Game/ParallelBeam/Core/BPs/Interfaces/BPI_HUD.WeaponFired` (`/Game/ParallelBeam/Core/BPs/FunctionLib/BFL_MSK.GetMSK_HUD` (`self.OwnerPawn`)))
          (`/Engine/EditorBlueprintResources/StandardMacros.IncrementInt` (`self.RecoilCount`)
            (:`  `
              (`|ExecutionSequence`
                (:`then_0`
                  (if (`self.Muzzle Flash Trigger`)
                    (`PlayerCameraManager.StartCameraShake` :`self` (`self.Player Camera Manager`) :`ShakeClass` (`self.FireShake`))))
                (:`then_1`
                  (`self.CalculateAnimRecoil` (`local.LOC_Aiming`))))))
          (else
            (set `self.RecoilCount` 0)))))))

(fn `ValidateHits`
  (params (Array :type "Array of HitResult Structure"))
  (locals (LOC_ActorsToIgnore :type "Array of Actor Object Reference") (LOC_EndTraceSize :type "Vector Structure"))
  ;[0 0 0] a simple check by server to see if all the hits client did were infact valid and should be possible , if so then server deals the damage else ignores the damage request and discards any of the pending hit checks
  (set `self.IgnoreList` (`self.BuildIgnoreActorList`))
  (set `local.LOC_ActorsToIgnore` (`self.IgnoreList`))
  (for (_array_element _array_index) Array
    (bind (_bblockinghit _binitialoverlap _time _distance _location _impactpoint _normal _impactnormal _physmat _hitactor) (`GameplayStatics.BreakHitResult` _array_element))
    (`KismetArrayLibrary.Array_Add` (`local.LOC_ActorsToIgnore`) _hitactor)
    (if (== _array_index 0)
      (set `local.LOC_EndTraceSize` (`self.K2_GetComponentLocation`))
      (else
        (set `local.LOC_EndTraceSize` (`.Location` (`GameplayStatics.BreakHitResult` (`|GetArrayItem` Array (- _array_index 1)))))))
    (bind (_outhit _returnvalue) (`KismetSystemLibrary.LineTraceSingle` _location (`local.LOC_EndTraceSize`) "TraceTypeQuery3" false (`local.LOC_ActorsToIgnore`)))
    (if _returnvalue
      (break)
      (else
        (`self.OnObjectHit` _array_element)))))