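; Component on an enterable pawn, such as a vehicle, that handles entering, seating and exiting players.
; Server events either possess the pawn or directly seat the player, updating input mapping, UI and crosshair.
; A multicast toggles the rider's collision, movement and linked anim layers while attached to the tagged seat.
; Exiting tries tagged exits nearest-first with ground and capsule traces, then repossesses the original pawn; look pitch is clamped and replicated.
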(event `SVR_EnteredPawn`
  (params (Controller :type "Controller Object Reference"))
  (bind _ownerpawn (`self.OwnerPawn`))
  (bind _returnvalue (`Actor.GetComponentByClass` (`self.Controller`) "/Game/ParallelBeam/Core/BPs/Components/GameModeComponents/BP_ControllerComponent.BP_ControllerComponent_C"))
  ;[0 0 0] Once its confirmed we can enter, we enter this pawn and set correct refrences, and attach existing pawn to it
  (set `self.Controller` Controller)
  (set `self.OwnerPawn` (`/Game/ParallelBeam/Core/BPs/Components/GameModeComponents/BP_ControllerComponent.MainPawn` (`Actor.GetComponentByClass` (`self.Controller`) "/Game/ParallelBeam/Core/BPs/Components/GameModeComponents/BP_ControllerComponent.BP_ControllerComponent_C")))
  (`self.AddMappingContext` true)
  (set `/Game/ParallelBeam/Core/BPs/Components/GameModeComponents/BP_ControllerComponent.CurrentConnectedPawn` self _returnvalue)
  (`/Game/ParallelBeam/Core/BPs/Components/GameModeComponents/BP_ControllerComponent.CLT_UpdatePawnUI` _returnvalue (`self.VehicleWidget`))
  (`/Game/ParallelBeam/Core/BPs/Components/GameModeComponents/BP_ControllerComponent.CLT_SetCrosshairWidget` _returnvalue (`self.VehicleCrosshair`))
  (`self.MLT_ChangePawnCollusion` false _ownerpawn)
  (`Actor.K2_AttachToComponent` _ownerpawn (`self.SeatLocation`) "None" "SnapToTarget" "SnapToTarget" "SnapToTarget" true)
  (set `/Game/ParallelBeam/Core/BPs/Components/BP_MSK_Locomotion.AttachToComponent` (`self.SeatLocation`) (`/Game/ParallelBeam/Core/BPs/FunctionLib/BFL_MSK.GetMSKLocomotionComponent` _ownerpawn)))

(event `SVR_RequestExit`
  (bind _ownerpawn (`self.OwnerPawn`))
  (bind (_returnvalue_roll _returnvalue_pitch _returnvalue_yaw) (`KismetMathLibrary.BreakRotator` (`Actor.K2_GetActorRotation` _ownerpawn)))
  ;[0 0 0] OnExit, check ecit location, if valid exit and posses original pawn
  (`/Engine/EditorBlueprintResources/StandardMacros.IsValid` (`self.OwnerPawn`)
    (:`Is Valid`
      (bind (_return_value _exitloc) (`self.ExitPawn`))
      (if _return_value
        (`self.AddMappingContext` false)
        (set `/Game/ParallelBeam/Core/BPs/Components/GameModeComponents/BP_ControllerComponent.CurrentConnectedPawn` null (`Actor.GetComponentByClass` (`self.Controller`) "/Game/ParallelBeam/Core/BPs/Components/GameModeComponents/BP_ControllerComponent.BP_ControllerComponent_C"))
        (`Actor.K2_SetActorLocation` _ownerpawn (+ _exitloc (0.0 0.0 45.0)) false false)
        (`Actor.K2_SetActorRotation` _ownerpawn (`KismetMathLibrary.MakeRotator` 0.0 0.0 _returnvalue_yaw) false)
        (set `/Game/ParallelBeam/Core/BPs/Components/BP_MSK_Locomotion.AttachToComponent` null (`/Game/ParallelBeam/Core/BPs/FunctionLib/BFL_MSK.GetMSKLocomotionComponent` _ownerpawn))
        (`self.MLT_ChangePawnCollusion` true _ownerpawn)
        (`Actor.K2_DetachFromActor` _ownerpawn "KeepWorld" "KeepWorld" "KeepWorld")
        (`Controller.Possess` (`self.Controller`) _ownerpawn)
        (set `self.OwnerPawn` null)))))

(event `SVR_AttemptEnter Pawn`
  (params (Controller :type "Controller Object Reference"))
  (bind _as_pawn (`self.As Pawn`))
  ;[0 0 0] OnTryToEnter, we check if we can enter, then check if we should posses it or simply attach to it?
  (bind _return_value (message `/Game/ParallelBeam/Core/BPs/Interfaces/BPI_Interaction.CanInteract` _as_pawn (`Controller.K2_GetPawn` Controller)))
  (if _return_value
    (if (`self.CanPossesThisPawn`)
      (`Controller.Possess` Controller _as_pawn)
      (else
        (`self.SVR_EnteredPawn` Controller)))))

(event `self.ReceiveBeginPlay`
  ;[0 0 0] FindingNessaryComponentsOnStart
  (bind _aspawn (cast `Pawn` (`self.GetOwner`)))
  (bind _output_get (set `self.As Pawn` _aspawn))
  (set `self.SeatLocation` (`|GetArrayItem` (`Actor.GetComponentsByTag` _output_get "/Script/Engine.SceneComponent" "SeatLocation")))
  (set `self.Exits` (`Actor.GetComponentsByTag` _output_get "/Script/Engine.SceneComponent" "ExitLocation")))

(event `CLT_ConfirmedExit`
  ;[0 0 0] LetClientRemove the mapings when exiting
  (if (`self.CanPossesThisPawn`)
    (bind _asplayer_controller (cast `PlayerController` (`Pawn.GetController` (`self.As Pawn`))))
    (`EnhancedInputSubsystemInterface.RemoveMappingContext` (pcsubsystem `EnhancedInputLocalPlayerSubsystem` _asplayer_controller) (`self.Mapping Context`) (struct))))

(event `AddMappingContext`
  (params (Add :type Boolean))
  ;[0 0 0] OnClientEntered confirmed, we add the mapping context to control this
  (if (`self.CanPossesThisPawn`)
    (`/Game/ParallelBeam/Core/BPs/Components/GameModeComponents/BP_ControllerComponent.CLT_AddMappingContext` (`Actor.GetComponentByClass` (`self.Controller`) "/Game/ParallelBeam/Core/BPs/Components/GameModeComponents/BP_ControllerComponent.BP_ControllerComponent_C") (`self.Mapping Context`) Add)))

(event `MLT_ChangePawnCollusion`
  (params (Enable :type Boolean) (Pawn :type "Actor Object Reference"))
  ;[0 0 0] UpdatePawnCollusions and anim instance for everyon e
  (`CharacterMovementComponent.SetMovementMode` (`Actor.GetComponentByClass` Pawn "/Script/Engine.CharacterMovementComponent") (select `bool` Enable :`false` "MOVE_None" :`true` "MOVE_Walking" :!type "EMovementMode Enum") 0)
  (`PrimitiveComponent.SetCollisionEnabled` (`Actor.GetComponentByClass` Pawn "/Script/Engine.CapsuleComponent") (select `bool` Enable :`false` "NoCollision" :`true` "QueryAndPhysics" :!type "ECollisionEnabled Enum"))
  (`SkeletalMeshComponent.LinkAnimClassLayers` (`|GetArrayItem` (`Actor.GetComponentsByTag` Pawn "/Script/Engine.SkeletalMeshComponent" "MainMesh")) (select `bool` Enable :`false` (`self.AnimBP`)))
  (if (not Enable)
    (`Actor.K2_AttachToComponent` Pawn (`self.SeatLocation`) "None" "SnapToTarget" "SnapToTarget" "SnapToTarget" true)))

(event `SetLookRotation`
  (bind _controller (`self.Controller`))
  (bind (_pitchlimits_x _pitchlimits_y) (`KismetMathLibrary.BreakVector2D` (`self.PitchLimits`)))
  (bind _returnvalue (`Controller.GetControlRotation` _controller))
  (bind _pitch (.pitch _returnvalue))
  ;[0 0 0] Manupulating the InputROtation to limit it at angles (UPand Down)
  (`Controller.SetControlRotation` _controller (`KismetMathLibrary.MakeRotator` (.roll _returnvalue) (`KismetMathLibrary.FClamp` (select `bool` (> _pitch 95.0) :`false` _pitch :`true` (- _pitch 360.0) :!type "Float (double-precision)") _pitchlimits_x _pitchlimits_y) (.yaw _returnvalue)))
  (bind _output_get (set `self.LookRotation` _returnvalue))
  (`self.SVR_SetLookRotation` _output_get))

(event `SVR_SetLookRotation`
  (params (NewRotation :type "Rotator Structure"))
  ;[0 0 0] Manupulating the InputROtation to limit it at angles (UPand Down)
  (set `self.LookRotation` NewRotation))

(fn `ExitPawn`
  (returns (`Return Value` :type Boolean) (ExitLoc :type "Vector Structure"))
  (locals (Loc_PawnLocation :type "Vector Structure" :default (0.0 0.0 0.0)) (Loc_Distances :type "Array of Float (double-precision)") (Loc_SelectedDistanceIndex :type Integer :default 0) (Loc_ExitLoc :type "Vector Structure" :default (0.0 0.0 0.0)) (Loc_Controller :type "Controller Object Reference") (Loc_TempExits :type "Array of SceneComponent Object Reference"))
  (bind _loc_selecteddistanceindex (`local.Loc_SelectedDistanceIndex`))
  (bind _loc_tempexits (`local.Loc_TempExits`))
  (bind _array (`|MakeArray` (`self.As Pawn`) :!type "Actor Object Reference"))
  (bind _returnvalue (`SceneComponent.K2_GetComponentLocation` (`|GetArrayItem` _loc_tempexits (`local.Loc_SelectedDistanceIndex`))))
  (set `local.Loc_Controller` (`self.Controller`))
  (set `local.Loc_TempExits` (`self.Exits`))
  (set `local.Loc_PawnLocation` (`Actor.K2_GetActorLocation` (`/Game/ParallelBeam/Core/BPs/Components/GameModeComponents/BP_ControllerComponent.MainPawn` (`Actor.GetComponentByClass` (`self.Controller`) "/Game/ParallelBeam/Core/BPs/Components/GameModeComponents/BP_ControllerComponent.BP_ControllerComponent_C"))))
  (for (_array_element _array_index) _loc_tempexits
    (`KismetArrayLibrary.Array_Set` (`local.Loc_Distances`) _array_index (`KismetMathLibrary.Abs` (`KismetMathLibrary.Vector_Distance` (`local.Loc_PawnLocation`) (`SceneComponent.K2_GetComponentLocation` _array_element))) true))
  (set `local.Loc_SelectedDistanceIndex` (`KismetMathLibrary.MinOfFloatArray` (`local.Loc_Distances`)) :!label _label)
  (bind (_outhit _returnvalue_2) (`KismetSystemLibrary.SphereTraceSingle` _returnvalue (- _returnvalue (0.0 0.0 200.0)) 50.0 "TraceTypeQuery1" false _array))
  (if _returnvalue_2
    (bind (_bblockinghit _binitialoverlap _time _distance _location) (`GameplayStatics.BreakHitResult` _outhit))
    (set `local.Loc_ExitLoc` _location)
    (bind _returnvalue_3 (+ _location (0.0 0.0 50.0)))
    (bind (_outhit_2 _returnvalue_4) (`KismetSystemLibrary.CapsuleTraceSingle` _returnvalue_3 _returnvalue_3 50.0 90.0 "TraceTypeQuery1" false _array "None" true (struct :`G` 0.35567 :`B` 1.0 :`A` 1.0) (struct :`R` 1.0 :`G` 0.719642 :`A` 1.0)))
    (if _returnvalue_4
      _
      (else
        (return true (`local.Loc_ExitLoc`)))))
  (`KismetArrayLibrary.Array_Remove` (`local.Loc_Distances`) _loc_selecteddistanceindex)
  (`KismetArrayLibrary.Array_Remove` (`local.Loc_TempExits`) _loc_selecteddistanceindex)
  (if (`KismetArrayLibrary.Array_IsNotEmpty` (`local.Loc_Distances`))
    (goto _label)))

(fn `SetAiming`
  (params (Aiming :type Boolean))
  (set `self.Aiming` Aiming))