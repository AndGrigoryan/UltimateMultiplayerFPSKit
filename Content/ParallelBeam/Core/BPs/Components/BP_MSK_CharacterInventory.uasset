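; Character inventory component that handles item pickup, weapon equipping, interaction and input actions like firing, aiming, reloading and leaning.
; Pickup events drive stacking, auto-equipping and weapon swaps, with trace-based placement for dropped items.
; Actions pass through a gameplay-tag state gate that blocks or undoes conflicting states, with server calls for several.
; A tick-driven sphere trace on the locally controlled player selects the interaction target and updates the HUD.
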(event `CustomEvent` :!signature `self.OnItemUpdated`
  (params (Item :type "Actor Object Reference") (UpdateType :type "EAGR_ItemUpdateType Enum" :default "PickedUp"))
  (`self.CheckInventoryStorage` Item UpdateType))

(event `self.ReceiveBeginPlay`
  (bind _as_character (`self.As Character`))
  ;[0 0 0] On start set bindings and base variabbles AND set the tick to happen on owning player only (for interactions)
  (add `self.OnItemUpdated` (delegate `CustomEvent`))
  (set `self.LocomotionComponent` (`/Game/ParallelBeam/Core/BPs/FunctionLib/BFL_MSK.GetMSKLocomotionComponent` (`self.GetOwner`)))
  (bind _ascharacter (cast `Character` (`self.GetOwner`))
    (:`then`
      (set `self.As Character` _ascharacter)
      (`self.SetComponentTickEnabled` false)
      (`KismetSystemLibrary.Delay` 2.0)
      (`self.SetComponentTickEnabled` (and (`Pawn.IsLocallyControlled` _as_character) (`Pawn.IsPlayerControlled` _as_character))))
    (:`CastFailed`
      (`self.SetComponentTickEnabled` false))))

(event `self.ReceiveTick`
  (params (DeltaSeconds :type "Float (single-precision)"))
  ;[0 0 0] Interaction Traces (OnOwningPlayer only)
  (`self.InteractionTraces`))

(event `RequestReload`
  ;[0 0 0] Requsting reload
  (`self.Reload`)
  (`self.SVR_Reload`))

(event `PrimaryAction`
  (params (Begin :type Boolean))
  ;[0 0 0] Primary And SecondaryActions
  (bind _output_get (set `self.AttemptPrimaryAction` Begin))
  (bind _blocked (`self.Change Action State` (struct :`TagName` "States.Firing") _output_get))
  (if (not _blocked)
    (message `/Game/ParallelBeam/Core/BPs/Interfaces/BPI_Weapon.Interact` (`self.GetItemInSlot` (struct :`TagName` "CharacterSlots.RightHand")) (`self.AttemptPrimaryAction`))))

(event `SVR_Reload`
  ;[0 0 0] Requsting reload
  (`self.Reload`))

(event `SecondaryAction`
  (params (Begin :type Boolean))
  ;[0 0 0] Primary And SecondaryActions
  (bind _output_get (set `self.AttemptSecondaryAction` Begin))
  (if (`/Game/ParallelBeam/Core/BPs/Components/BP_MSK_Locomotion.IsDuelWelding` (`/Game/ParallelBeam/Core/BPs/FunctionLib/BFL_MSK.GetMSKLocomotionComponent` (`self.GetOwner`)))
    (bind _blocked (`self.Change Action State` (struct :`TagName` "States.Firing") _output_get))
    (if (not _blocked)
      (message `/Game/ParallelBeam/Core/BPs/Interfaces/BPI_Weapon.Interact` (`self.GetItemInSlot` (struct :`TagName` "CharacterSlots.LeftHand")) (`self.AttemptSecondaryAction`)))
    (else
      (bind _blocked_2 (`self.Change Action State` (struct :`TagName` "States.Aiming") (`self.AttemptSecondaryAction`)))
      (if (not _blocked_2)
        (`self.SVR_Aiming` (`self.AttemptSecondaryAction`))))))

(event `ChangeItemMaterialSetting`
  (params (Picked :type Boolean) (Actor :type "Actor Object Reference"))
  (bind (_attachment_inventory _returnvalue) (`/Game/ParallelBeam/Core/BPs/FunctionLib/BFL_MSK.GetAttachmentInventory` Actor))
  (bind _returnvalue_2 (`KismetMathLibrary.Conv_BoolToDouble` Picked))
  (bind _returnvalue_3 (select `bool` Picked :`true` 1))
  ;[0 0 0] When we Equip Something, this updates its meshes to have the FOV effect for owning player
  (`/Engine/EditorBlueprintResources/StandardMacros.IsValid` Actor
    (:`Is Valid`
      (if (`Pawn.IsPlayerControlled` (`self.As Character`))
        (set `SceneComponent.bUseAttachParentBound` Picked (`|GetArrayItem` (`Actor.K2_GetComponentsByClass` Actor "/Script/Engine.BoxComponent")))
        (if _returnvalue
          (bind _return_value (`/Game/ParallelBeam/Core/BPs/Components/BP_AttachmentInventory.GetAllAttachments` _attachment_inventory))
          (for _array_element _return_value
            (bind _returnvalue_4 (`Actor.K2_GetComponentsByClass` _array_element "/Script/Engine.StaticMeshComponent"))
            (`MeshComponent.SetScalarParameterValueOnMaterials` _returnvalue_4 "UseFOV" _returnvalue_2)
            (bind _returnvalue_5 (`Actor.K2_GetComponentsByClass` _array_element "/Script/Engine.SkeletalMeshComponent"))
            (`MeshComponent.SetScalarParameterValueOnMaterials` _returnvalue_5 "UseFOV" _returnvalue_2)
            (`PrimitiveComponent.SetCustomDepthStencilValue` _returnvalue_4 _returnvalue_3)
            (`PrimitiveComponent.SetCustomDepthStencilValue` _returnvalue_5 _returnvalue_3)))
        (`MeshComponent.SetScalarParameterValueOnMaterials` (`Actor.K2_GetComponentsByClass` Actor "/Script/Engine.StaticMeshComponent") "UseFOV" _returnvalue_2)
        (`MeshComponent.SetScalarParameterValueOnMaterials` (`Actor.K2_GetComponentsByClass` Actor "/Script/Engine.SkeletalMeshComponent") "UseFOV" _returnvalue_2)
        (`MeshComponent.SetScalarParameterValueOnMaterials` (`Actor.K2_GetComponentsByClass` (`self.As Character`) "/Script/Engine.SkeletalMeshComponent") "UseFOV" 1.0)))))

(event `SVR_Aiming`
  (params (Enter :type Boolean))
  ;[0 0 0] Primary And SecondaryActions
  (`self.Change Action State` (struct :`TagName` "States.Aiming") Enter))

(event `SVR_EquipWeapon`
  (params (Slot :type "GameplayTag Structure"))
  (bind _returnvalue (`self.GetItemInSlot` Slot))
  ;[0 0 0] Equip Weapon input
  (`/Engine/EditorBlueprintResources/StandardMacros.IsValid` _returnvalue
    (:`Is Valid`
      (if (not (== (`self.GetItemInSlot` (struct :`TagName` "CharacterSlots.RightHand")) _returnvalue))
        (`AGR_ItemComponent.EquipItem` (`AGR_InventoryFunctionLibrary.GetItemComponent` _returnvalue) self (struct :`TagName` "CharacterSlots.RightHand") true)))))

(event `CLT_EquipmentUpdated`
  (bind _hud (`/Game/ParallelBeam/Core/BPs/FunctionLib/BFL_MSK.GetMSK_HUD` (`self.GetOwner`)))
  ;[0 0 0] Update UI when new Inventoru pics smth
  (message `/Game/ParallelBeam/Core/BPs/Interfaces/BPI_HUD.ShowGameUI` _hud true)
  (message `/Game/ParallelBeam/Core/BPs/Interfaces/BPI_HUD.UpdateGameUIValues` _hud))

(event `Leaning`
  (params (Right :type Boolean) (Start :type Boolean))
  ;[0 0 0] Leaning
  (bind _blocked (`self.Change Action State` (select `bool` Right :`false` (struct :`TagName` "States.Leaning.Left") :`true` (struct :`TagName` "States.Leaning.Right") :!type "GameplayTag Structure") Start))
  (if (not _blocked)
    (`self.SVR_Leaning` Right Start)))

(event `SVR_Leaning`
  (params (Right :type Boolean) (Start :type Boolean))
  ;[0 0 0] Leaning
  (`self.Change Action State` (select `bool` Right :`false` (struct :`TagName` "States.Leaning.Left") :`true` (struct :`TagName` "States.Leaning.Right") :!type "GameplayTag Structure") Start))

(event `SVR_Interact`
  (params (Start :type Boolean) (Actor :type "Actor Object Reference"))
  (bind _currentconnectedpawn (`/Game/ParallelBeam/Core/BPs/Components/GameModeComponents/BP_ControllerComponent.CurrentConnectedPawn` (`Actor.GetComponentByClass` (`Pawn.GetController` (`self.As Character`)) "/Game/ParallelBeam/Core/BPs/Components/GameModeComponents/BP_ControllerComponent.BP_ControllerComponent_C")))
  ;[0 0 0] Interaction Input
  (if Start
    (`/Engine/EditorBlueprintResources/StandardMacros.IsValid` _currentconnectedpawn
      (:`Is Valid`
        (`/Game/ParallelBeam/Core/BPs/Components/BP_PawnPossesion.SVR_RequestExit` _currentconnectedpawn))
      (:`Is Not Valid`
        (message `/Game/ParallelBeam/Core/BPs/Interfaces/BPI_Interaction.StartInteract` Actor (`self.As Character`))))
    (else
      (message `/Game/ParallelBeam/Core/BPs/Interfaces/BPI_Interaction.StopInteract` Actor))))

(event `Interact`
  (params (Start :type Boolean))
  ;[0 0 0] Interaction Input
  (`self.SVR_Interact` Start (`self.InteractionActor`)))

(fn `CalculateDropTransform`
  (params (InItem :type "Actor Object Reference") (InDistance :type "Float (single-precision)"))
  (returns (ReturnValue :type "Transform Structure"))
  (bind _returnvalue (`Actor.K2_GetActorLocation` (`self.As Character`)))
  (bind _returnvalue_location (`KismetMathLibrary.BreakTransform` (`parent.CalculateDropTransform` (`local.InItem`) (`local.InDistance`))))
  (bind _returnvalue_2 (+ (+ (* (`KismetMathLibrary.GetForwardVector` (`KismetMathLibrary.ComposeRotators` (`Actor.K2_GetActorRotation` (`self.As Character`)) (`KismetMathLibrary.MakeRotator` 0.0 (`KismetMathLibrary.RandomFloatInRange` -45.0 45.0) (`KismetMathLibrary.RandomFloatInRange` -45.0 45.0)))) InDistance) _returnvalue) (0.0 0.0 -200.0)))
  (bind _outhit (`KismetSystemLibrary.BoxTraceSingleForObjects` (+ _returnvalue (0.0 0.0 0.0)) _returnvalue_2 (5.0 5.0 5.0) (`Actor.K2_GetActorRotation` InItem) (`|MakeArray` "ObjectTypeQuery1" "ObjectTypeQuery2" :!type "EObjectTypeQuery Enum")))
  (bind (_bblockinghit _binitialoverlap _time _distance _location _impactpoint) (`GameplayStatics.BreakHitResult` _outhit))
  (bind _returnvalue_3 (+ (select `bool` _bblockinghit :`false` _returnvalue_2 :`true` (- _impactpoint (* (`KismetMathLibrary.GetForwardVector` (`Pawn.GetControlRotation` (`self.As Character`))) 20.0))) (0.0 0.0 90.0)))
  (bind _outhit_2 (`KismetSystemLibrary.LineTraceSingleForObjects` _returnvalue_3 (- _returnvalue_3 (0.0 0.0 300.0)) (`|MakeArray` "ObjectTypeQuery1" "ObjectTypeQuery2" :!type "EObjectTypeQuery Enum")))
  (bind (_bblockinghit_2 _binitialoverlap_2 _time_2 _distance_2 _location_2 _impactpoint_2) (`GameplayStatics.BreakHitResult` _outhit_2))
  (return (`KismetMathLibrary.MakeTransform` (+ (select `bool` _bblockinghit_2 :`false` (- _returnvalue_location (`KismetMathLibrary.MakeVector` 0.0 0.0 (`CapsuleComponent.GetScaledCapsuleHalfHeight` (`Character.CapsuleComponent` (`self.As Character`))))) :`true` _impactpoint_2) (`KismetMathLibrary.MakeVector` 0.0 0.0 (.z (- (`Actor.K2_GetActorLocation` InItem) (`SceneComponent.GetSocketLocation` (`|GetArrayItem` (`Actor.GetComponentsByTag` InItem "/Script/Engine.PrimitiveComponent" "MainMesh")) "BottomPoint"))))) (`KismetMathLibrary.MakeRotator` 0.0 0.0 (`KismetMathLibrary.RandomFloatInRange` 0.0 360.0)))))

(fn `Change Action State`
  (params (ActionTag :type "GameplayTag Structure") (Add :type Boolean))
  (returns (Blocked :type Boolean))
  (locals (NewLocalVar :type Boolean :default false))
  (bind _actiontag (`local.ActionTag`))
  (bind _actiontag_2 (`local.ActionTag`))
  (bind (_value _returnvalue) (`BlueprintMapLibrary.Map_Find` (`self.BusyConditions`) ActionTag))
  (bind (_blockusagein _undostates) (break `/Game/ParallelBeam/Core/BPs/Data/Structures/S_BusyCondition` _value))
  (if Add
    (if _returnvalue
      (if (`BlueprintGameplayTagLibrary.HasAnyTags` (`self.ActionStates`) _blockusagein)
        (return true)
        (else
          (for _array_element (`BlueprintGameplayTagLibrary.BreakGameplayTagContainer` _undostates)
            (if (`BlueprintGameplayTagLibrary.HasTag` (`self.ActionStates`) _array_element)
              (`self.Change Action State` _array_element))))))
    (`BlueprintGameplayTagLibrary.AddGameplayTag` (`self.ActionStates`) _actiontag)
    (`self.OnActionStatesChanged` _actiontag)
    (return false)
    (elif (`BlueprintGameplayTagLibrary.HasTag` (`self.ActionStates`) _actiontag_2)
      (`BlueprintGameplayTagLibrary.RemoveGameplayTag` (`self.ActionStates`) _actiontag_2)
      (`self.OnActionStatesChanged` (struct) _actiontag_2)
      (return false))))

(fn `CheckInventoryStorage`
  (params (Item :type "Actor Object Reference") (UpdateType :type "EAGR_ItemUpdateType Enum" :default "PickedUp"))
  (locals (Loc_SlotsUsed :type "Array of GameplayTag Structure") (Loc_rightHandWep :type "AGR_ItemComponent Object Reference"))
  (bind _returnvalue (`self.GetItemInSlot` (struct :`TagName` "CharacterSlots.LeftHand")))
  (bind _returnvalue_2 (`self.GetItemInSlot` (struct :`TagName` "CharacterSlots.RightHand")))
  (bind _returnvalue_3 (`self.GetItemInSlot` (struct :`TagName` "CharacterSlots.LeftHand")))
  (bind _returnvalue_4 (`self.GetItemInSlot` (struct :`TagName` "CharacterSlots.RightHand")))
  (bind _returnvalue_5 (`AGR_InventoryFunctionLibrary.GetItemComponent` (`local.Item`)))
  (bind (_returnvalue_location _returnvalue_rotation) (`KismetMathLibrary.BreakTransform` (`self.CalculateDropTransform` (`self.GetOwner` (`local.Loc_rightHandWep`)) 250.0)))
  (switch `EAGR_ItemUpdateType` UpdateType
    (:`PickedUp`
      (`Actor.SetLifeSpan` Item 0.0)
      (if (`AGR_ItemComponent.bIsStackable` _returnvalue_5)
        (bind _returnvalue_6 (`self.GetAllItemsByName` (`AGR_ItemComponent.ItemName` _returnvalue_5)))
        (for _array_element _returnvalue_6
          (bind _returnvalue_7 (`AGR_InventoryFunctionLibrary.GetItemComponent` _array_element))
          (bind _returnvalue_8 (+ (`AGR_ItemComponent.GetStackCount` _returnvalue_7) (`AGR_ItemComponent.GetStackCount` _returnvalue_5)))
          (bind _maxstackcount (`AGR_ItemComponent.MaxStackCount` _returnvalue_7))
          (`AGR_ItemComponent.SetStackCount` _returnvalue_7 (`KismetMathLibrary.ClampInt64` _returnvalue_8 0 _maxstackcount))
          (bind _returnvalue_9 (- _returnvalue_8 _maxstackcount))
          (if (> _returnvalue_9 0)
            (`AGR_ItemComponent.SetStackCount` _returnvalue_5 _returnvalue_9)
            (else
              (`AGR_ItemComponent.DestroyItem` _returnvalue_7 self)))))
      (if (== (`AGR_ItemComponent.ItemType` (`AGR_InventoryFunctionLibrary.GetItemComponent` (`local.Item`))) (struct :`TagName` "Item.Weapons"))
        (`/Engine/EditorBlueprintResources/StandardMacros.IsValid` _returnvalue_4
          (:`Is Valid`
            (set `local.Loc_rightHandWep` (`AGR_InventoryFunctionLibrary.GetItemComponent` _returnvalue_4))
            (`|ExecutionSequence`
              (:`then_0`
                (bind _keys (`BlueprintMapLibrary.Map_Keys` (`self.ActiveEquipmentSlotsMap`)))
                (for _array_element_2 _keys
                  (if (== (`self.GetItemInSlot` _array_element_2) (`self.GetItemInSlot` (struct :`TagName` "CharacterSlots.RightHand")))
                    (`KismetArrayLibrary.Array_Add` (`local.Loc_SlotsUsed`) _array_element_2)))
                (for _array_element_3 (`local.Loc_SlotsUsed`)
                  (`AGR_ItemComponent.EquipItem` (`AGR_InventoryFunctionLibrary.GetItemComponent` (`local.Item`)) self _array_element_3 true)))
              (:`then_1`
                (`AGR_ItemComponent.DropItem` (`local.Loc_rightHandWep`) self _returnvalue_location _returnvalue_rotation true)
                (`/Engine/EditorBlueprintResources/StandardMacros.IsValid` _returnvalue_3
                  (:`Is Valid`
                    (`AGR_ItemComponent.DropItem` (`AGR_InventoryFunctionLibrary.GetItemComponent` _returnvalue_3) self _returnvalue_location _returnvalue_rotation true)))))))
        (else
          (bind (_tag _equipinall) (message `/Game/ParallelBeam/Core/BPs/Interfaces/BPI_Item.GetEquipmentSlots` (`local.Item`)))
          (bind _gameplaytags (`BlueprintGameplayTagLibrary.BreakGameplayTagContainer` _tag))
          (if (`KismetArrayLibrary.Array_IsNotEmpty` _gameplaytags)
            (for _array_element_4 _gameplaytags
              (if _equipinall
                (`AGR_ItemComponent.EquipItem` (`AGR_InventoryFunctionLibrary.GetItemComponent` (`local.Item`)) self _array_element_4 false)
                (elif (not (`KismetSystemLibrary.IsValid` (`self.GetItemInSlot` _array_element_4)))
                  (bind _boutsuccess (`AGR_ItemComponent.EquipItem` (`AGR_InventoryFunctionLibrary.GetItemComponent` (`local.Item`)) self _array_element_4 false))
                  (if _boutsuccess
                    (return)))))
            (`AGR_ItemComponent.EquipItem` (`AGR_InventoryFunctionLibrary.GetItemComponent` (`local.Item`)) self (`|GetArrayItem` _gameplaytags) false)))))
    (:`Equipped`
      (`|ExecutionSequence` :!label _label
        (:`then_1`
          ;[0 0 0] Unequip left hand item is Right hand item dont allow it
          (`/Engine/EditorBlueprintResources/StandardMacros.IsValid` _returnvalue
            (:`Is Valid`
              (`/Engine/EditorBlueprintResources/StandardMacros.IsValid` _returnvalue_2
                (:`Is Valid`
                  (bind _return_value (message `/Game/ParallelBeam/Core/BPs/Interfaces/BPI_Weapon.GetIsSingleHanded` _returnvalue))
                  (bind _return_value_2 (message `/Game/ParallelBeam/Core/BPs/Interfaces/BPI_Weapon.GetIsSingleHanded` _returnvalue_2))
                  (if (not (and _return_value_2 _return_value))
                    (`AGR_ItemComponent.UnequipItem` (`AGR_InventoryFunctionLibrary.GetItemComponent` (`self.GetItemInSlot` (struct :`TagName` "CharacterSlots.LeftHand"))) self (struct :`TagName` "CharacterSlots.LeftHand") :!label _label_2)))
                (:`Is Not Valid`
                  (goto _label_2))))))))
    (:`Unequipped`
      (if (== (`AGR_ItemComponent.ItemType` (`AGR_InventoryFunctionLibrary.GetItemComponent` (`local.Item`))) (struct :`TagName` "Item.Weapons"))
        (goto _label)))))

(fn `DropItemsOnDeath`
  (bind (_equipmentstodrop _itemstagstodrop) (message `/Game/ParallelBeam/Core/BPs/Interfaces/BPI_Gamemode.GetDroppableItems` (`GameplayStatics.GetGameMode`)))
  (for _array_element (`BlueprintGameplayTagLibrary.BreakGameplayTagContainer` _equipmentstodrop)
    (bind _returnvalue (`self.GetItemInSlot` _array_element))
    (`/Engine/EditorBlueprintResources/StandardMacros.IsValid` _returnvalue
      (:`Is Valid`
        (bind (_returnvalue_location _returnvalue_rotation) (`KismetMathLibrary.BreakTransform` (`self.CalculateDropTransform` _returnvalue (`KismetMathLibrary.RandomFloatInRange` 300.0 450.0))))
        (`AGR_ItemComponent.DropItem` (`AGR_InventoryFunctionLibrary.GetItemComponent` _returnvalue) self _returnvalue_location _returnvalue_rotation true))))
  (for _array_element_2 _itemstagstodrop
    (bind _returnvalue_2 (`self.GetAllItemsByName` _array_element_2))
    (for _array_element_3 _returnvalue_2
      (bind (_returnvalue_location_2 _returnvalue_rotation_2) (`KismetMathLibrary.BreakTransform` (`self.CalculateDropTransform` _array_element_3 (`KismetMathLibrary.RandomFloatInRange` 300.0 450.0))))
      (`AGR_ItemComponent.DropItem` (`AGR_InventoryFunctionLibrary.GetItemComponent` _array_element_3) self _returnvalue_location_2 _returnvalue_rotation_2 true))))

(fn `InteractionTraces`
  (bind _returnvalue (`Pawn.GetController` (`self.As Character`)))
  (bind (_location _rotation) (`Controller.GetPlayerViewPoint` _returnvalue))
  (`/Game/ParallelBeam/Core/BPs/Components/BP_MSK_Locomotion.AttachToComponent` (`self.LocomotionComponent`)
    (:`then`
      (message `/Game/ParallelBeam/Core/BPs/Interfaces/BPI_HUD.SetInteractionText` (`/Game/ParallelBeam/Core/BPs/FunctionLib/BFL_MSK.GetMSK_HUD` (`self.As Character`)) null :!label _label))
    (:`else`
      (`/Engine/EditorBlueprintResources/StandardMacros.IsValid` _returnvalue
        (:`Is Valid`
          (bind (_outhit _returnvalue_2) (`KismetSystemLibrary.SphereTraceSingle` _location (+ (* (`KismetMathLibrary.GetForwardVector` _rotation) (`BlueprintMapLibrary.Map_Find` (`self.InteractionRange`) (`/Game/ParallelBeam/Core/BPs/Components/BP_MSK_Locomotion.CameraType` (`self.LocomotionComponent`)))) _location) 5.0 "TraceTypeQuery4" false (`self.GetAllEquippedItems`)))
          (if _returnvalue_2
            (bind (_bblockinghit _binitialoverlap _time _distance _location_2 _impactpoint _normal _impactnormal _physmat _hitactor) (`GameplayStatics.BreakHitResult` _outhit))
            (if (`KismetSystemLibrary.DoesImplementInterface` _hitactor "/Game/ParallelBeam/Core/BPs/Interfaces/BPI_Interaction.BPI_Interaction_C")
              (if (!= _hitactor (`self.InteractionActor`))
                (bind _return_value (message `/Game/ParallelBeam/Core/BPs/Interfaces/BPI_Interaction.CanInteract` _hitactor (`self.GetOwner`)))
                (if _return_value
                  (set `self.InteractionActor` _hitactor)
                  (else
                    (set `self.InteractionActor` null :!label _label_2)))
                (message `/Game/ParallelBeam/Core/BPs/Interfaces/BPI_HUD.SetInteractionText` (`/Game/ParallelBeam/Core/BPs/FunctionLib/BFL_MSK.GetMSK_HUD` (`self.As Character`)) (`self.InteractionActor`)))
              (else
                (if (!= (`self.InteractionActor`) null) :!label _label_3
                  (goto _label_2))))
            (else
              (goto _label_3))))
        (:`Is Not Valid`
          (goto _label))))))

(fn `Reload`
  (locals (LOC_RightWep :type "Actor Object Reference") (LOCLeftWep :type "Actor Object Reference"))
  (bind _returnvalue (`self.GetItemInSlot` (struct :`TagName` "CharacterSlots.RightHand")))
  (bind _blocked (`self.Change Action State` (struct :`TagName` "States.Reloading") true))
  (if (not _blocked)
    (`|ExecutionSequence`
      (:`then_0`
        (set `local.LOC_RightWep` _returnvalue)
        (`AGR_ProjectileLauncherComponent.SV_EndFire` (`AGR_ProjectileFunctionLibrary.GetProjectileLauncherComponent` _returnvalue))
        (if (`/Game/ParallelBeam/Core/BPs/Components/BP_MSK_Locomotion.IsDuelWelding` (`self.LocomotionComponent`))
          (set `local.LOCLeftWep` (`self.GetItemInSlot` (struct :`TagName` "CharacterSlots.LeftHand")))
          (`AGR_ProjectileLauncherComponent.SV_EndFire` (`AGR_ProjectileFunctionLibrary.GetProjectileLauncherComponent` (`local.LOCLeftWep`)))))
      (:`then_1`
        (bind _return_value (message `/Game/ParallelBeam/Core/BPs/Interfaces/BPI_Weapon.Reload` (`local.LOC_RightWep`)))
        (bind _locleftwep (`local.LOCLeftWep`)
          (:`then`
            (bind _return_value_2 (message `/Game/ParallelBeam/Core/BPs/Interfaces/BPI_Weapon.Reload` _locleftwep))
            (if (not _return_value_2)
              (`self.Change Action State` (struct :`TagName` "States.Reloading") :!label _label)))
          (:`else`
            (if (not _return_value)
              (goto _label))))))))