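; Inventory component for weapon attachments that spawns and equips them, including attachments mounted on other attachments through their own nested inventories.
; On server BeginPlay it fills empty slots with a random allowed set (flag inherited from any parent inventory) or puts stock attachments in compulsory slots.
; Equipment changes re-run that compulsory-slot refill after a retriggerable delay and broadcast an effect update.
; Adding checks the allowed list, reuses stored items and recurses into child inventories, as does gathering all attachments.
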(event `self.ReceiveBeginPlay`
  ;[0 0 0] Runs on Server only
  (`/Engine/EditorBlueprintResources/ActorComponentMacros.Switch Has Authority`
    (:`Authority`
      (`self.RandomizeAttachments`)
      (add `self.OnEquipmentSlotUpdated` (`|CreateDelegate` :!event `OnEquipmentUpdated`))
      (if (`self.RandomizeAttachmentsOnSpawn`)
        ;[0 0 0] Initial spawning of random attachments
        (`KismetSystemLibrary.RetriggerableDelay` (`GameplayStatics.GetWorldDeltaSeconds`))
        (bind _keys (`BlueprintMapLibrary.Map_Keys` (`self.ActiveEquipmentSlotsMap`)))
        (for _array_element _keys
          (`/Engine/EditorBlueprintResources/StandardMacros.IsValid` (`self.GetItemInSlot` _array_element)
            (:`Is Not Valid`
              (for _array_element_2 (`self.StartUpAttachments`)
                (if (`BlueprintGameplayTagLibrary.HasTag` (`/Game/ParallelBeam/Core/BPs/Data/DTA_Attachment.EquipSlot` _array_element_2) _array_element)
                  (bind _class (`|LoadAssetClass` (`/Game/ParallelBeam/Core/BPs/Data/DTA_Attachment.ActorRef` _array_element_2))
                    (:`then`
                      (break))
                    (:`Completed`
                      (`self.AddAttachment` _class))))))))
        (else
          ;[0 0 0] when any equipment change happnes we basicall do a refresh for all attachments to see if any of them needs to be removed or added
          (`KismetSystemLibrary.RetriggerableDelay` (* (`GameplayStatics.GetWorldDeltaSeconds`) 1.0) :!label _label)
          (bind _keys_2 (`BlueprintMapLibrary.Map_Keys` (`self.ActiveEquipmentSlotsMap`)))
          (for _array_element_3 _keys_2
            (if (`BlueprintGameplayTagLibrary.HasTag` (`self.CompulsorySlots`) _array_element_3)
              (`/Engine/EditorBlueprintResources/StandardMacros.IsValid` (`self.GetItemInSlot` _array_element_3)
                (:`Is Not Valid`
                  (for _array_element_4 (`self.StockAttachments`)
                    (if (`BlueprintGameplayTagLibrary.HasTag` (`/Game/ParallelBeam/Core/BPs/Data/DTA_Attachment.EquipSlot` _array_element_4) _array_element_3)
                      (bind _class_2 (`|LoadAssetClass` (`/Game/ParallelBeam/Core/BPs/Data/DTA_Attachment.ActorRef` _array_element_4))
                        (:`then`
                          (break))
                        (:`Completed`
                          (`self.AddAttachment` _class_2))))))))))))))

(event `OnEquipmentUpdated` :!signature `self.OnEquipmentSlotUpdated`
  (params (Item :type "Actor Object Reference") (SlotAction :type "EAGR_EquipmentSlotAction Enum" :default "Set") (Slot :type "GameplayTag Structure (by ref)"))
  ;[0 0 0] when any equipment change happnes we basicall do a refresh for all attachments to see if any of them needs to be removed or added
  (`|ExecutionSequence`
    (:`then_0`
      (goto _label))
    (:`then_1`
      (`KismetSystemLibrary.RetriggerableDelay` (* (`GameplayStatics.GetWorldDeltaSeconds`) 1.0))
      (`self.AttachmentEffectUpdated`))))

(fn `AddAttachment`
  (params (Class :type "Object Class Reference"))
  (returns (Output :type "Actor Object Reference"))
  (locals (LOC_RefActor :type "Actor Object Reference"))
  (bind _returnvalue (`self.GetOwner`))
  (bind _loc_refactor (`local.LOC_RefActor`))
  ;[0 0 0] Making sure this attachment is for this weapon
  (bind _asactor (castclass `Actor` Class))
  (for _array_element (`self.AllowedAttachments`)
    (if (== (`|ConvertAsset` _asactor) (`/Game/ParallelBeam/Core/BPs/Data/DTA_Attachment.ActorRef` _array_element))
      ;[0 0 0] Spawn and equip attachment, if already in inventory storage then equip it directly to all slots
      (bind _returnvalue_2 (`self.GetAllItemsByClass` _asactor))
      (if (`KismetArrayLibrary.Array_IsEmpty` _returnvalue_2)
        (bind _returnvalue_3 (`|SpawnActorFromClass` _asactor (`KismetMathLibrary.MakeTransform` (0.0 0.0 0.0)) "AlwaysSpawn" "MultiplyWithRoot" _returnvalue (`Actor.GetInstigator` _returnvalue)))
        (set `local.LOC_RefActor` _returnvalue_3)
        (else
          (set `local.LOC_RefActor` (`|GetArrayItem` _returnvalue_2))))
      ;;[1 1 1] Equip item in all the Equip slots ( for the items that take more then 1 slo
      (bind _slot (message `/Game/ParallelBeam/Core/BPs/Interfaces/BPI_Attachment.GetAttachSlot` (`local.LOC_RefActor`)))
      (for _array_element_2 (`BlueprintGameplayTagLibrary.BreakGameplayTagContainer` _slot)
        (`/Engine/EditorBlueprintResources/StandardMacros.IsValid` _loc_refactor
          (:`Is Valid`
            (`AGR_ItemComponent.EquipItem` (`AGR_InventoryFunctionLibrary.GetItemComponent` _loc_refactor) self _array_element_2 true))))
      (return (`local.LOC_RefActor`))))
  ;[0 0 0] If not for this weapon then check if attachment is for one of the Equiped items on this weapon
  (for _array_element_3 (`self.GetAllEquippedItems`)
    (bind (_attachment_inventory _returnvalue_4) (`/Game/ParallelBeam/Core/BPs/FunctionLib/BFL_MSK.GetAttachmentInventory` _array_element_3))
    (if _returnvalue_4
      (bind _output (`self.AddAttachment` _attachment_inventory (`local.Class`)))
      (return _output))))

(fn `FindOwnerWeapon`
  (returns (Weapon :type "Actor Object Reference"))
  (locals (LOC_PossibleWeapon :type "Actor Object Reference"))
  ;[1 1 1] Loops till it finds the weapon this attachment is attached to
  ; Kinda risky but as long as u dont attach weapon to smth that isnt a weapon its fine
  (set `local.LOC_PossibleWeapon` (`self.GetOwner`))
  (if (`KismetSystemLibrary.DoesImplementInterface` (`local.LOC_PossibleWeapon`) "/Game/ParallelBeam/Core/BPs/Interfaces/BPI_Weapon.BPI_Weapon_C") :!label _label
    (return (`local.LOC_PossibleWeapon`))
    (else
      (set `local.LOC_PossibleWeapon` (`Actor.GetOwner` (`local.LOC_PossibleWeapon`)))
      (goto _label))))

(fn `GetAllAttachments`
  (returns (`Return Value` :type "Array of Actor Object Reference"))
  (locals (LOC_SourceArray :type "Array of Actor Object Reference"))
  (bind _loc_sourcearray (`local.LOC_SourceArray`))
  ;[1 1 1] Finds all the attachments that are part of this inventory
  ; including the attachments on top of attachments
  ; its a recursive funtion
  (for _array_element (`self.GetAllEquippedItems`)
    (`KismetArrayLibrary.Array_AddUnique` (`local.LOC_SourceArray`) _array_element)
    (bind (_attachment_inventory _returnvalue) (`/Game/ParallelBeam/Core/BPs/FunctionLib/BFL_MSK.GetAttachmentInventory` _array_element))
    (if _returnvalue
      (bind _return_value (`self.GetAllAttachments` _attachment_inventory))
      (`KismetArrayLibrary.Array_Append` (`local.LOC_SourceArray`) _return_value)))
  (set `self.AllAttachments` _loc_sourcearray)
  (return _loc_sourcearray))

(fn `GetAllAttachmentsByClass`
  (params (Class :type "Actor Class Reference"))
  (returns (`Return Value` :type "Array of Actor Object Reference"))
  (locals (LOC_SourceArray :type "Array of Actor Object Reference") (LOC_Final :type "Array of Actor Object Reference"))
  ;[1 1 1] Same as Get All Attachments but we can filter out a class specific
  ; useed when loading attachments for weapons that are not directly applied on weapon
  (for _array_element (`self.GetAllEquippedItems`)
    (`KismetArrayLibrary.Array_AddUnique` (`local.LOC_SourceArray`) _array_element)
    (bind (_attachment_inventory _returnvalue) (`/Game/ParallelBeam/Core/BPs/FunctionLib/BFL_MSK.GetAttachmentInventory` _array_element))
    (if _returnvalue
      (bind _return_value (`self.GetAllAttachments` _attachment_inventory))
      (`KismetArrayLibrary.Array_Append` (`local.LOC_SourceArray`) _return_value)))
  (for _array_element_2 (`local.LOC_SourceArray`)
    (if (== (`GameplayStatics.GetObjectClass` _array_element_2) (`local.Class`))
      (`KismetArrayLibrary.Array_AddUnique` (`local.LOC_Final`) _array_element_2)))
  (return (`local.LOC_Final`)))

(fn `RandomizeAttachments`
  (locals (Loc_StockAttachments :type "Array of /Game/ParallelBeam/Core/BPs/Data/DTA_Attachment Object Reference") (Loc_RandomAttachments :type "Array of /Game/ParallelBeam/Core/BPs/Data/DTA_Attachment Object Reference") (`FoundAttachment?` :type Boolean))
  (bind (_attachment_inventory _returnvalue) (`/Game/ParallelBeam/Core/BPs/FunctionLib/BFL_MSK.GetAttachmentInventory` (`Actor.GetOwner` (`self.GetOwner`))))
  (`|ExecutionSequence`
    (:`then_0`
      (if _returnvalue
        (set `self.RandomizeAttachmentsOnSpawn` (`/Game/ParallelBeam/Core/BPs/Components/BP_AttachmentInventory.RandomizeAttachmentsOnSpawn` _attachment_inventory))))
    (:`then_1`
      (if (`self.RandomizeAttachmentsOnSpawn`)
        (set `local.Loc_StockAttachments` (`self.StockAttachments`))
        ;[0 0 0] Adding Random Attachments
        (for _ (range (+ (`KismetArrayLibrary.Array_Length` (`self.AllowedAttachments`)) 1))
          (`KismetArrayLibrary.Array_AddUnique` (`self.StartUpAttachments`) (`KismetArrayLibrary.Array_Random` (`self.AllowedAttachments`))))
        (for _array_element (`BlueprintGameplayTagLibrary.BreakGameplayTagContainer` (`self.CompulsorySlots`))
          (set `local.FoundAttachment?` false)
          (for _array_element_2 (`self.StockAttachments`)
            (if (`BlueprintGameplayTagLibrary.HasTag` (`/Game/ParallelBeam/Core/BPs/Data/DTA_Attachment.EquipSlot` _array_element_2) _array_element)
              (set `local.FoundAttachment?` true)
              (break)))
          (if (not (`local.FoundAttachment?`))
            (for _array_element_3 (`local.Loc_StockAttachments`)
              (if (`BlueprintGameplayTagLibrary.HasTag` (`/Game/ParallelBeam/Core/BPs/Data/DTA_Attachment.EquipSlot` _array_element_3) _array_element)
                (`KismetArrayLibrary.Array_AddUnique` (`self.StartUpAttachments`) _array_element_3)
                (break)))))
        (else
          (set `self.StartUpAttachments` (`self.StockAttachments`)))))))

(fn `RemoveAttachFromSlot`
  (params (Slot :type "GameplayTag Structure"))
  (locals (Loc_ItemToUnequip :type "Actor Object Reference"))
  (bind _returnvalue (`self.GetItemInSlot` Slot))
  (`/Engine/EditorBlueprintResources/StandardMacros.IsValid` _returnvalue
    (:`Is Valid`
      (set `local.Loc_ItemToUnequip` _returnvalue)
      (bind _keys (`BlueprintMapLibrary.Map_Keys` (`self.ActiveEquipmentSlotsMap`)))
      (for _array_element _keys
        (if (== (`self.GetItemInSlot` _array_element) (`local.Loc_ItemToUnequip`))
          (`AGR_ItemComponent.UnequipItem` (`AGR_InventoryFunctionLibrary.GetItemComponent` _returnvalue) self (`local.Slot`)))))))