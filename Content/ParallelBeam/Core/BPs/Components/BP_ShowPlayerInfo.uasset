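; Player controller component that reveals info widgets over pawns the local player looks at, destroying itself on non-local controllers.
; Each tick, a sphere trace along the view finds world depth, setting the length of a box trace for pawns and vehicles that ignores the view target.
; Hit pawns pass a line-trace occlusion check back to the viewpoint before Show is called on their BP_PawnInfo3dWidget component.
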(event `self.ReceiveBeginPlay`
  (bind _asplayer_controller (cast `PlayerController` (`self.GetOwner`)))
  (bind _output_get (set `self.As Player Controller` _asplayer_controller))
  (if (not (`Controller.IsLocalPlayerController` _output_get))
    (`self.K2_DestroyComponent`)))

(event `self.ReceiveTick`
  (params (DeltaSeconds :type "Float (single-precision)"))
  (bind _actorstoshow (`self.CheckingPlayersTo show info`))
  (for _array_element _actorstoshow
    (bind _returnvalue (`Actor.GetComponentByClass` _array_element "/Game/ParallelBeam/Core/BPs/Components/BP_PawnInfo3dWidget.BP_PawnInfo3dWidget_C"))
    (`/Engine/EditorBlueprintResources/StandardMacros.IsValid` _returnvalue
      (:`Is Valid`
        (`/Game/ParallelBeam/Core/BPs/Components/BP_PawnInfo3dWidget.Show` _returnvalue)))))

(fn `CheckingPlayersTo show info`
  (returns (ActorsToShow :type "Array of Actor Object Reference"))
  (locals (LOC_ActorHits :type "Array of Actor Object Reference") (SelfPawn :type "Actor Object Reference") (LOC_ActorsToShow :type "Array of Actor Object Reference"))
  (bind _as_player_controller (`self.As Player Controller`))
  (bind (_location _rotation) (`Controller.GetPlayerViewPoint` _as_player_controller))
  (bind _returnvalue (`Controller.GetViewTarget` _as_player_controller))
  (bind _returnvalue_2 (`KismetMathLibrary.GetForwardVector` _rotation))
  (bind _array (`|MakeArray` _returnvalue))
  (set `local.SelfPawn` _returnvalue)
  (`/Engine/EditorBlueprintResources/StandardMacros.IsValid` _returnvalue
    (:`Is Valid`
      (bind _outhit (`KismetSystemLibrary.SphereTraceSingleForObjects` _location (+ _location (* _returnvalue_2 500000.0)) 50.0 (`|MakeArray` "ObjectTypeQuery1" "ObjectTypeQuery2" :!type "EObjectTypeQuery Enum") false _array))
      (bind _outhits (`KismetSystemLibrary.BoxTraceMultiForObjects` _location (+ _location (* _returnvalue_2 (+ (`.Distance` (`GameplayStatics.BreakHitResult` _outhit)) 500.0))) (150.0 100.0 20.0) _rotation (`|MakeArray` "ObjectTypeQuery3" "ObjectTypeQuery5" :!type "EObjectTypeQuery Enum") false _array))
      (for _array_element _outhits
        (bind (_bblockinghit _binitialoverlap _time _distance _location_2 _impactpoint _normal _impactnormal _physmat _hitactor) (`GameplayStatics.BreakHitResult` _array_element))
        (cast `Pawn` _hitactor)
        (bind _outhit_2 (`KismetSystemLibrary.LineTraceSingleForObjects` _location_2 (`Controller.GetPlayerViewPoint` (`self.As Player Controller`)) (`|MakeArray` "ObjectTypeQuery1" "ObjectTypeQuery2" :!type "EObjectTypeQuery Enum") false (`|MakeArray` (`local.SelfPawn`) _hitactor)))
        (if (not (`GameplayStatics.BreakHitResult` _outhit_2))
          (`KismetArrayLibrary.Array_Add` (`local.LOC_ActorsToShow`) _hitactor)))
      (return (`local.LOC_ActorsToShow`)))
    (:`Is Not Valid`
      (return (`local.LOC_ActorsToShow`)))))