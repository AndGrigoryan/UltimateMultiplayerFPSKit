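; Player state component that tracks a player's kill and death stats, squad membership and match-facing UI events.
; It keeps server-side totals plus client-side per-opponent kill maps for spectator display.
; Kill feed and match-end events forward to the owning controller's HUD, with match end also removing the character input mapping.
; RepNotifies broadcast pawn and squad updates, assigning each squadmate a colour by index.
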(event `self.ReceiveBeginPlay`
  (bind _asplayer_state (cast `PlayerState` (`self.GetOwner`)))
  (set `self.As Player State` _asplayer_state))

(event `AddPersonalKill`
  (params (Killed :type "UniqueNetIdRepl Structure (by ref)"))
  (bind _personalkills (`self.PersonalKills`))
  ;[0 0 0] Client Side Score of which enemy u killed and how many times they killed u ( used in spectator menu and in future for more complicated scores like comaback and revenge stuff)
  (`BlueprintMapLibrary.Map_Add` _personalkills Killed (+ (`BlueprintMapLibrary.Map_Find` _personalkills Killed) 1)))

(event `AddEnemyKill`
  (params (Killer :type "UniqueNetIdRepl Structure (by ref)"))
  (bind _enemykills (`self.EnemyKills`))
  ;[0 0 0] Client Side Score of which enemy u killed and how many times they killed u ( used in spectator menu and in future for more complicated scores like comaback and revenge stuff)
  (`BlueprintMapLibrary.Map_Add` _enemykills Killer (+ (`BlueprintMapLibrary.Map_Find` _enemykills Killer) 1)))

(event `AddDeath`
  ;[0 0 0] Add Kills and deaths SERVER ONLY
  (`/Engine/EditorBlueprintResources/StandardMacros.IncrementInt` (`self.TotalDeaths`)))

(event `AddKill`
  ;[0 0 0] Add Kills and deaths SERVER ONLY
  (`/Engine/EditorBlueprintResources/StandardMacros.IncrementInt` (`self.TotalKills`)))

(event `AddKillFeedMessage`
  (params (Killer :type "PlayerState Object Reference") (Killed :type "PlayerState Object Reference") (DamageCauser :type "Actor Object Reference"))
  (bind _returnvalue (`PlayerState.GetPlayerController` (`self.As Player State`)))
  ;[0 0 0] Adding the Kill feed Message
  (`/Engine/EditorBlueprintResources/StandardMacros.IsValid` _returnvalue
    (:`Is Valid`
      (message `/Game/ParallelBeam/Core/BPs/Interfaces/BPI_HUD.AddKillFeedElement` (`PlayerController.GetHUD` _returnvalue) Killer Killed DamageCauser))))

(event `MatchEnded`
  (params (Win :type Boolean) (Draw :type Boolean))
  (bind _returnvalue (`PlayerState.GetPlayerController` (`self.As Player State`)))
  ;[0 0 0] On Match ended show the screen and remove the inputs
  (`/Engine/EditorBlueprintResources/StandardMacros.IsValid` _returnvalue
    (:`Is Valid`
      (message `/Game/ParallelBeam/Core/BPs/Interfaces/BPI_HUD.MatchEndScreen` (`PlayerController.GetHUD` _returnvalue) Win Draw)
      (`EnhancedInputSubsystemInterface.RemoveMappingContext` (pcsubsystem `EnhancedInputLocalPlayerSubsystem` _returnvalue) "/Game/ParallelBeam/Core/Inputs/IMC_Character.IMC_Character" (struct)))))

(fn `OnRep_CurrentMainPawn`
  (`self.ControlledPawnUpdated` (`self.CurrentMainPawn`)))

(fn `OnRep_SquadStates`
  (locals (LOC_PlayerStates :type "Array of PlayerState Object Reference"))
  (set `local.LOC_PlayerStates` (`self.SquadStates`))
  (for (_array_element _array_index) (`local.LOC_PlayerStates`)
    (`/Engine/EditorBlueprintResources/StandardMacros.IsValid` _array_element
      (:`Is Valid`
        (bind _return_value (`/Game/ParallelBeam/Core/BPs/FunctionLib/BFL_MSK.GetPlayerStateComponent` _array_element))
        (set `/Game/ParallelBeam/Core/BPs/Components/GameModeComponents/BP_PlayerState_PS_Component.LocalColour` (select `int` _array_index :`0` (struct :`R` 0.791335 :`B` 1.0 :`A` 1.0) :`1` (struct :`G` 0.063502 :`B` 1.0 :`A` 1.0) :`2` (struct :`R` 1.0 :`G` 0.172808 :`A` 1.0) :`3` (struct :`G` 0.853376 :`B` 1.0 :`A` 1.0) :!type "LinearColor Structure") _return_value)
        (set `/Game/ParallelBeam/Core/BPs/Components/GameModeComponents/BP_PlayerState_PS_Component.IsSquadmember` true _return_value))))
  (`self.OnSquadUpdated`))