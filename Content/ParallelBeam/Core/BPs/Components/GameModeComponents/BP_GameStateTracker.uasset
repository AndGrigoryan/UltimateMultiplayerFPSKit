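; Game state component that tracks the match timer, round progress and leading team.
; Tick derives remaining time from a stored start time and replicated server world time, with the authority firing the time-out call.
; EndRound records the winner in RoundHistory, then messages the game mode to reset the round or end the match.
; Team components supply scores and indices for leader lookups, and round RepNotifies broadcast updates.
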(event `SetStartedTime`
  ;[0 0 0] Sets a Started time
  ; We are using it so we can utilize the defaul Server world time that is already replicated in game states
  (set `self.GameStartedTime` (`GameStateBase.GetServerWorldTimeSeconds` (`GameplayStatics.GetGameState`))))

(event `self.ReceiveTick`
  (params (DeltaSeconds :type "Float (single-precision)"))
  ;[0 0 0] Time tracking for game mode , on server initicates game end when time runs out
  (if (== (`self.GameStartedTime`) 0.0)
    (set `self.PendingGameTime` 0.0)
    (else
      (bind _output_get (set `self.PendingGameTime` (`KismetMathLibrary.FClamp` (- (+ (`self.TotalGameTime`) (`self.GameStartedTime`)) (`GameStateBase.GetServerWorldTimeSeconds` (`self.GameState`))) 0.0 (`self.TotalGameTime`))))
      (`/Engine/EditorBlueprintResources/ActorComponentMacros.Switch Has Authority`
        (:`Authority`
          (if (== _output_get 0.0)
            (`self.OnTimeRunOut`)
            (`self.SetComponentTickEnabled` false)))))))

(event `ResetTime`
  (params (NewTime :type "Float (double-precision)"))
  ;[0 0 0] Time tracking for game mode , on server initicates game end when time runs out
  (bind _output_get (set `self.TotalGameTime` NewTime))
  (set `self.PendingGameTime` _output_get)
  (`self.SetStartedTime`)
  (`self.SetComponentTickEnabled` true))

(event `self.ReceiveBeginPlay`
  ;[0 0 0] Setting the parent game state
  (set `self.GameState` (`GameplayStatics.GetGameState`))
  (`/Engine/EditorBlueprintResources/ActorComponentMacros.Switch Has Authority`
    (:`Authority`
      (if (`self.UseRounds`)
        (set `self.TotalGameTime` (`self.RoundTime`))
        (set `self.MaxNumberOfRounds` (- (`self.MaxNumberOfRounds`) 1))
        (set `self.NumberOfRoundsToSwitchSides` (- (`self.NumberOfRoundsToSwitchSides`) 1))
        (for _index (range (+ (`self.MaxNumberOfRounds`) 1))
          (`KismetArrayLibrary.Array_Set` (`self.RoundHistory`) _index -1 true))))))

(event `EndRound`
  (params (WinningTeam :type Integer))
  (bind (_team_index _roundswon) (`self.GetTopRoundWinningTeam`))
  (bind _returnvalue (+ (`self.CurrentRound`) 1))
  (`KismetArrayLibrary.Array_Set` (`self.RoundHistory`) (`self.CurrentRound`) WinningTeam true)
  (`self.SetComponentTickEnabled` false)
  ;[1 1 1] If One of the teams achive the number of required rounds to win then end game with that team as winer
  (if (or (>= _roundswon (`self.NumberOfRoundsToWin`)) (> _returnvalue (`self.MaxNumberOfRounds`)))
    (message `/Game/ParallelBeam/Core/BPs/Interfaces/BPI_Gamemode.Trigger End Match` (`GameplayStatics.GetGameMode`) _team_index)
    (else
      (set `self.CurrentRound` _returnvalue)
      (message `/Game/ParallelBeam/Core/BPs/Interfaces/BPI_Gamemode.ResetRound` (`GameplayStatics.GetGameMode`)))))

(fn `FindMaxScoreTeam`
  (returns (WinningTeamIndex :type Integer) (IsDraw :type Boolean))
  (locals (Loc_HighestScore :type Integer :default 0) (Loc_TeamIndex :type Integer) (Loc_Draw :type Boolean :default true))
  ;[1 1 1] Loops through all the team stat components to find the team with max score
  (for _array_element (`Actor.K2_GetComponentsByClass` (`self.GameState`) "/Game/ParallelBeam/Core/BPs/Components/GameModeComponents/BP_GameStateTeam_Component.BP_GameStateTeam_Component_C")
    (bind _teamscore (`/Game/ParallelBeam/Core/BPs/Components/GameModeComponents/BP_GameStateTeam_Component.TeamScore` _array_element))
    (if (and (> _teamscore 0) (>= _teamscore (`local.Loc_HighestScore`)))
      (set `local.Loc_Draw` false)
      (if (== _teamscore (`local.Loc_HighestScore`))
        (set `local.Loc_Draw` true))
      (set `local.Loc_HighestScore` _teamscore)
      (set `local.Loc_TeamIndex` (`/Game/ParallelBeam/Core/BPs/Components/GameModeComponents/BP_GameStateTeam_Component.TeamIndex` _array_element))))
  (return (`local.Loc_TeamIndex`) (`local.Loc_Draw`)))

(fn `GetRoundWinsForTeam`
  (params (TeamIndex :type Integer))
  (returns (RoundWinCount :type Integer))
  (locals (Loc_WinCount :type Integer))
  (for _array_element (`self.RoundHistory`)
    (if (== _array_element TeamIndex)
      (`/Engine/EditorBlueprintResources/StandardMacros.IncrementInt` (`local.Loc_WinCount`))))
  (return (`local.Loc_WinCount`)))

(fn `GetTopRoundWinningTeam`
  (returns (`Team Index` :type Integer) (RoundsWon :type Integer))
  (locals (Loc_WinCount :type Integer :default 0) (Loc_winingTeamIndex :type Integer :default 0))
  (for _array_element (`Actor.K2_GetComponentsByClass` (`self.GameState`) "/Game/ParallelBeam/Core/BPs/Components/GameModeComponents/BP_GameStateTeam_Component.BP_GameStateTeam_Component_C")
    (bind _teamindex (`/Game/ParallelBeam/Core/BPs/Components/GameModeComponents/BP_GameStateTeam_Component.TeamIndex` _array_element))
    (bind _roundwincount (`self.GetRoundWinsForTeam` _teamindex))
    (if (> _roundwincount (`local.Loc_WinCount`))
      (set `local.Loc_WinCount` _roundwincount)
      (set `local.Loc_winingTeamIndex` _teamindex)))
  (return (`local.Loc_winingTeamIndex`) (`local.Loc_WinCount`)))

(fn `OnRep_CurrentRound`
  (`self.OnRoundUpdated`))

(fn `OnRep_RoundHistory`
  (`self.OnRoundUpdated`))