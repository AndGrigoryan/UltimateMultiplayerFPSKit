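; Game state component that represents one team in a match, tagged with its team index and tracking its players, score and squads.
; New players get the team index, are announced by multicast and fill open squads, with squad components spawned as needed.
; Score is clamped, can end the match at the limit, and its RepNotify informs listeners and the game mode.
; It also relays match results and checks for living, non-spectator players.
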(event `self.ReceiveBeginPlay`
  (`KismetArrayLibrary.Array_Add` (`self.ComponentTags`) (`KismetStringLibrary.Conv_StringToName` (`KismetStringLibrary.Conv_IntToString` (`self.TeamIndex`)))))

(event `AddPlayer`
  (params (PlayerState :type "PlayerState Object Reference (by ref)"))
  (bind _return_value (`/Game/ParallelBeam/Core/BPs/FunctionLib/BFL_MSK.GetPlayerStateComponent` PlayerState))
  ;[0 0 0] Just adding a new player and assigning the team index on them
  (`KismetArrayLibrary.Array_AddUnique` (`self.TeamPlayers`) PlayerState)
  (`self.MLTNewPlayerAdded` PlayerState)
  (set `/Game/ParallelBeam/Core/BPs/Components/GameModeComponents/BP_PlayerState_PS_Component.TeamIndex` (`self.TeamIndex`) _return_value)
  (`KismetArrayLibrary.Array_AddUnique` (`self.PlayerStateComponents`) _return_value)
  (`self.AddPlayerToSquad` PlayerState))

(event `MLTNewPlayerAdded`
  (params (PlayerState :type "PlayerState Object Reference"))
  ;[0 0 0] When a new player is added we tell everone someone joined
  (`self.TeamPlayerAdded` PlayerState))

(event `AddScore`
  (params (Score :type Integer))
  ;[0 0 0] Adding score and if reached score limit then trigger end game
  (set `self.TeamScore` (`KismetMathLibrary.Clamp` (+ Score (`self.TeamScore`)) 0 (`self.MaxScore`)))
  (if (`self.EndGameIfReachMaxScore`)
    (if (== (`self.TeamScore`) (`self.MaxScore`))
      (message `/Game/ParallelBeam/Core/BPs/Interfaces/BPI_Gamemode.Trigger End Match` (`GameplayStatics.GetGameMode`) (`self.TeamIndex`)))))

(event `MatchEnded`
  (params (WiningTeamIndex :type Integer))
  ;[0 0 0] Telling all players match ended
  (`/Game/ParallelBeam/Core/BPs/Components/GameModeComponents/BP_PlayerState_PS_Component.MatchEnded` (`self.PlayerStateComponents`) (== WiningTeamIndex (`self.TeamIndex`)) (== WiningTeamIndex -1)))

(fn `AddPlayerToSquad`
  (params (PlayerState :type "PlayerState Object Reference"))
  (if (> (`self.PlayerSquadLimit`) 1)
    (for _array_element (`self.PlayerSquadComponents`)
      (if (< (`KismetArrayLibrary.Array_Length` (`/Game/ParallelBeam/Core/BPs/Components/GameModeComponents/BP_GameState_SquadComponent.SquadPlayerStates` _array_element)) (`self.PlayerSquadLimit`))
        (`/Game/ParallelBeam/Core/BPs/Components/GameModeComponents/BP_GameState_SquadComponent.AddSquadMember` _array_element PlayerState)
        (return)))
    (bind _returnvalue (`|AddComponentByClass` (`self.GetOwner`) "/Game/ParallelBeam/Core/BPs/Components/GameModeComponents/BP_GameState_SquadComponent.BP_GameState_SquadComponent_C"))
    (bind _returnvalue_2 (`KismetArrayLibrary.Array_Add` (`self.PlayerSquadComponents`) _returnvalue))
    (set `/Game/ParallelBeam/Core/BPs/Components/GameModeComponents/BP_GameState_SquadComponent.SquadID` _returnvalue_2 _returnvalue)
    (`/Game/ParallelBeam/Core/BPs/Components/GameModeComponents/BP_GameState_SquadComponent.AddSquadMember` _returnvalue PlayerState)
    (return)))

(fn `DoesTeamHaveAnyPlayerAlive`
  (returns (`Return Value` :type Boolean))
  (for _array_element (`self.TeamPlayers`)
    (bind _pawnprivate (`PlayerState.PawnPrivate` _array_element))
    (`/Engine/EditorBlueprintResources/StandardMacros.IsValid` _pawnprivate
      (:`Is Valid`
        (if (not (`Actor.ActorHasTag` _pawnprivate "Spectator"))
          (return true)))))
  (return false))

(fn `OnRep_TeamScore`
  (bind _returnvalue (`GameplayStatics.GetGameMode`))
  (`self.TeamScoreUpdated`)
  (`/Engine/EditorBlueprintResources/StandardMacros.IsValid` _returnvalue
    (:`Is Valid`
      (message `/Game/ParallelBeam/Core/BPs/Interfaces/BPI_Gamemode.ScoreUpdated` _returnvalue self))))