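; Controller component that runs the spawn, death and respawn cycle, plus kill and experience tracking.
; A server timer asks the GameMode whether respawn is allowed, while clients get a loadout screen unless auto-spawning.
; Saved loadouts go to the server, which spawns items off-map, restarts the pawn, then equips them and adds ammo.
; Tick turns view toward the killer, and earned experience persists to a PlayerProgress save.
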(event `self.ReceiveBeginPlay`
  ;[0 0 0] On begin play set the defaulty pitch and yaw values And Show the spawn screen
  (`|ExecutionSequence`
    (:`then_0`
      (bind _ascontroller (cast `Controller` (`self.GetOwner`)))
      (bind _output_get (set `self.As Controller` _ascontroller))
      (bind _asplayer_controller (cast `PlayerController` _output_get))
      (bind _playercameramanager (`PlayerController.PlayerCameraManager` _asplayer_controller))
      (set `self.DefaultYaw Max` (`PlayerCameraManager.ViewYawMax` _playercameramanager))
      (set `self.ViewPitch` (`KismetMathLibrary.MakeVector2D` (`PlayerCameraManager.ViewPitchMax` _playercameramanager) (`PlayerCameraManager.ViewPitchMin` _playercameramanager)))
      (`/Engine/EditorBlueprintResources/ActorComponentMacros.Switch Has Authority`
        (:`Authority`
          (`self.RespawnCheck` true))))
    (:`then_1`
      (`/Engine/EditorBlueprintResources/ActorComponentMacros.Switch Has Authority`
        (:`Authority`
          (message `/Game/ParallelBeam/Core/BPs/Interfaces/BPI_Gamemode.AddNewController` (`GameplayStatics.GetGameMode`) (`self.As Controller`))
          (bind _output_get_2 (set `self.Team Index` (`/Game/ParallelBeam/Core/BPs/Components/GameModeComponents/BP_PlayerState_PS_Component.TeamIndex` (`/Game/ParallelBeam/Core/BPs/FunctionLib/BFL_MSK.GetPlayerStateComponent` (`Controller.PlayerState` (`self.As Controller`))))))
          (bind _return_value (`/Game/ParallelBeam/Core/BPs/FunctionLib/BFL_MSK.Get GameStateTeamComponent` (`GameplayStatics.GetGameState`) _output_get_2))
          (`/Engine/EditorBlueprintResources/StandardMacros.IsValid` _return_value
            (:`Is Valid`
              (set `self.SpawnPlayersAutomatically` (`/Game/ParallelBeam/Core/BPs/Components/GameModeComponents/BP_GameStateTeam_Component.SpawnPlayersAutomatically` _return_value)))))))
    (:`then_2`
      (`KismetSystemLibrary.Delay` 1.0)
      (if (`Controller.IsLocalPlayerController` (`self.As Controller`))
        (`self.PlayerReset`)))
    (:`then_3`
      (add `Actor.OnEndPlay` (`self.As Controller`) (`|CreateDelegate` :!event `OnEndPlaySaveExp`)))))

(event `RespawnCheck`
  (params (Start :type Boolean))
  (bind _respawnchecktimer (`self.RespawnCheckTimer`))
  ;[0 0 0] Timer that runs on server to see if the player can or cant respawn
  (if Start
    (if (`KismetSystemLibrary.K2_IsValidTimerHandle` _respawnchecktimer)
      (`KismetSystemLibrary.K2_UnPauseTimerHandle` (`self.RespawnCheckTimer`))
      (else
        (bind _returnvalue (`KismetSystemLibrary.K2_SetTimerDelegate` (delegate `CheckIfCanRespawn`) 1.0 true true))
        (set `self.RespawnCheckTimer` _returnvalue)))
    (`self.CheckIfCanRespawn`)
    (else
      (`KismetSystemLibrary.K2_PauseTimerHandle` _respawnchecktimer))))

(event `PlayerReset`
  ;[0 0 0] On begin play set the defaulty pitch and yaw values And Show the spawn screen
  (if (`self.SpawnPlayersAutomatically`)
    (set `self.CanRespawn` true)
    (`self.SpawnCharacter` (`self.DefaultLoadout`))
    (`self.RespawnCheck` false)
    (`self.CLTSwitchClientSpawnScreenm` false)
    (else
      (`self.CLTSwitchClientSpawnScreenm` true))))

(event `CheckIfCanRespawn`
  ;[0 0 0] Timer that runs on server to see if the player can or cant respawn
  (bind _asplayer_controller (cast `PlayerController` (`self.As Controller`))
    (:`then`
      (bind _returnvalue (`GameModeBase.PlayerCanRestart` (`GameplayStatics.GetGameMode`) _asplayer_controller))
      (set `self.CanRespawn` _returnvalue))
    (:`CastFailed`
      (set `self.CanRespawn` true))))

(event `SpawnCharacter`
  (params (Loadout :type String))
  ;[0 0 0] The Client Event to spawn the Player
  ; checks the save game and loads accordingly
  (if (`self.CanRespawn`)
    (bind _returnvalue (`GameplayStatics.DoesSaveGameExist` Loadout))
    (if _returnvalue
      (bind _returnvalue_2 (`GameplayStatics.LoadGameFromSlot` Loadout))
      (bind _ass_loadout (cast `/Game/ParallelBeam/Core/BPs/Data/S_Loadout` _returnvalue_2)
        (:`then`
          (set `self.SaveGame` _ass_loadout))
        (:`CastFailed`
          (bind _returnvalue_3 (`GameplayStatics.CreateSaveGameObject` (`self.LoadoutSaveClass`) :!label _label))
          (set `self.SaveGame` _returnvalue_3)))
      (else
        (goto _label)))
    (`self.SVR_SpawnPlayer` (`/Game/ParallelBeam/Core/BPs/Data/S_Loadout.Equipments` (`self.SaveGame`)))
    (`self.CLTSwitchClientSpawnScreenm` false)))

(event `SVR_SpawnPlayer`
  (params (Equipments :type "Array of /Game/ParallelBeam/Core/BPs/Data/Structures/S_EquipmentSave Structure"))
  (bind _returnvalue (`Controller.K2_GetPawn` (`self.As Controller`)))
  (bind _return_value (`/Game/ParallelBeam/Core/BPs/FunctionLib/BFL_MSK.GetPlayerStateComponent` (`Controller.PlayerState` (`self.As Controller`))))
  (bind _returnvalue_2 (`Actor.GetComponentByClass` _returnvalue "/Game/ParallelBeam/Core/BPs/Components/BP_HealthComponent.BP_HealthComponent_C"))
  ;[0 0 0] Spawns the player with the Selected Loadout
  ; if u want the server to load the loadout for players like from AWS servies or smth then do that here
  (set `self.Equipments` Equipments)
  (`self.RespawnCheck` false)
  (`BlueprintMapLibrary.Map_Clear` (`self.CurrentSpawnedEquipments`))
  (`KismetArrayLibrary.Array_Clear` (`self.AmmoToSpawn`))
  (`self.SpawnLoadout`)
  (`KismetSystemLibrary.Delay` 1.0)
  (`GameModeBase.RestartPlayer` (`GameplayStatics.GetGameMode`) (`self.As Controller`))
  (set `self.MainPawn` _returnvalue)
  (set `/Game/ParallelBeam/Core/BPs/Components/GameModeComponents/BP_PlayerState_PS_Component.CurrentMainPawn` _returnvalue _return_value)
  (`/Engine/EditorBlueprintResources/StandardMacros.IsValid` _returnvalue_2
    (:`Is Valid`
      (add `/Game/ParallelBeam/Core/BPs/Components/BP_HealthComponent.OnDeath` _returnvalue_2 (`|CreateDelegate` :!event `OnDeath`)))
    (:`Is Not Valid`
      _))
  (`self.PickUPLoadout`)
  (`/Engine/EditorBlueprintResources/StandardMacros.IsValid` _return_value
    (:`Is Valid`
      (`KismetArrayLibrary.Array_AddUnique` (`Actor.Tags` _returnvalue) (`KismetStringLibrary.Conv_StringToName` (`KismetStringLibrary.Conv_IntToString` (`/Game/ParallelBeam/Core/BPs/Components/GameModeComponents/BP_PlayerState_PS_Component.TeamIndex` _return_value)))))))

(event `ConfirmedKill`
  (params (Exp :type Integer) (PlayerState :type "PlayerState Object Reference") (Reason :type "GameplayTag Structure"))
  ;[0 0 0] OnKillConfirmed, add a kill to personal tracker for kills, and also show the reward points
  (`/Engine/EditorBlueprintResources/StandardMacros.IsValid` PlayerState
    (:`Is Valid`
      (`/Game/ParallelBeam/Core/BPs/Components/GameModeComponents/BP_PlayerState_PS_Component.AddPersonalKill` (`/Game/ParallelBeam/Core/BPs/FunctionLib/BFL_MSK.GetPlayerStateComponent` (`Controller.PlayerState` (`self.As Controller`))) (`PlayerState.BP_GetUniqueId` PlayerState)))
    (:`Is Not Valid`
      _))
  (`self.ConfirmedHit` Exp Reason))

(event `CLTSwitchClientSpawnScreenm`
  (params (Show :type Boolean))
  (bind (_viewpitch_x _viewpitch_y) (`KismetMathLibrary.BreakVector2D` (`self.ViewPitch`)))
  (bind _as_controller (`self.As Controller`))
  ;[0 0 0] Show the Spawn Screen
  (bind _asplayer_controller (cast `PlayerController` _as_controller))
  (message `/Game/ParallelBeam/Core/BPs/Interfaces/BPI_HUD.ShowLoadout` (`/Game/ParallelBeam/Core/BPs/FunctionLib/BFL_MSK.GetMSK_HUD` _as_controller) Show)
  (if Show
    (`WidgetBlueprintLibrary.SetInputMode_UIOnlyEx` _asplayer_controller null)
    (else
      (`WidgetBlueprintLibrary.SetInputMode_GameOnly` _asplayer_controller)))
  (set `PlayerController.bShowMouseCursor` Show _asplayer_controller)
  (bind _returnvalue (pcsubsystem `EnhancedInputLocalPlayerSubsystem` _asplayer_controller))
  (`/Engine/EditorBlueprintResources/StandardMacros.IsValid` _returnvalue
    (:`Is Valid`
      (if (not Show)
        (`EnhancedInputSubsystemInterface.AddMappingContext` _returnvalue "/Game/ParallelBeam/Core/Inputs/IMC_Character.IMC_Character" 0 (struct))
        (bind _playercameramanager (`PlayerController.PlayerCameraManager` _asplayer_controller))
        (set `PlayerCameraManager.ViewYawMin` 0.0 _playercameramanager)
        (set `PlayerCameraManager.ViewYawMax` (`self.DefaultYaw Max`) _playercameramanager)
        (set `PlayerCameraManager.ViewPitchMax` _viewpitch_x _playercameramanager)
        (set `PlayerCameraManager.ViewPitchMin` _viewpitch_y _playercameramanager)
        (else
          (`EnhancedInputSubsystemInterface.RemoveMappingContext` _returnvalue "/Game/ParallelBeam/Core/Inputs/IMC_Character.IMC_Character" (struct))
          (bind _outactors (`GameplayStatics.GetAllActorsOfClassWithTag` "/Script/Engine.CameraActor" "MapLookTop"))
          (`PlayerController.SetViewTargetWithBlend` _asplayer_controller (`|GetArrayItem` _outactors) 0.8 "VTBlend_EaseInOut" 2.0 false))))))

(event `OnDeath`
  ;[1 0 0] On Death Unposses the current pawn and Add a Spawning Screen for the client
  (`Controller.UnPossess` (`self.As Controller`))
  (if (`self.SpawnPlayersAutomatically`)
    (`KismetSystemLibrary.Delay` 2.0)
    (`self.SpawnCharacter` "Loadout A")
    (else
      (`self.RespawnCheck` true)
      (`KismetSystemLibrary.Delay` 3.0)
      (`self.CLTSwitchClientSpawnScreenm` true))))

(event `SetTargetToFollow`
  (params (KillerPawn :type "Pawn Object Reference") (Duration :type "Float (single-precision)") (Owner :type "Pawn Object Reference") (KillerWeapon :type "Actor Object Reference"))
  ;[1 0 0] Following the Killer Player Pawn (enables and disables ticking when we stop following)
  (`/Game/ParallelBeam/Core/BPs/Components/GameModeComponents/BP_PlayerState_PS_Component.AddEnemyKill` (`/Game/ParallelBeam/Core/BPs/FunctionLib/BFL_MSK.GetPlayerStateComponent` (`Controller.PlayerState` (`self.As Controller`))) (`PlayerState.BP_GetUniqueId` (`Pawn.PlayerState` KillerPawn)))
  (`/Engine/EditorBlueprintResources/StandardMacros.IsValid` KillerPawn
    (:`Is Valid`
      (`self.SetComponentTickEnabled` true))
    (:`Is Not Valid`
      _))
  (message `/Game/ParallelBeam/Core/BPs/Interfaces/BPI_HUD.ShowKillerScreen` (`/Game/ParallelBeam/Core/BPs/FunctionLib/BFL_MSK.GetMSK_HUD` (`self.As Controller`)) KillerPawn KillerWeapon Duration)
  (`KismetSystemLibrary.Delay` Duration)
  (`self.SetComponentTickEnabled` false))

(event `self.ReceiveTick`
  (params (DeltaSeconds :type "Float (single-precision)"))
  (bind _as_controller (`self.As Controller`))
  ;[1 0 0] Following the Killer Player Pawn (enables and disables ticking when we stop following)
  (`Controller.SetControlRotation` _as_controller (`KismetMathLibrary.RInterpTo` (`Controller.GetControlRotation` _as_controller) (`KismetMathLibrary.FindLookAtRotation` (`Actor.K2_GetActorLocation` (stale `SetTargetToFollow` Owner)) (`Actor.K2_GetActorLocation` (stale `SetTargetToFollow` KillerPawn))) DeltaSeconds 5.0)))

(event `CLT_SetCrosshairWidget`
  (params (Crosshair :type "/Game/ParallelBeam/Core/Widgets/Game/Croshairs/WB_MasterCrossHair Class Reference"))
  ;[0 0 0] SetCrosshair
  (message `/Game/ParallelBeam/Core/BPs/Interfaces/BPI_HUD.SetCrosshair` (`/Game/ParallelBeam/Core/BPs/FunctionLib/BFL_MSK.GetMSK_HUD` (`self.As Controller`)) Crosshair))

(event `CLT_AddMappingContext`
  (params (MappingContext :type "InputMappingContext Object Reference") (Add :type Boolean))
  ;[0 0 0] OnClientEntered confirmed, we add the mapping context to control this
  (bind _asplayer_controller (cast `PlayerController` (`self.As Controller`)))
  (if Add
    (bind _returnvalue (pcsubsystem `EnhancedInputLocalPlayerSubsystem` _asplayer_controller))
    (`EnhancedInputSubsystemInterface.AddMappingContext` _returnvalue MappingContext 0 (struct))
    (else
      (`EnhancedInputSubsystemInterface.RemoveMappingContext` _returnvalue MappingContext (struct)))))

(event `CLT_UpdatePawnUI`
  (params (Widget :type "/Game/ParallelBeam/Core/Widgets/Game/PawnUIs/WB_MasterPawnUI Class Reference"))
  ;[0 0 0] UpdateMainUIOfPawn
  (message `/Game/ParallelBeam/Core/BPs/Interfaces/BPI_HUD.UpdatePawnUI` (`/Game/ParallelBeam/Core/BPs/FunctionLib/BFL_MSK.GetMSK_HUD` (`self.As Controller`)) Widget))

(event `ConfirmedHit`
  (params (Exp :type Integer) (Reason :type "GameplayTag Structure"))
  ;[0 0 0] OnConfirmedHit, add experiencePoints
  (set `self.AccumulatedExp` (+ (`self.AccumulatedExp`) Exp))
  (message `/Game/ParallelBeam/Core/BPs/Interfaces/BPI_HUD.AddExperiencePoint` (`/Game/ParallelBeam/Core/BPs/FunctionLib/BFL_MSK.GetMSK_HUD` (`self.As Controller`)) Exp Reason)
  (if (`self.ApplyExpInstantly`)
    (`self.OnEndPlaySaveExp` null)))

(fn `OnEndPlaySaveExp`
  (params (Actor :type "Actor Object Reference") (EndPlayReason :type "EEndPlayReason Enum" :default "Destroyed"))
  (locals (PlayerProgressSave :type "/Game/ParallelBeam/Core/BPs/Data/S_PlayerProgress Object Reference"))
  (bind _playerprogresssave (`local.PlayerProgressSave`))
  (bind _returnvalue (`GameplayStatics.LoadGameFromSlot` "PlayerProgress"))
  (`/Engine/EditorBlueprintResources/StandardMacros.IsValid` _returnvalue
    (:`Is Valid`
      (bind _ass_player_progress (cast `/Game/ParallelBeam/Core/BPs/Data/S_PlayerProgress` _returnvalue))
      (set `local.PlayerProgressSave` _ass_player_progress))
    (:`Is Not Valid`
      (bind _returnvalue_2 (`GameplayStatics.CreateSaveGameObject` "/Game/ParallelBeam/Core/BPs/Data/S_PlayerProgress.S_PlayerProgress_C"))
      (set `local.PlayerProgressSave` _returnvalue_2)))
  (set `/Game/ParallelBeam/Core/BPs/Data/S_PlayerProgress.CurrentExp` (+ (`/Game/ParallelBeam/Core/BPs/Data/S_PlayerProgress.CurrentExp` _playerprogresssave) (`self.AccumulatedExp`)) _playerprogresssave)
  (`GameplayStatics.SaveGameToSlot` _playerprogresssave "PlayerProgress"))

(fn `PickUPLoadout`
  (bind _returnvalue (`AGR_InventoryFunctionLibrary.GetInventoryComponent` (`Controller.K2_GetPawn` (`self.As Controller`))))
  (bind _returnvalue_2 (`AGR_InventoryFunctionLibrary.GetInventoryComponent` (`Controller.K2_GetPawn` (`self.As Controller`))))
  (bind _returnvalue_3 (`AGR_InventoryFunctionLibrary.GetItemComponent` (`AGR_InventoryComponent.GetItemInSlot` _returnvalue_2 (struct :`TagName` "CharacterSlots.Primary"))))
  (`/Engine/EditorBlueprintResources/StandardMacros.IsValid` (`AGR_InventoryFunctionLibrary.GetInventoryComponent` (`Controller.K2_GetPawn` (`self.As Controller`)))
    (:`Is Valid`
      (bind _keys (`BlueprintMapLibrary.Map_Keys` (`self.CurrentSpawnedEquipments`)))
      (for _array_element _keys
        (bind _returnvalue_4 (`AGR_InventoryFunctionLibrary.GetItemComponent` _array_element))
        (`/Engine/EditorBlueprintResources/StandardMacros.IsValid` _returnvalue_4
          (:`Is Valid`
            (`AGR_ItemComponent.PickUpItem` _returnvalue_4 _returnvalue true true false)
            (`AGR_ItemComponent.EquipItem` _returnvalue_4 _returnvalue (`BlueprintMapLibrary.Map_Find` (`self.CurrentSpawnedEquipments`) _array_element) false))))
      (for _array_element_2 (`self.AmmoToSpawn`)
        (bind _returnvalue_5 (`|SpawnActorFromClass` _array_element_2 (`KismetMathLibrary.MakeTransform` (0.0 0.0 0.0)) "Undefined" "MultiplyWithRoot" null null))
        (bind _returnvalue_6 (`AGR_InventoryFunctionLibrary.GetItemComponent` _returnvalue_5))
        (`/Engine/EditorBlueprintResources/StandardMacros.IsValid` _returnvalue_6
          (:`Is Valid`
            (`AGR_ItemComponent.PickUpItem` _returnvalue_6 _returnvalue true true true))))
      (`/Engine/EditorBlueprintResources/StandardMacros.IsValid` _returnvalue_3
        (:`Is Valid`
          (`AGR_ItemComponent.EquipItem` _returnvalue_3 _returnvalue_2 (struct :`TagName` "CharacterSlots.RightHand") true))))))

(fn `SpawnLoadout`
  (locals (LOC_Equipment :type "/Game/ParallelBeam/Core/BPs/Data/Structures/S_EquipmentSave Structure"))
  (bind _currentspawnedequipments (`self.CurrentSpawnedEquipments`))
  (bind ((`Attachments_8_EBB2B0EC465F28A94A927E9764FFFEAA` _attachments) (`Skin_12_1EB6AC82493DC0F299966DB8AFDC4978` _skin) (`EquippedSlot_18_C57B8920467B02D3376AE7B46107EA30` _equippedslot)) (break `/Game/ParallelBeam/Core/BPs/Data/Structures/S_EquipmentSave` (`local.LOC_Equipment`)))
  (bind ((`EquippedSlot_18_C57B8920467B02D3376AE7B46107EA30` _equippedslot_2)) (break `/Game/ParallelBeam/Core/BPs/Data/Structures/S_EquipmentSave` (`local.LOC_Equipment`)))
  (bind _returnvalue (== _equippedslot_2 (struct :`TagName` "CharacterSlots.Primary.Akimbo")))
  (`BlueprintMapLibrary.Map_Clear` (`self.CurrentSpawnedEquipments`))
  (for (_array_element _array_index) (`self.Equipments`)
    (set `local.LOC_Equipment` _array_element)
    (if (or _returnvalue (== _equippedslot_2 (struct :`TagName` "CharacterSlots.Secondary.Akimbo")))
      (bind _values (`BlueprintMapLibrary.Map_Values` _currentspawnedequipments))
      (bind _keys (`BlueprintMapLibrary.Map_Keys` _currentspawnedequipments))
      (bind _return_value (message `/Game/ParallelBeam/Core/BPs/Interfaces/BPI_Weapon.GetIsSingleHanded` (`|GetArrayItem` _keys (`KismetArrayLibrary.Array_Find` _values (`BlueprintGameplayTagLibrary.MakeLiteralGameplayTag` (select `bool` _returnvalue :`false` (struct :`TagName` "CharacterSlots.Secondary") :`true` (struct :`TagName` "CharacterSlots.Primary") :!type "GameplayTag Structure"))))))
      (if _return_value
        (bind _returnvalue_2 (`KismetSystemLibrary.LoadClassAsset_Blocking` (`.Item_9_6D1F1966495809AA11DE939997BC96A0` (break `/Game/ParallelBeam/Core/BPs/Data/Structures/S_EquipmentSave` (`local.LOC_Equipment`))) :!label _label))
        (bind _asactor (castclass `Actor` _returnvalue_2))
        (bind _returnvalue_3 (`|SpawnActorFromClass` _asactor (`KismetMathLibrary.MakeTransform` (+ (* _array_index (0.0 0.0 -100.0)) (0.0 0.0 -100000.0))) "Undefined" "MultiplyWithRoot" (`self.As Controller`) null))
        (message `/Game/ParallelBeam/Core/BPs/Interfaces/BPI_Skin.ApplySkin` _returnvalue_3 _skin)
        (`BlueprintMapLibrary.Map_Add` (`self.CurrentSpawnedEquipments`) _returnvalue_3 _equippedslot)
        (for _array_element_2 _attachments
          (bind (_item _attachments_2) (break `/Game/ParallelBeam/Core/BPs/Data/Structures/S_AttachmentSave` _array_element_2))
          (bind _returnvalue_4 (`KismetSystemLibrary.LoadClassAsset_Blocking` _item))
          (bind _asactor_2 (castclass `Actor` _returnvalue_4))
          (bind _attachment_inventory (`/Game/ParallelBeam/Core/BPs/FunctionLib/BFL_MSK.GetAttachmentInventory` _returnvalue_3))
          (bind _return_value_2 (`/Game/ParallelBeam/Core/BPs/Components/BP_AttachmentInventory.GetAllAttachmentsByClass` _attachment_inventory _asactor_2))
          (if (> (`KismetArrayLibrary.Array_Length` _return_value_2) 0)
            (bind _returnvalue_5 (`KismetSystemLibrary.LoadClassAsset_Blocking` (`/Game/ParallelBeam/Core/BPs/Data/DTA_Attachment.ActorRef` _attachments_2)))
            (bind (_attachment_inventory_2 _returnvalue_6) (`/Game/ParallelBeam/Core/BPs/FunctionLib/BFL_MSK.GetAttachmentInventory` (`|GetArrayItem` _return_value_2)))
            (`/Game/ParallelBeam/Core/BPs/Components/BP_AttachmentInventory.AddAttachment` (select `bool` _returnvalue_6 :`false` _attachment_inventory :`true` _attachment_inventory_2) _returnvalue_5)))
        (bind _return_value_3 (message `/Game/ParallelBeam/Core/BPs/Interfaces/BPI_Weapon.GetAmmoType` _returnvalue_3))
        (`KismetArrayLibrary.Array_AddUnique` (`self.AmmoToSpawn`) _return_value_3))
      (else
        (goto _label)))))