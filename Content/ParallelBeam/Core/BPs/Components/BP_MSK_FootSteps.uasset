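; Actor component that plays surface-dependent footstep sounds for its owning Pawn.
; On BeginPlay it caches the owner and its skeletal mesh tagged "RootMesh".
; PlayFootStep box-traces down from a given socket against world objects, ignoring the owner.
; On a hit, it looks up the step type in a Sounds map, resolves the physical material's surface to a sound, and plays it at the socket.
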(event `self.ReceiveBeginPlay`
  (bind _aspawn (cast `Pawn` (`self.GetOwner`)))
  (bind _output_get (set `self.OwnerPawn` _aspawn))
  (set `self.SkeletalMesh` (`|GetArrayItem` (`Actor.GetComponentsByTag` _output_get "/Script/Engine.SkeletalMeshComponent" "RootMesh"))))

(event `PlayFootStep`
  (params (InSocketName :type Name) (Type :type "GameplayTag Structure"))
  (bind _returnvalue (`SceneComponent.GetSocketLocation` (`self.SkeletalMesh`) InSocketName))
  (bind _outhit (`KismetSystemLibrary.BoxTraceSingleForObjects` _returnvalue (- _returnvalue (0.0 0.0 100.0)) (5.0 5.0 5.0) (struct) (`|MakeArray` "ObjectTypeQuery1" "ObjectTypeQuery2" :!type "EObjectTypeQuery Enum") false (`|MakeArray` (`self.OwnerPawn`) :!type "Actor Object Reference")))
  (bind (_bblockinghit _binitialoverlap _time _distance _location _impactpoint _normal _impactnormal _physmat) (`GameplayStatics.BreakHitResult` _outhit))
  (if _bblockinghit
    (bind (_value _returnvalue_2) (`/Game/ParallelBeam/Core/BPs/Data/DTA_SurfaceSounds.Get Sound by Surface` (`BlueprintMapLibrary.Map_Find` (`self.Sounds`) Type) (`PhysicalMaterial.SurfaceType` _physmat)))
    (if _returnvalue_2
      (`GameplayStatics.PlaySoundAtLocation` _value _returnvalue (struct) 1.0 1.0 0.0 null null null null))))