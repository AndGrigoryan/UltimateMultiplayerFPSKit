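; Health component that gives its owning actor replicated health, damage handling, regeneration and death in multiplayer.
; Point and radial hits feed DealDamage, which scales damage by a per-DamageType multiplier map, ignoring unlisted types.
; Death fires once, crediting kill or headshot experience, posting a kill message, multicasting death and making the victim's client follow the stencil-highlighted killer.
; Non-lethal hits award experience, and delayed looping-timer regen restores health.
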(event `self.ReceiveBeginPlay`
  (bind _returnvalue (`self.GetOwner`))
  ;[0 0 0] Bindings on damage
  (add `Actor.OnTakePointDamage` _returnvalue (`|CreateDelegate` :!event `OnPointHit`))
  (add `Actor.OnTakeRadialDamage` _returnvalue (`|CreateDelegate` :!event `OnRadialHit`))
  (set `self.CurrentHealth` (`self.MaxHealth`)))

(event `OnPointHit`
  (params (DamagedActor :type "Actor Object Reference") (Damage :type "Float (single-precision)") (InstigatedBy :type "Controller Object Reference") (HitLocation :type "Vector Structure") (FHitComponent :type "PrimitiveComponent Object Reference") (BoneName :type Name) (ShotFromDirection :type "Vector Structure") (DamageType :type "DamageType Object Reference") (DamageCauser :type "Actor Object Reference"))
  ;[0 0 0] Bindings on damage
  (`self.DealDamage` Damage InstigatedBy HitLocation ShotFromDirection BoneName DamageCauser DamageType))

(event `OnRadialHit`
  (params (DamagedActor :type "Actor Object Reference") (Damage :type "Float (single-precision)") (DamageType :type "DamageType Object Reference") (Origin :type "Vector Structure") (HitInfo :type "HitResult Structure (by ref)") (InstigatedBy :type "Controller Object Reference") (DamageCauser :type "Actor Object Reference"))
  (bind (_bblockinghit _binitialoverlap _time _distance _location _impactpoint _normal _impactnormal _physmat _hitactor _hitcomponent _hitbonename _bonename) (`GameplayStatics.BreakHitResult` HitInfo))
  ;[0 0 0] Bindings on damage
  (`self.DealDamage` Damage InstigatedBy Origin _impactnormal _bonename DamageCauser DamageType))

(event `MLT_CallDeath`
  (params (Side :type "Vector Structure"))
  ;[0 0 0] Telling Everyone to Play appropriate Death animations and destroying the Player items if it was called on server
  (set `self.Hit From direction` Side)
  (`self.OnDeath`))

(event `DealDamage`
  (params (Damage :type "Float (double-precision)") (Instigator :type "Controller Object Reference") (HitLocation :type "Vector Structure") (HitDirection :type "Vector Structure") (Bone :type Name) (` Causer` :type "Actor Object Reference") (DamageType :type "DamageType Object Reference"))
  (bind _return_value (`self.FindDamageMultiplierValue` DamageType))
  (bind _hitexperience (`self.HitExperience`))
  (bind _returnvalue (`Pawn.GetController` (`Actor.Instigator` (`self.GetOwner`))))
  ;[0 0 0] Just basic damage calculation and death mechanics calling
  (if (> _return_value 0.0)
    (`/Engine/EditorBlueprintResources/StandardMacros.IsValid` Instigator
      (:`Is Valid`
        (set `self.DamageInstigator` Instigator)
        (set `self.Causer` ` Causer`))
      (:`Is Not Valid`
        _))
    (bind _output_get (set `self.CurrentHealth` (`KismetMathLibrary.FClamp` (- (`self.CurrentHealth`) (* Damage _return_value)) 0.0 (`self.MaxHealth`))))
    (bind _output_get_2 (set `self.Bone` Bone))
    (`self.TriggerHealthRegen`)
    (if (<= _output_get 0.0)
      (`/Engine/EditorBlueprintResources/StandardMacros.DoOnce` false
        (:`Completed`
          (bind _damageinstigator (`self.DamageInstigator`)
            (:`then`
              (bind _returnvalue_2 (`KismetArrayLibrary.Array_Contains` (`self.HeadShotBones`) _output_get_2))
              (`/Game/ParallelBeam/Core/BPs/Components/GameModeComponents/BP_ControllerComponent.ConfirmedKill` (`Actor.GetComponentByClass` _damageinstigator "/Game/ParallelBeam/Core/BPs/Components/GameModeComponents/BP_ControllerComponent.BP_ControllerComponent_C") (select `bool` _returnvalue_2 :`false` (`self.KillExperience`) :`true` (`self.HeadshotKillExperience`)) (`Pawn.PlayerState` (`Actor.Instigator` (`self.GetOwner`))) (select `bool` _returnvalue_2 :`false` (`self.KillReason`) :`true` (struct :`TagName` "Exp.Hit.Kill.HeadShot")))
              (`/Engine/EditorBlueprintResources/StandardMacros.IsValid` _returnvalue
                (:`Is Valid`
                  (message `/Game/ParallelBeam/Core/BPs/Interfaces/BPI_Gamemode.AddKill` (`GameplayStatics.GetGameMode`) (`self.DamageInstigator`) _returnvalue (`self.Causer`))
                  (`self.CLT_HighlightEnemy` (`Controller.K2_GetPawn` (`self.DamageInstigator`)) (`self.Causer`)))
                (:`Is Not Valid`
                  _)))
            (:`else`
              _))
          (`self.MLT_CallDeath` HitDirection)))
      (else
        (bind _damageinstigator_2 (`self.DamageInstigator`)
          (:`then`
            (if (> _hitexperience 0)
              (`/Game/ParallelBeam/Core/BPs/Components/GameModeComponents/BP_ControllerComponent.ConfirmedHit` (`Actor.GetComponentByClass` _damageinstigator_2 "/Game/ParallelBeam/Core/BPs/Components/GameModeComponents/BP_ControllerComponent.BP_ControllerComponent_C") _hitexperience (`self.HitReason`))))
          (:`else`))))))

(event `CLT_HighlightEnemy`
  (params (Target :type "Pawn Object Reference") (Causer :type "Actor Object Reference"))
  (bind _returnvalue (`Actor.GetComponentByClass` Target "BP_HealthComponent_C"))
  (bind _returnvalue_2 (`self.GetOwner`))
  (bind _instigator (`Actor.Instigator` _returnvalue_2))
  ;[1 0 0] Local player is told to highlight and follow the Character that killer it
  (message `/Game/ParallelBeam/Core/BPs/Interfaces/BPI_HUD.ShowGameUI` (`/Game/ParallelBeam/Core/BPs/FunctionLib/BFL_MSK.GetMSK_HUD` _returnvalue_2) false)
  (`/Engine/EditorBlueprintResources/StandardMacros.IsValid` (`AIBlueprintHelperLibrary.GetAIController` _instigator)
    (:`Is Not Valid`
      (`/Engine/EditorBlueprintResources/StandardMacros.IsValid` Target
        (:`Is Valid`
          (`/Engine/EditorBlueprintResources/StandardMacros.IsValid` _returnvalue
            (:`Is Valid`
              (`self.HighlightCharacter` _returnvalue 3.0)
              (`/Game/ParallelBeam/Core/BPs/Components/GameModeComponents/BP_ControllerComponent.SetTargetToFollow` (`Actor.GetComponentByClass` (`GameplayStatics.GetPlayerController` 0) "/Game/ParallelBeam/Core/BPs/Components/GameModeComponents/BP_ControllerComponent.BP_ControllerComponent_C") Target 3.0 _instigator Causer))))))))

(event `HighlightCharacter`
  (params (Duration :type "Float (single-precision)"))
  (bind _returnvalue (`Actor.GetComponentsByTag` (`self.GetOwner`) "/Script/Engine.SkeletalMeshComponent" "MainMesh"))
  ;[1 0 0] Highlights the Pawn that was the killer for the local player
  (for _array_element _returnvalue
    (`PrimitiveComponent.SetCustomDepthStencilValue` _array_element 2))
  (`KismetSystemLibrary.RetriggerableDelay` Duration)
  (for _array_element_2 _returnvalue
    (`PrimitiveComponent.SetCustomDepthStencilValue` _array_element_2 1)))

(event `TriggerHealthRegen`
  ;[0 0 0] HEALTH REGEN
  (if (`self.CanRegen`)
    (`KismetSystemLibrary.K2_ClearAndInvalidateTimerHandle` (`self.RegenTimer`))
    (if (> (`self.CurrentHealth`) 0.0)
      (`KismetSystemLibrary.RetriggerableDelay` (`self.TimeToWaitAfterDamageForRegen`))
      (if (> (`self.CurrentHealth`) 0.0)
        (bind _returnvalue (`KismetSystemLibrary.K2_SetTimerDelegate` (delegate `RegenHealth`) (`self.RegenLoopTime`) true))
        (set `self.RegenTimer` _returnvalue)))))

(event `RegenHealth`
  (bind _maxhealth (`self.MaxHealth`))
  ;[0 0 0] HEALTH REGEN
  (bind _output_get (set `self.CurrentHealth` (`KismetMathLibrary.FClamp` (+ (`self.CurrentHealth`) (`self.RegenAmmount`)) 0.0 _maxhealth)))
  (if (>= _output_get _maxhealth)
    (`KismetSystemLibrary.K2_ClearAndInvalidateTimerHandle` (`self.RegenTimer`))))

(fn `FindDamageMultiplierValue`
  (params (`Damage Type` :type "DamageType Object Reference"))
  (returns (`Return Value` :type "Float (double-precision)"))
  (bind (_value _returnvalue) (`BlueprintMapLibrary.Map_Find` (`self.DamageTypeMultiplier`) (`GameplayStatics.GetObjectClass` `Damage Type`)))
  (return (select `bool` _returnvalue :`true` _value)))

(fn `OnRep_CurrentHealth`
  (`self.OnHealthUpdated` (`self.CurrentHealth`)))