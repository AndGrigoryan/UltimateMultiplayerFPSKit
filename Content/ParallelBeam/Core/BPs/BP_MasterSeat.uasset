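; BP_MasterSeat is a possessable seat pawn that a character can enter through interaction and exit with the F key.
; A BPPawnPossesion component handles entering, exit requests and exit points, and interaction is allowed only while the seat is unpossessed.
; The interaction box copies location and extent from InteractionBoxParent at construction and BeginPlay, and is destroyed at BeginPlay when no parent is valid.
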(event `self.ReceivePossessed`
  (params (NewController :type "Controller Object Reference"))
  (if (`Controller.IsPlayerController` NewController)
    (`/Game/ParallelBeam/Core/BPs/Components/BP_PawnPossesion.SVR_EnteredPawn` (`self.BP_PawnPossesion`) NewController)))

(event `Key|F`
  (params (Key :type "Key Structure"))
  (:`Pressed`
    (`/Game/ParallelBeam/Core/BPs/Components/BP_PawnPossesion.SVR_RequestExit` (`self.BP_PawnPossesion`))))

(event `self.ReceiveBeginPlay`
  (bind _interactiobox (`self.InteractioBox`))
  (bind _interactionboxparent (`self.InteractionBoxParent`))
  (`/Engine/EditorBlueprintResources/StandardMacros.IsValid` _interactionboxparent
    (:`Is Valid`
      (`SceneComponent.K2_SetWorldLocation` _interactiobox (`SceneComponent.K2_GetComponentLocation` _interactionboxparent) false false)
      (`BoxComponent.SetBoxExtent` _interactiobox (`BoxComponent.BoxExtent` _interactionboxparent) true))
    (:`Is Not Valid`
      (`ActorComponent.K2_DestroyComponent` _interactiobox)))
  (set `/Game/ParallelBeam/Core/BPs/Components/BP_PawnPossesion.Exits` (`self.ExitPoints`) (`self.BP_PawnPossesion`)))

(fn `CanGetIcon`
  (returns (ReturnValue :type Boolean))
  (return false))

(fn `CanInteract`
  (params (Actor :type "Actor Object Reference"))
  (returns (`Return Value` :type Boolean))
  (return (not (`/Game/ParallelBeam/Core/BPs/Components/BP_PawnPossesion.Possesed` (`self.BP_PawnPossesion`)))))

(fn `GetIcon`
  (params (Stock :type Boolean))
  (returns (Texture :type "Texture Object Reference"))
  (return null))

(fn `GetInteractionInfo`
  (params (InteractingActor :type "Actor Object Reference"))
  (returns (Item :type Text) (Type :type Text) (HoldType :type Text))
  (return "Seat" "Enter" ""))

(fn `StartInteract`
  (params (Character :type "Character Object Reference"))
  (returns (`Return Value` :type Boolean))
  (`/Game/ParallelBeam/Core/BPs/Components/BP_PawnPossesion.SVR_AttemptEnter Pawn` (`self.BP_PawnPossesion`) (`self.GetController` Character))
  (return true))

(fn `UserConstructionScript`
  (bind _interactiobox (`self.InteractioBox`))
  (bind _interactionboxparent (`self.InteractionBoxParent`))
  (`/Engine/EditorBlueprintResources/StandardMacros.IsValid` _interactionboxparent
    (:`Is Valid`
      (`SceneComponent.K2_SetWorldLocation` _interactiobox (`SceneComponent.K2_GetComponentLocation` _interactionboxparent) false false)
      (`BoxComponent.SetBoxExtent` _interactiobox (`BoxComponent.BoxExtent` _interactionboxparent) true))))