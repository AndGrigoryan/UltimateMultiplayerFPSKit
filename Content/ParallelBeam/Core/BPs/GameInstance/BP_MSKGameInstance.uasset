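; Game instance that handles online sessions, level launching, game settings and player progression.
; StartPlay joins the first found session for multiplayer levels or falls back to creating one, then opens the selected level as a listen server, broadcasting each stage.
; Init loads or creates settings and progress saves, deriving player level from an XP data table.
; Settings changes save asynchronously, and a getter supplies the settings widget.
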(event `CreateSession`
  (params (PublicConnections :type Integer) (bUseLAN :type Boolean) (bUseLobbiesIfAvailable :type Boolean))
  (bind _returnvalue (`GameplayStatics.GetPlayerController` 0))
  (`CreateSessionCallbackProxy.CreateSession` _returnvalue _returnvalue PublicConnections bUseLAN bUseLobbiesIfAvailable
    (:`OnSuccess`
      (`self.OnSessionCreated` true)
      (`KismetSystemLibrary.PrintString` "Created"))
    (:`OnFailure`
      (`self.OnSessionCreated` false)
      (`KismetSystemLibrary.PrintString` "Session failed"))))

(event `FindSessions`
  (params (MaxResults :type Integer) (bUseLAN :type Boolean))
  (bind _returnvalue (`GameplayStatics.GetPlayerController` 0))
  (bind _results (`FindSessionsCallbackProxy.FindSessions` _returnvalue _returnvalue MaxResults bUseLAN)
    (:`OnSuccess`
      (`KismetSystemLibrary.PrintString` "Found")
      ;[1 1 1] it wont allow array to be moved so doing a loop
      (`self.OnFoundSessions` (struct))
      (for _array_element _results
        (`self.OnFoundSessions` _array_element)))
    (:`OnFailure`
      (`KismetSystemLibrary.PrintString` "Session failed")
      (`self.OnFoundSessions` (struct)))))

(event `SelectLevel`
  (params (DTA :type "/Game/ParallelBeam/Core/BPs/Data/DTA_Level Object Reference"))
  (bind _output_get (set `self.DTA` DTA))
  (`self.OnLevelChanged` _output_get))

(event `OnlevelLoaded`
  (`self.UpdateStage` "LEVEL LOADED | JOINING GAME" :!label _label)
  (`KismetSystemLibrary.Delay` 1.0)
  (`GameplayStatics.OpenLevelBySoftObjectPtr` (`/Game/ParallelBeam/Core/BPs/Data/DTA_Level.LevelRefrence` (`self.DTA`)) true "listen"))

(event `StartPlay`
  (bind _returnvalue (`GameplayStatics.GetPlayerController` 0))
  (bind _returnvalue_2 (`GameplayStatics.GetPlayerController` 0))
  (if (`/Game/ParallelBeam/Core/BPs/Data/DTA_Level.IsMultiplayer` (`self.DTA`))
    (bind _results (`FindSessionsCallbackProxy.FindSessions` _returnvalue_2 _returnvalue_2 50)
      (:`then`
        (`self.UpdateStage` "Finding Sessions"))
      (:`OnSuccess`
        (if (`KismetArrayLibrary.Array_IsEmpty` _results)
          (`self.UpdateStage` "Unable to Find Sessions, Creating Own Session" :!label _label_2)
          (`CreateSessionCallbackProxy.CreateSession` _returnvalue _returnvalue (`/Game/ParallelBeam/Core/BPs/Data/DTA_Level.MaxPlayers` (`self.DTA`))
            (:`OnSuccess`
              (`self.UpdateStage` "Session Created")
              (`self.UpdateStage` "LOADING LEVEL" :!label _label_3)
              (goto _label))
            (:`OnFailure`
              (`self.UpdateStage` "Failed to Create Session" 5.0)))
          (else
            (`JoinSessionCallbackProxy.JoinSession` _returnvalue_2 (`|GetArrayItem` _results)
              (:`then`
                (`self.UpdateStage` "Attempting To Join Session"))
              (:`OnSuccess`
                (`self.UpdateStage` "Session Joined Sucessfully"))
              (:`OnFailure`
                (`self.UpdateStage` "Failed To Join Session")
                (goto _label_2))))))
      (:`OnFailure`
        (goto _label_2)))
    (else
      (goto _label_3))))

(event `self.ReceiveInit`
  (`parent.ReceiveInit`)
  (`self.CreateGameSettings`)
  (bind _returnvalue (`GameplayStatics.LoadGameFromSlot` "PlayerProgress"))
  (`/Engine/EditorBlueprintResources/StandardMacros.IsValid` _returnvalue
    (:`Is Valid`
      (bind _ass_player_progress (cast `/Game/ParallelBeam/Core/BPs/Data/S_PlayerProgress` _returnvalue))
      (set `self.PlayerProgressSave` _ass_player_progress))
    (:`Is Not Valid`
      (bind _returnvalue_2 (`GameplayStatics.CreateSaveGameObject` "/Game/ParallelBeam/Core/BPs/Data/S_PlayerProgress.S_PlayerProgress_C"))
      (set `self.PlayerProgressSave` _returnvalue_2)))
  (`self.UpdateCurrentLevel`))

(event `CreateGameSettings`
  (bind _returnvalue (`GameplayStatics.DoesSaveGameExist` "GameSettings"))
  (if _returnvalue
    (bind _returnvalue_2 (`GameplayStatics.LoadGameFromSlot` "GameSettings"))
    (bind _ass_game_settings (cast `/Game/ParallelBeam/Core/BPs/Data/S_GameSettings` _returnvalue_2))
    (set `self.GameSettingsSave` _ass_game_settings)
    (else
      (bind _returnvalue_3 (`GameplayStatics.CreateSaveGameObject` "/Game/ParallelBeam/Core/BPs/Data/S_GameSettings.S_GameSettings_C"))
      (`AsyncActionHandleSaveGame.AsyncSaveGameToSlot` self _returnvalue_3 "GameSettings"
        (:`then`
          (set `self.GameSettingsSave` _returnvalue_3)))))
  (bind _returnvalue_4 (`GameUserSettings.GetGameUserSettings`))
  (`GameUserSettings.LoadSettings` _returnvalue_4 true)
  (add `GameUserSettings.OnGameUserSettingsUINeedsUpdate` _returnvalue_4 (delegate `OnGameUserSettingsUINeedsUpdate_Event`)))

(event `OnGameUserSettingsUINeedsUpdate_Event`
  (`self.SaveGameSettings`))

(event `SaveGameSettings`
  (`AsyncActionHandleSaveGame.AsyncSaveGameToSlot` self (`self.GameSettingsSave`) "GameSettings"
    (:`Completed`
      (`self.GameSettingsUpdated`))))

(event `SetFloatValue`
  (params (Command :type String) (Value :type "Float (double-precision)"))
  (if (not (`KismetStringLibrary.IsEmpty` Command))
    (`/Game/ParallelBeam/Core/BPs/Data/S_GameSettings.SetFloatValue` (`self.GameSettingsSave`) Command Value (`GameplayStatics.GetPlayerController` 0))
    (`self.SaveGameSettings`)))

(event `SetIntValue`
  (params (Command :type String) (Value :type Integer))
  (if (not (`KismetStringLibrary.IsEmpty` Command))
    (`/Game/ParallelBeam/Core/BPs/Data/S_GameSettings.SetintValue` (`self.GameSettingsSave`) Command Value (`GameplayStatics.GetPlayerController` 0))
    (`self.SaveGameSettings`)))

(fn `GetGameSettings`
  (returns (Settings :type "/Game/ParallelBeam/Core/BPs/Data/S_GameSettings Object Reference"))
  (return (`self.GameSettingsSave`)))

(fn `GetSettingsWidget`
  (returns (SettignsWidget :type "/Game/ParallelBeam/Core/Widgets/Menu/WB_Settings Object Reference"))
  (bind _settignswidget (`self.SettignsWidget`)
    (:`then`
      (if (not (`Widget.IsInViewport` _settignswidget))
        (bind _returnvalue (`|CreateWidget` "/Game/ParallelBeam/Core/Widgets/Menu/WB_Settings.WB_Settings_C" :!label _label))
        (bind _output_get (set `self.SettignsWidget` _returnvalue))
        (`UserWidget.AddToViewport` _output_get 999)))
    (:`else`
      (goto _label)))
  (return (`self.SettignsWidget`)))

(fn `UpdateCurrentLevel`
  (bind _currentexp (`/Game/ParallelBeam/Core/BPs/Data/S_PlayerProgress.CurrentExp` (`self.PlayerProgressSave`)))
  (bind _outrownames (`DataTableFunctionLibrary.GetDataTableRowNames` "/Game/ParallelBeam/Core/BPs/Data/DT_PlayerLevels.DT_PlayerLevels"))
  (for (_array_element _array_index) _outrownames
    (bind _returnvalue (`|GetDataTableRow` "/Game/ParallelBeam/Core/BPs/Data/DT_PlayerLevels.DT_PlayerLevels" _array_element)
      (:`then`
        (bind _returnvalue_2 (+ _array_index 1))
        (if (`KismetArrayLibrary.Array_IsValidIndex` _outrownames _returnvalue_2)
          (bind _returnvalue_3 (`|GetDataTableRow` "/Game/ParallelBeam/Core/BPs/Data/DT_PlayerLevels.DT_PlayerLevels" (`|GetArrayItem` _outrownames _returnvalue_2))
            (:`then`
              (if (and (> (`.Exp_2_259B735742EE5F385E9401B56F1863D4` (break `/Game/ParallelBeam/Core/BPs/Data/Structures/S_PlayerLevels` _returnvalue_3)) _currentexp) (>= _currentexp (`.Exp_2_259B735742EE5F385E9401B56F1863D4` (break `/Game/ParallelBeam/Core/BPs/Data/Structures/S_PlayerLevels` _returnvalue))))
                (set `self.CurrentPlayerLevel` (+ _array_index 1) :!label _label)
                (`self.OnPlayerExpUpdated`)
                (return)))
            (:`RowNotFound`
              (goto _label))))))))

(fn `UpdateStage`
  (params (NewStage :type Text) (Timer :type "Float (double-precision)"))
  (bind _output_get (set `self.CurrentStage` NewStage))
  (`self.StageUpdated` _output_get Timer)
  (`KismetSystemLibrary.LogString` (`KismetTextLibrary.Conv_TextToString` _output_get)))