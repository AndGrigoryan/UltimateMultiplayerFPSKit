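; BP_TargetButton is an interactable button that moves its referenced Targets when a character uses it.
; It always allows interaction and provides no icon or item name.
; StartInteract fires the interaction callback, then calls MoveTarget, which stores the Far flag and passes it to Targets.
; Interaction always sends Far as true, as the toggle logic is left unconnected.
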(event `self.ReceiveBeginPlay`)

(event `MoveTarget`
  (params (Far :type Boolean))
  (set `self.Far` Far)
  (`/Game/ParallelBeam/Core/BPs/Actors/Level/BP_Target.Move` (`self.Targets`) Far))

(fn `CanGetIcon`
  (returns (ReturnValue :type Boolean))
  (return false))

(fn `CanInteract`
  (params (Actor :type "Actor Object Reference"))
  (returns (`Return Value` :type Boolean))
  (return true))

(fn `GetIcon`
  (params (Stock :type Boolean))
  (returns (Texture :type "Texture Object Reference"))
  (return null))

(fn `GetInteractionInfo`
  (params (InteractingActor :type "Actor Object Reference"))
  (returns (Item :type Text) (Type :type Text) (HoldType :type Text))
  (return "" (`self.Interaction Text`) ""))

(fn `StartInteract`
  (params (Character :type "Character Object Reference"))
  (returns (`Return Value` :type Boolean))
  (`self.OnInteracted`)
  (`self.MoveTarget` true))

(fn `UserConstructionScript`)