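; BP_Explosive is an actor that explodes when it takes any damage.
; A short random delay precedes Explode, so nearby explosives can go off in a staggered chain.
; Explode runs once, applying radial damage with falloff credited to the owner and instigator, then calls the MLT effect event and destroys the actor.
; That event spawns a Niagara system and a sound at the actor's location.
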(event `self.ReceiveAnyDamage`
  (params (Damage :type "Float (single-precision)") (DamageType :type "DamageType Object Reference") (InstigatedBy :type "Controller Object Reference") (DamageCauser :type "Actor Object Reference"))
  (`KismetSystemLibrary.Delay` (`KismetMathLibrary.RandomFloatInRange` 0.1 0.2))
  (`self.Explode`))

(event `Explode`
  (`/Engine/EditorBlueprintResources/StandardMacros.DoOnce` false
    (:`Completed`
      (`GameplayStatics.ApplyRadialDamageWithFalloff` :`BaseDamage` (`self.Base Damage`) :`MinimumDamage` (`self.Minimum Damage`) :`Origin` (`self.K2_GetActorLocation`) :`DamageInnerRadius` (`self.Damage Inner Radius`) :`DamageOuterRadius` (`self.Damage Outer Radius`) :`DamageFalloff` (`self.Damage Falloff`) :`DamageTypeClass` (`self.Damage Type Class`) :`DamageCauser` (`self.GetOwner`) :`InstigatedByController` (`self.GetInstigatorController`))
      (`self.MLT_Effect`)
      (`self.K2_DestroyActor`))))

(event `MLT_Effect`
  (bind _returnvalue (`self.K2_GetActorLocation`))
  (`NiagaraFunctionLibrary.SpawnSystemAtLocation` (`self.System Template`) _returnvalue (struct) (`self.NiagraScale`) true true "AutoRelease")
  (`GameplayStatics.SpawnSoundAtLocation` (`self.Sound`) _returnvalue (struct) 1.0 1.0 0.0 null null))

(fn `UserConstructionScript`
  (`parent.UserConstructionScript`))