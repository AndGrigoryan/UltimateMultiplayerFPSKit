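; BP_WeaponGenerator is an interactable button that spawns a random weapon when used.
; Interaction calls SVR_GenerateWeapon and plays a timeline that moves the Cylinder vertically as a press animation.
; Generation line-traces downward through randomized points around SpawnArea, then spawns a random ClassToSpawnFrom entry at the hit, pitched sideways with random yaw.
; Spawned weapons receive BP_MasterSkin and the RandomizeAttachmentsOnSpawn setting.
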(event `SVR_GenerateWeapon`
  (bind _returnvalue (`KismetMathLibrary.RandomPointInBoundingBox` (`SceneComponent.K2_GetComponentLocation` (`self.Spawn Area`)) (25.0 25.0 1.0)))
  (bind _outhit (`KismetSystemLibrary.LineTraceSingleForObjects` (+ _returnvalue (0.0 0.0 100.0)) (+ _returnvalue (0.0 0.0 -100.0)) (`|MakeArray` "ObjectTypeQuery1" "ObjectTypeQuery7" :!type "EObjectTypeQuery Enum")))
  (bind (_bblockinghit _binitialoverlap _time _distance _location) (`GameplayStatics.BreakHitResult` _outhit))
  (if _bblockinghit
    (`|SpawnActorFromClass` (`KismetArrayLibrary.Array_Random` (`self.ClassToSpawnFrom`)) (`KismetMathLibrary.MakeTransform` _location (`KismetMathLibrary.MakeRotator` 0.0 90.0 (`KismetMathLibrary.RandomFloatInRange` 0.0 360.0))) "AlwaysSpawn" "MultiplyWithRoot" null "/Game/ParallelBeam/Core/BPs/Actors/BP_MasterSkin.BP_MasterSkin_C" (`self.Randomize Attachments On Spawn`) null)))

(event `PlayPressAniomation`
  (bind (_direction _newtrack_0) (`Timeline|Timeline` :!via `PlayFromStart`)
    (:`Update`
      (`SceneComponent.K2_SetRelativeLocation` (`self.Cylinder`) (`KismetMathLibrary.MakeVector` 0.0 0.0 _newtrack_0) false false))))

(fn `CanGetIcon`
  (returns (ReturnValue :type Boolean))
  (return false))

(fn `CanInteract`
  (params (Actor :type "Actor Object Reference"))
  (returns (`Return Value` :type Boolean))
  (return true))

(fn `GetIcon`
  (params (Stock :type Boolean))
  (returns (Texture :type "Texture Object Reference"))
  (return null))

(fn `GetInteractionInfo`
  (params (InteractingActor :type "Actor Object Reference"))
  (returns (Item :type Text) (Type :type Text) (HoldType :type Text))
  (return "Generate Weapon" "USE" ""))

(fn `StartInteract`
  (params (Character :type "Character Object Reference"))
  (returns (`Return Value` :type Boolean))
  (`self.SVR_GenerateWeapon`)
  (`self.PlayPressAniomation`)
  (return false))

(fn `UserConstructionScript`)