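; BP_MSK_MasterEquipment is a base Blueprint for stack-based usable equipment, such as throwables.
; Interact sets the UsingEquipment state, stops primary and secondary actions, and plays throw montages locally and through the server.
; Montages call Use_Equipment, which aims from camera and control rotation, then spawns the item server-side at that point or a socket, removing one stack.
; A DoOnce, reset on each server interact, prevents duplicate spawns from multiple montage instances.
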(event `self.Interact`
  (params (Trigger :type Boolean))
  (bind _return_value (`/Game/ParallelBeam/Core/BPs/FunctionLib/BFL_MSK.GetMSKCharacterInventory` (`self.GetOwner`)))
  ;[0 0 0] On interaction add the tag to action states And stop primary and secondary actions and play the throw montages
  (if Trigger
    (if (> (`AGR_ItemComponent.GetStackCount` (`self.BP_MSK_Item`)) 1)
      (bind _blocked (`/Game/ParallelBeam/Core/BPs/Components/BP_MSK_CharacterInventory.Change Action State` _return_value (struct :`TagName` "States.UsingEquipment") true))
      (if (not _blocked)
        (`/Game/ParallelBeam/Core/BPs/Components/BP_MSK_CharacterInventory.PrimaryAction` _return_value false)
        (`/Game/ParallelBeam/Core/BPs/Components/BP_MSK_CharacterInventory.SecondaryAction` _return_value false)
        (`/Game/ParallelBeam/Core/BPs/Components/BP_MSK_Montage.PlayMontage` (`/Game/ParallelBeam/Core/BPs/FunctionLib/BFL_MSK.GetMSK_MontageComponent` (`self.GetOwner`)) true false self (struct :`TagName` "Actions.Fire"))
        (`self.SVR_Interact` (struct :`TagName` "Actions.Fire"))))
    (else
      (`/Game/ParallelBeam/Core/BPs/Components/BP_MSK_Montage.EndMontage` (`/Game/ParallelBeam/Core/BPs/FunctionLib/BFL_MSK.GetMSK_MontageComponent` (`self.GetOwner`)) false self))))

(event `Use_Equipment`
  (params (Action :type "GameplayTag Structure"))
  (bind _returnvalue (`self.GetOwner`))
  (bind _spawnlocation (`self.SpawnLocation`))
  (bind _returnvalue_2 (`self.GetInstigatorController` _returnvalue))
  (bind _returnvalue_3 (`Controller.GetControlRotation` _returnvalue_2))
  ;[0 0 0] Spawning the equipment on server
  ; needs a do once node cuz eahc instance of montage is calling this function and can lead to multiple proectile spawning at the same time
  (`/Engine/EditorBlueprintResources/StandardMacros.IsValid` _returnvalue_2
    (:`Is Valid`
      (`SceneComponent.K2_SetWorldRotation` _spawnlocation _returnvalue_3 false false)
      (`SceneComponent.K2_SetWorldLocation` _spawnlocation (+ (* (`KismetMathLibrary.GetForwardVector` _returnvalue_3) 50.0) (`SceneComponent.K2_GetComponentLocation` (`self.GetComponentByClass` _returnvalue "/Script/Engine.CameraComponent"))) false false))
    (:`Is Not Valid`
      _))
  (`/Engine/EditorBlueprintResources/ActorMacros.Switch Has Authority`
    (:`Authority`
      (`/Engine/EditorBlueprintResources/StandardMacros.DoOnce` false :!label _label
        (:`Completed`
          (`self.SpawnItem` Action))))))

(event `SpawnItem`
  (params (Action :type "GameplayTag Structure"))
  ;[0 0 0] Spawning the equipment on server
  ; needs a do once node cuz eahc instance of montage is calling this function and can lead to multiple proectile spawning at the same time
  (`|SpawnActorFromClass` (`self.EquipmentToSpawn`) (select `bool` (`self.UseSocketLocationToSpawnAt`) :`false` (`SceneComponent.K2_GetComponentToWorld` (`self.SpawnLocation`)) :`true` (`SceneComponent.GetSocketTransform` (`|GetArrayItem` (`self.GetComponentsByTag` (`self.GetOwner`) "/Script/Engine.SkeletalMeshComponent" "MainMesh")) (`self.SocketName`) "RTS_World")) "AlwaysSpawn" "MultiplyWithRoot" self (`self.GetInstigator`))
  (`AGR_InventoryComponent.RemoveStacks` (`AGR_InventoryFunctionLibrary.GetInventoryComponent` (`self.GetOwner`)) (`|MakeArray` self :!type "Actor Object Reference") 1))

(event `SVR_Interact`
  (params (Action :type "GameplayTag Structure"))
  ;[0 0 0] Spawning the equipment on server
  ; needs a do once node cuz eahc instance of montage is calling this function and can lead to multiple proectile spawning at the same time
  (if (> (`AGR_ItemComponent.GetStackCount` (`self.BP_MSK_Item`)) 0)
    (bind _blocked (`/Game/ParallelBeam/Core/BPs/Components/BP_MSK_CharacterInventory.Change Action State` (`/Game/ParallelBeam/Core/BPs/FunctionLib/BFL_MSK.GetMSKCharacterInventory` (`self.GetOwner`)) (struct :`TagName` "States.UsingEquipment") true))
    (if (not _blocked)
      (`|ExecutionSequence`
        (:`then_0`
          (goto _label :!via `Reset`))
        (:`then_1`
          (`/Game/ParallelBeam/Core/BPs/Components/BP_MSK_Montage.PlayMontage` (`/Game/ParallelBeam/Core/BPs/FunctionLib/BFL_MSK.GetMSK_MontageComponent` (`self.GetOwner`)) false false self Action))))))

(fn `GetActionMontage`
  (params (Action :type "GameplayTag Structure") (DuelWelding :type Boolean))
  (returns (Character :type "AnimMontage Object Reference") (Weapon :type "AnimMontage Object Reference"))
  (bind (_character _weapon) (`/Game/ParallelBeam/Core/BPs/Data/DTA_WeaponAnimation.GetActionMontage` (`self.DT_Anims`) Action DuelWelding))
  (return _character _weapon))

(fn `GetAmmoType`
  (returns (`Return Value` :type "/Game/ParallelBeam/Core/BPs/Actors/BP_MasterAmmo Class Reference"))
  (return null))

(fn `GetAnimationData`
  (returns (`DT Animation` :type "/Game/ParallelBeam/Core/BPs/Data/DTA_WeaponAnimation Object Reference"))
  (return (`self.DT_Anims`)))

(fn `GetIsOnWeaponLayer`
  (returns (`Return Value` :type Boolean))
  (return false))

(fn `GetIsRightHanded`
  (returns (`Return Value` :type Boolean))
  (return false))

(fn `GetIsSingleHanded`
  (returns (`Return Value` :type Boolean))
  (return false))

(fn `GetMaxAmmo`
  (returns (MaxAmmo :type Integer))
  (return 0))

(fn `Reload`
  (returns (`Return Value` :type Boolean))
  (return false))

(fn `UserConstructionScript`)