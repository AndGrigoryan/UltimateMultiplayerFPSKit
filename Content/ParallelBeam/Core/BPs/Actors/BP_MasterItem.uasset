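; BP_MasterItem is the base inventory item actor, built around a BP_MSK_Item component and interactable for pickup by characters.
; Interaction picks it up if its inventory ID is empty or matches the picker's, and stack changes refresh the owner's HUD.
; Pickup and drop toggle the item's material setting through the character inventory.
; Drops animate along a curve-offset timeline lerp with a game-mode lifespan, or destroy the item when that lifetime isn't positive.
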(event `self.BP_MSK_Item.OnStackCountUpdated`
  (params (OldStackCount :type Integer64) (NewStackCount :type Integer64))
  (message `/Game/ParallelBeam/Core/BPs/Interfaces/BPI_HUD.UpdateGameUIValues` (`/Game/ParallelBeam/Core/BPs/FunctionLib/BFL_MSK.GetMSK_HUD` (`self.GetOwner`))))

(event `self.BP_MSK_Item.OnItemPickedUp`
  (params (InventoryComponent :type "AGR_InventoryComponent Object Reference"))
  (bind _asbp_msk_character_inventory (cast `/Game/ParallelBeam/Core/BPs/Components/BP_MSK_CharacterInventory` InventoryComponent))
  (`/Game/ParallelBeam/Core/BPs/Components/BP_MSK_CharacterInventory.ChangeItemMaterialSetting` _asbp_msk_character_inventory true self)
  (set `self.OwnerInventory` _asbp_msk_character_inventory)
  (`self.MLT_DroppingCancel`))

(event `MLT_Dropped`
  (params (DropLocation :type "Vector Structure") (Startlocation :type "Vector Structure"))
  (bind (_direction _lerp) (`Timeline|DropTimeline` :!via `PlayFromStart` :!label _label)
    (:`Update`
      (`self.K2_SetActorLocation` (+ (`KismetMathLibrary.VLerp` Startlocation DropLocation _lerp) (`CurveVector.GetVectorValue` (`self.DropTransformCurve`) _lerp))))))

(event `MLT_DroppingCancel`
  (goto _label :!via `Stop`))

(event `self.BP_MSK_Item.OnItemDropped`
  (params (InventoryComponent :type "AGR_InventoryComponent Object Reference") (DropLocation :type "Vector Structure (by ref)"))
  (bind _lifetime (message `/Game/ParallelBeam/Core/BPs/Interfaces/BPI_Gamemode.GetDroppedItemLifetime` (`GameplayStatics.GetGameMode`)))
  (if (> _lifetime 0.0)
    (`self.SetLifeSpan` _lifetime)
    (`self.K2_DetachFromActor` "KeepWorld" "KeepWorld" "KeepWorld")
    (`/Game/ParallelBeam/Core/BPs/Components/BP_MSK_CharacterInventory.ChangeItemMaterialSetting` (`self.OwnerInventory`) false self)
    (`self.MLT_Dropped` DropLocation (`self.K2_GetActorLocation` (`ActorComponent.GetOwner` InventoryComponent)))
    (else
      (`AGR_ItemComponent.DestroyItem` (`self.BP_MSK_Item`) InventoryComponent))))

(fn `CanGetIcon`
  (returns (ReturnValue :type Boolean))
  (return true))

(fn `CanInteract`
  (params (Actor :type "Actor Object Reference"))
  (returns (`Return Value` :type Boolean))
  (return (`self.CanItemBePickedUp` (`/Game/ParallelBeam/Core/BPs/FunctionLib/BFL_MSK.GetMSKCharacterInventory` Actor))))

(fn `CanItemBeDestroyed`
  (params (InventoryComponent :type "AGR_InventoryComponent Object Reference"))
  (returns (ReturnValue :type Boolean))
  (return true))

(fn `CanItemBeDropped`
  (params (InventoryComponent :type "AGR_InventoryComponent Object Reference"))
  (returns (ReturnValue :type Boolean))
  (return true))

(fn `CanItemBeEquipped`
  (params (InventoryComponent :type "AGR_InventoryComponent Object Reference") (Slot :type "GameplayTag Structure"))
  (returns (ReturnValue :type Boolean))
  (return true))

(fn `CanItemBePickedUp`
  (params (InventoryComponent :type "AGR_InventoryComponent Object Reference"))
  (returns (ReturnValue :type Boolean))
  (bind _returnvalue (`AGR_ItemComponent.GetInventoryID` (`self.BP_MSK_Item`)))
  (if (== (`AGR_InventoryComponent.InventoryID` InventoryComponent) _returnvalue)
    (return true)
    (else
      (return (`KismetStringLibrary.IsEmpty` _returnvalue)))))

(fn `CanItemBeUnequipped`
  (params (InventoryComponent :type "AGR_InventoryComponent Object Reference") (Slot :type "GameplayTag Structure"))
  (returns (ReturnValue :type Boolean))
  (return true))

(fn `CanItemBeUsed`
  (params (InventoryComponent :type "AGR_InventoryComponent Object Reference") (ActionType :type "GameplayTag Structure"))
  (returns (ReturnValue :type Boolean))
  (return true))

(fn `GetEquipmentSlots`
  (returns (Tag :type "GameplayTagContainer Structure") (EquipInAll :type Boolean))
  (return (`self.EquipableSlots`) (`self.Equip in All`)))

(fn `GetIcon`
  (params (Stock :type Boolean))
  (returns (Texture :type "Texture Object Reference"))
  (return (`self.StockICON`)))

(fn `GetInteractionInfo`
  (params (InteractingActor :type "Actor Object Reference"))
  (returns (Item :type Text) (Type :type Text) (HoldType :type Text))
  (return (`AGR_ItemComponent.ItemName` (`self.BP_MSK_Item`)) (`self.Interaction Type`) (`self.HOLD Interaction Type`)))

(fn `StartInteract`
  (params (Character :type "Character Object Reference"))
  (returns (`Return Value` :type Boolean))
  (bind _boutsuccess (`AGR_ItemComponent.PickUpItem` (`self.BP_MSK_Item`) (`AGR_InventoryFunctionLibrary.GetInventoryComponent` Character) true true true))
  (return _boutsuccess))

(fn `UserConstructionScript`
  (set `AGR_ItemComponent.ItemName` (`self.ItemName`) (`self.BP_MSK_Item`)))