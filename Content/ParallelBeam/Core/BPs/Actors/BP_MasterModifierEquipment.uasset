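; Base equipment item Blueprint that applies action modifiers to whoever carries it.
; On pickup, it passes its Modifiers to the inventory owner's MSK locomotion component, and on drop it applies them inversely to undo the effect.
; The construction script creates a dynamic material on the mesh's second material slot and sets its Icon texture from StockICON.
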(event `self.BP_MSK_Item.OnItemPickedUp`
  (params (InventoryComponent :type "AGR_InventoryComponent Object Reference"))
  (bind _return_value (`/Game/ParallelBeam/Core/BPs/FunctionLib/BFL_MSK.GetMSKLocomotionComponent` (`ActorComponent.GetOwner` InventoryComponent)))
  (`/Engine/EditorBlueprintResources/StandardMacros.IsValid` _return_value
    (:`Is Valid`
      (`/Game/ParallelBeam/Core/BPs/Components/BP_MSK_Locomotion.Modify Action Modifier` _return_value (`self.Modifiers`) false))))

(event `self.BP_MSK_Item.OnItemDropped`
  (params (InventoryComponent :type "AGR_InventoryComponent Object Reference") (DropLocation :type "Vector Structure (by ref)"))
  (bind _return_value (`/Game/ParallelBeam/Core/BPs/FunctionLib/BFL_MSK.GetMSKLocomotionComponent` (`ActorComponent.GetOwner` InventoryComponent)))
  (`/Engine/EditorBlueprintResources/StandardMacros.IsValid` _return_value
    (:`Is Valid`
      (`/Game/ParallelBeam/Core/BPs/Components/BP_MSK_Locomotion.Modify Action Modifier` _return_value (`self.Modifiers`) true))))

(fn `UserConstructionScript`
  (`parent.UserConstructionScript`)
  (bind _returnvalue (`PrimitiveComponent.CreateDynamicMaterialInstance` (`self.StaticMesh`) 1 (`PrimitiveComponent.GetMaterial` (`self.StaticMesh`) 1) "None"))
  (`MaterialInstanceDynamic.SetTextureParameterValue` _returnvalue "Icon" (`self.StockICON`)))