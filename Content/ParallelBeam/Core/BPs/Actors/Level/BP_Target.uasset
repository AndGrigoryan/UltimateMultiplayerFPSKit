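; Shooting-range style target actor that awards hit, kill and headshot Exp to the instigator's controller component.
; Point and radial damage feed one handler; when CanFold is set, depleted health folds the target via ABP_Target until it resets after a delay.
; Hits also play bone-specific reaction montages and spawn distance-scaled Niagara damage numbers, skipped on dedicated servers.
; Move drives a timeline that slides the target sideways to a random distance and back.
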(event `MarkDown`
  (params (IsDown :type Boolean))
  (bind _asabp_target (cast `/Game/ParallelBeam/Core/BPs/AnimBPs/ABP_Target` (`SkeletalMeshComponent.GetAnimInstance` (`self.SkeletalMesh`))))
  (set `/Game/ParallelBeam/Core/BPs/AnimBPs/ABP_Target.IsDown` IsDown _asabp_target)
  (set `self.IsDown` IsDown))

(event `self.ReceivePointDamage`
  (params (Damage :type "Float (single-precision)") (DamageType :type "DamageType Object Reference") (HitLocation :type "Vector Structure") (HitNormal :type "Vector Structure") (HitComponent :type "PrimitiveComponent Object Reference") (BoneName :type Name) (ShotFromDirection :type "Vector Structure") (InstigatedBy :type "Controller Object Reference") (DamageCauser :type "Actor Object Reference") (HitInfo :type "HitResult Structure (by ref)"))
  (`self.onDamaged` Damage HitLocation BoneName InstigatedBy))

(event `self.ReceiveRadialDamage`
  (params (DamageReceived :type "Float (single-precision)") (DamageType :type "DamageType Object Reference") (Origin :type "Vector Structure") (HitInfo :type "HitResult Structure (by ref)") (InstigatedBy :type "Controller Object Reference") (DamageCauser :type "Actor Object Reference"))
  (bind (_bblockinghit _binitialoverlap _time _distance _location _impactpoint _normal _impactnormal _physmat _hitactor _hitcomponent _hitbonename _bonename) (`GameplayStatics.BreakHitResult` HitInfo))
  (`self.onDamaged` DamageReceived _location _bonename InstigatedBy))

(event `onDamaged`
  (params (Damage :type "Float (single-precision)") (Location :type "Vector Structure") (Bone :type Name) (Instigator :type "Controller Object Reference"))
  (bind _returnvalue (`self.GetComponentByClass` Instigator "/Game/ParallelBeam/Core/BPs/Components/GameModeComponents/BP_ControllerComponent.BP_ControllerComponent_C"))
  (bind _returnvalue_2 (`KismetStringLibrary.Conv_NameToString` Bone))
  (if (not (`self.IsDown`))
    (`|ExecutionSequence`
      (:`then_0`
        (if (not (`self.CanFold`))
          (`/Game/ParallelBeam/Core/BPs/Components/GameModeComponents/BP_ControllerComponent.ConfirmedHit` _returnvalue 10 (struct :`TagName` "Exp.Hit") :!label _label)
          (else
            (bind _output_get (set `self.Health` (- (`self.Health`) Damage)))
            (if (> _output_get 0.0)
              (goto _label)
              (else
                (`/Game/ParallelBeam/Core/BPs/Components/GameModeComponents/BP_ControllerComponent.ConfirmedKill` _returnvalue 100 (`Controller.PlayerState` Instigator) (select `bool` (or (`KismetStringLibrary.Contains` _returnvalue_2 "neck") (== _returnvalue_2 "head")) :`false` (struct :`TagName` "Exp.Hit.Kill") :`true` (struct :`TagName` "Exp.Hit.Kill.HeadShot") :!type "GameplayTag Structure"))
                (`self.MarkDown` true)
                (`KismetSystemLibrary.Delay` (`self.ResetTime`))
                (`self.MarkDown` false)
                (set `self.Health` (`self.MaxHealth`)))))))
      (:`then_1`
        (switch `name` Bone
          (:`Default`
            (set `self.Montage` "/Game/ParallelBeam/UltimateFPSKit/Animations/Character/Additive/HitReaction/AS_Reaction_Torso.AS_Reaction_Torso"))
          (:`upperarm_l`
            (set `self.Montage` "/Game/ParallelBeam/UltimateFPSKit/Animations/Character/Additive/HitReaction/AS_Reaction_LeftArm.AS_Reaction_LeftArm"))
          (:`upperarm_r`
            (set `self.Montage` "/Game/ParallelBeam/UltimateFPSKit/Animations/Character/Additive/HitReaction/AS_Reaction_RightArm.AS_Reaction_RightArm"))
          (:`head`
            (set `self.Montage` "/Game/ParallelBeam/UltimateFPSKit/Animations/Character/Additive/HitReaction/AS_Reaction_Head.AS_Reaction_Head"))
          (:`thigh_l`
            (set `self.Montage` "/Game/ParallelBeam/UltimateFPSKit/Animations/Character/Additive/HitReaction/AS_Reaction_LeftLeg.AS_Reaction_LeftLeg"))
          (:`thigh_r`
            (set `self.Montage` "/Game/ParallelBeam/UltimateFPSKit/Animations/Character/Additive/HitReaction/AS_Reaction_RightLeg.AS_Reaction_RightLeg"))))
      (:`then_2`
        (if (not (`KismetSystemLibrary.IsDedicatedServer`))
          (`AnimInstance.PlaySlotAnimationAsDynamicMontage` (`SkeletalMeshComponent.GetAnimInstance` (`self.SkeletalMesh`)) (`self.Montage`) "DefaultSlot" 0.1 (`KismetMathLibrary.RandomFloatInRange` 0.15 0.25) (`KismetMathLibrary.RandomFloatInRange` 2.2 3.0) 1 -1.0 0.0)
          (bind _returnvalue_3 (`NiagaraFunctionLibrary.SpawnSystemAtLocation` "/Game/ParallelBeam/Core/VFX/NS_DamageNumber.NS_DamageNumber" Location (struct) (1.0 1.0 1.0) true true "AutoRelease"))
          (`PrimitiveComponent.SetRenderCustomDepth` _returnvalue_3 true)
          (`PrimitiveComponent.SetCustomDepthStencilValue` _returnvalue_3 1)
          (`NiagaraComponent.SetNiagaraVariableFloat` _returnvalue_3 "Scale" (`KismetMathLibrary.MapRangeUnclamped` (`self.GetDistanceTo` (`GameplayStatics.GetPlayerPawn` 0) self) 500.0 90000.0 100.0 5000.0))
          (bind _returnvalue_4 (`KismetMaterialLibrary.CreateDynamicMaterialInstance` "/Game/ParallelBeam/Core/VFX/Materials/M_DamageNumber_Inst.M_DamageNumber_Inst" "DamageMaterial"))
          (`NiagaraComponent.SetVariableMaterial` _returnvalue_3 "DamageMaterial" _returnvalue_4)
          (`MaterialInstanceDynamic.SetScalarParameterValue` _returnvalue_4 "DamageValue" Damage))))))

(event `Move`
  (params (Far :type Boolean))
  (bind (_returnvalue_roll _returnvalue_pitch _returnvalue_yaw) (`KismetMathLibrary.BreakRotator` (`self.K2_GetActorRotation`)))
  (bind _range (`self.Range`))
  (if Far
    (set `self.EndLocation` (+ (* (`self.GetActorRightVector`) (`KismetMathLibrary.RandomFloatInRange` (* _range 0.7) _range) -1.0) (`self.StartingLocation`)))
    (bind (_direction _move _rotation) (`Timeline|Timeline` :!label _label_2)
      (:`Update`
        (`self.K2_SetActorLocation` (`KismetMathLibrary.VLerp` (`self.StartingLocation`) (`self.EndLocation`) _move))
        (`self.K2_SetActorRotation` (`KismetMathLibrary.MakeRotator` _returnvalue_roll (`KismetMathLibrary.Lerp` (`self.StartingRotation`) 0.0 _rotation) _returnvalue_yaw))))
    (else
      (goto _label_2 :!via `Reverse`))))

(event `self.ReceiveBeginPlay`
  (set `self.StartingLocation` (`self.K2_GetActorLocation`)))

(fn `UserConstructionScript`
  (set `self.Health` (`self.MaxHealth`)))