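; BP_AmmoRefilPoint is an interactable ammo station that restocks the interacting character's equipment and weapon ammo.
; On interact, it sets every inventory item tagged Equipment, such as grenades, to its max stack count.
; For weapons in the primary, secondary and akimbo slots, it tops up existing ammo stacks of each weapon's ammo class.
; When none exist, it spawns that ammo actor far below the world origin and picks it up into the inventory.
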(fn `CanInteract`
  (params (Actor :type "Actor Object Reference"))
  (returns (`Return Value` :type Boolean))
  (return true))

(fn `GetInteractionInfo`
  (params (`Interacting Actor` :type "Actor Object Reference"))
  (returns (Item :type Text) (Type :type Text) (HoldType :type Text))
  (return "AMMO STATION" "REFIL" ""))

(fn `StartInteract`
  (params (Character :type "Character Object Reference"))
  (returns (`Return Value` :type Boolean))
  (locals (LOC_Inventory :type "AGR_InventoryComponent Object Reference"))
  (set `local.LOC_Inventory` (`AGR_InventoryFunctionLibrary.GetInventoryComponent` Character))
  ;[1 1 1] Refill Grenades
  (bind _returnvalue (`AGR_InventoryComponent.GetAllItemsByTags` (`local.LOC_Inventory`) (`|MakeArray` "Equipment" :!type "Name") false))
  (for _array_element _returnvalue
    (bind _returnvalue_2 (`AGR_InventoryFunctionLibrary.GetItemComponent` _array_element))
    (`AGR_ItemComponent.SetStackCount` _returnvalue_2 (`AGR_ItemComponent.MaxStackCount` _returnvalue_2)))
  ;[1 1 1] Checks for ammo for each weapon that we have equiped
  ; and sees if we need to refil thier ammo stacks or respawn new ones
  (for _array_element_2 (`|MakeArray` (`AGR_InventoryComponent.GetItemInSlot` (`local.LOC_Inventory`) (struct :`TagName` "CharacterSlots.Secondary")) (`AGR_InventoryComponent.GetItemInSlot` (`local.LOC_Inventory`) (struct :`TagName` "CharacterSlots.Primary")) (`AGR_InventoryComponent.GetItemInSlot` (`local.LOC_Inventory`) (struct :`TagName` "CharacterSlots.Secondary.Akimbo")) (`AGR_InventoryComponent.GetItemInSlot` (`local.LOC_Inventory`) (struct :`TagName` "CharacterSlots.Primary.Akimbo")) :!type "Object Object Reference")
    (`/Engine/EditorBlueprintResources/StandardMacros.IsValid` _array_element_2
      (:`Is Valid`
        (bind _return_value (message `/Game/ParallelBeam/Core/BPs/Interfaces/BPI_Weapon.GetAmmoType` _array_element_2))
        (bind _returnvalue_3 (`AGR_InventoryComponent.GetAllItemsByClass` (`local.LOC_Inventory`) _return_value))
        (if (`KismetArrayLibrary.Array_IsEmpty` _returnvalue_3)
          (bind _returnvalue_4 (`|SpawnActorFromClass` _return_value (`KismetMathLibrary.MakeTransform` (0.0 0.0 -10000.0)) "Undefined" "MultiplyWithRoot" null null))
          (`/Engine/EditorBlueprintResources/StandardMacros.IsValid` _returnvalue_4
            (:`Is Valid`
              (`AGR_ItemComponent.PickUpItem` (`AGR_InventoryFunctionLibrary.GetItemComponent` _returnvalue_4) (`local.LOC_Inventory`) true true false)))
          (else
            (for _array_element_3 _returnvalue_3
              (`/Engine/EditorBlueprintResources/StandardMacros.IsValid` _array_element_3
                (:`Is Valid`
                  (bind _returnvalue_5 (`AGR_InventoryFunctionLibrary.GetItemComponent` _array_element_3))
                  (`AGR_ItemComponent.SetStackCount` _returnvalue_5 (`AGR_ItemComponent.MaxStackCount` _returnvalue_5))))))))))
  (return true))

(fn `UserConstructionScript`)