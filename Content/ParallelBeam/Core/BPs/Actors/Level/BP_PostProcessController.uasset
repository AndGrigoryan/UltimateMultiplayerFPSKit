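; Level actor that applies the player's saved graphics settings to the post process volumes in the level.
; On BeginPlay it applies them and binds to the MSK game instance's settings-updated event to reapply on change.
; It loops over every PostProcessVolume, writing saved chromatic aberration, bloom, Lumen methods, lens flare, film grain, ambient occlusion and motion blur values.
; Lumen toggles between None and Lumen, while lens flare is remapped to an intensity range.
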(event `self.ReceiveBeginPlay`
  (add `/Game/ParallelBeam/Core/BPs/GameInstance/BP_MSKGameInstance.GameSettingsUpdated` (`/Game/ParallelBeam/Core/BPs/FunctionLib/BFL_MSK.Get MSKGameInstance` self) (delegate `ApplySettings`))
  (`self.ApplySettings`))

(event `ApplySettings`
  (bind _gamesettingssave (`/Game/ParallelBeam/Core/BPs/GameInstance/BP_MSKGameInstance.GameSettingsSave` (`/Game/ParallelBeam/Core/BPs/FunctionLib/BFL_MSK.Get MSKGameInstance` self)))
  (bind _return_value (`/Game/ParallelBeam/Core/BPs/Data/S_GameSettings.Get Int Value` _gamesettingssave "Lumen"))
  (bind _outactors (`GameplayStatics.GetAllActorsOfClass` "/Script/Engine.PostProcessVolume"))
  (for _array_element _outactors
    (bind _structout (setmembers `PostProcessSettings` :`StructRef` (`PostProcessVolume.Settings` _array_element) :`SceneFringeIntensity` (`/Game/ParallelBeam/Core/BPs/Data/S_GameSettings.GetFloatValue` _gamesettingssave "CHROMATICABERRATION") :`BloomIntensity` (`/Game/ParallelBeam/Core/BPs/Data/S_GameSettings.GetFloatValue` _gamesettingssave "Bloom") :`DynamicGlobalIlluminationMethod` (select `int` _return_value :`0` "None" :`1` "Lumen" :!type "EDynamicGlobalIlluminationMethod Enum") :`ReflectionMethod` (select `int` _return_value :`0` "None" :`1` "Lumen" :!type "EReflectionMethod Enum") :`LensFlareIntensity` (`KismetMathLibrary.MapRangeClamped` (`KismetMathLibrary.Conv_IntToDouble` (`/Game/ParallelBeam/Core/BPs/Data/S_GameSettings.Get Int Value` _gamesettingssave "LenseFlare")) 0.0 1.0 1.0 16.0) :`FilmGrainIntensity` (`/Game/ParallelBeam/Core/BPs/Data/S_GameSettings.GetFloatValue` _gamesettingssave "FILMGRAININTENSITY") :`AmbientOcclusionIntensity` (`/Game/ParallelBeam/Core/BPs/Data/S_GameSettings.GetFloatValue` _gamesettingssave "AMBIENTOCCLUSION") :`MotionBlurAmount` (`/Game/ParallelBeam/Core/BPs/Data/S_GameSettings.GetFloatValue` _gamesettingssave "MotionBlur")))
    (set `PostProcessVolume.Settings` _structout _array_element)))

(fn `UserConstructionScript`)