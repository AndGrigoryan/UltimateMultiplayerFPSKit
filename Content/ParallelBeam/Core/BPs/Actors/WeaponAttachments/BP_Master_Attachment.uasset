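; Base actor for weapon attachments, building a skeletal or static mesh from its attachment data.
; When the replicated inventory component updates, it snaps to the data's socket on the owner's "MainMesh"; skeletal meshes follow that mesh's pose.
; On unequip it waits a tick, hands nested attachments to the replacement's empty slots, then destroys its item unless re-equipped.
; Getters expose slot and data, with default scope, sway, montage and view values.
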(event `self.ReceiveBeginPlay`)

(event `self.BP_Attachment_Item.OnItemEquipped`
  (params (InventoryComponent :type "AGR_InventoryComponent Object Reference") (EquipmentSlot :type "GameplayTag Structure (by ref)"))
  (set `self.Inventory Component` InventoryComponent)
  (set `self.Equiped` true))

(event `self.BP_Attachment_Item.OnItemUnequipped`
  (params (InventoryComponent :type "AGR_InventoryComponent Object Reference") (EquipmentSlot :type "GameplayTag Structure (by ref)"))
  (bind _returnvalue (`AGR_InventoryComponent.GetItemInSlot` InventoryComponent EquipmentSlot))
  (bind _returnvalue_2 (`AGR_InventoryFunctionLibrary.GetInventoryComponent` _returnvalue))
  (bind _returnvalue_3 (`AGR_InventoryFunctionLibrary.GetInventoryComponent` self))
  (set `self.Equiped` false)
  (`KismetSystemLibrary.DelayUntilNextTick`)
  (`/Engine/EditorBlueprintResources/StandardMacros.IsValid` _returnvalue_3
    (:`Is Valid`
      (`/Engine/EditorBlueprintResources/StandardMacros.IsValid` _returnvalue
        (:`Is Valid`
          (`/Engine/EditorBlueprintResources/StandardMacros.IsValid` _returnvalue_2
            (:`Is Valid`
              (bind _keys (`BlueprintMapLibrary.Map_Keys` (`AGR_InventoryComponent.ActiveEquipmentSlotsMap` _returnvalue_3)))
              (for _array_element _keys
                (bind _returnvalue_4 (`AGR_InventoryComponent.GetItemInSlot` _returnvalue_3 _array_element))
                (`/Engine/EditorBlueprintResources/StandardMacros.IsValid` _returnvalue_4
                  (:`Is Valid`
                    (`/Engine/EditorBlueprintResources/StandardMacros.IsValid` (`AGR_InventoryComponent.GetItemInSlot` _returnvalue_2 _array_element)
                      (:`Is Not Valid`
                        (`AGR_ItemComponent.EquipItem` (`AGR_InventoryFunctionLibrary.GetItemComponent` _returnvalue_4) _returnvalue_2 _array_element true)))))))
            (:`Is Not Valid`
              _)))
        (:`Is Not Valid`
          _)))
    (:`Is Not Valid`
      _))
  (if (not (`self.Equiped`))
    (`AGR_ItemComponent.DestroyItem` (`self.BP_Attachment_Item`) InventoryComponent)))

(fn `GetAttachmentEffects`
  (returns (`Return Value` :type "Map of GameplayTag Structure to Float (double-precision)"))
  (return (`self.EffectsData`)))

(fn `GetAttachmentReloadMontage`
  (params (Action :type "GameplayTag Structure"))
  (returns (Char :type "AnimMontage Object Reference") (Wep :type "AnimMontage Object Reference"))
  (return null null))

(fn `GetAttachSlot`
  (returns (Slot :type "GameplayTagContainer Structure"))
  (return (`/Game/ParallelBeam/Core/BPs/Data/DTA_Attachment.EquipSlot` (`self.Attachment_Data`))))

(fn `GetDataAsset`
  (returns (DataAsset :type "/Game/ParallelBeam/Core/BPs/Data/DTA_Attachment Object Reference"))
  (return (`self.Attachment_Data`)))

(fn `GetScopeInfo`
  (returns (CameraFOV :type "Map of /Game/ParallelBeam/Core/BPs/Data/Enum/E_CameraType Enum to Float (double-precision)") (WeaponFOV :type "Float (double-precision)") (ScopeRingOffset :type "Float (double-precision)") (BlurAmmount :type "Float (double-precision)") (Sensetivity :type "Float (double-precision)"))
  (return _ 0.0 0.0 0.0 0.0))

(fn `GetSwaySettings`
  (returns (Sway :type "/Game/ParallelBeam/Core/BPs/Data/Structures/S_Sway Structure"))
  (return))

(fn `OnRep_Inventory Component`
  (bind _socketname (`/Game/ParallelBeam/Core/BPs/Data/DTA_Attachment.SocketName` (`self.Attachment_Data`)))
  (bind _output (`|GetArrayItem` (`self.GetComponentsByTag` (`ActorComponent.GetOwner` (`self.Inventory Component`)) "/Script/Engine.SceneComponent" "MainMesh")))
  (`|ExecutionSequence`
    (:`then_0`
      (`/Engine/EditorBlueprintResources/StandardMacros.IsValid` _output
        (:`Is Valid`
          (`self.K2_AttachToComponent` _output _socketname "SnapToTarget" "SnapToTarget" "SnapToTarget")
          (`SceneComponent.K2_SetWorldTransform` (`self.Scene`) (`SceneComponent.GetSocketTransform` _output _socketname "RTS_World") false false))))
    (:`then_1`
      (bind _skeletalcomponent (`self.SkeletalComponent`)
        (:`then`
          (bind _asskinned_mesh_component (cast `SkinnedMeshComponent` _output))
          (`SkinnedMeshComponent.SetLeaderPoseComponent` _skeletalcomponent _asskinned_mesh_component true false))
        (:`else`)))))

(fn `ShouldForceFPview`
  (returns (ReturnValue :type Boolean))
  (return false))

(fn `UseAlternateScopeAnim`
  (returns (`Return Value` :type Boolean))
  (return false))

(fn `UserConstructionScript`
  (bind _attachment_data (`self.Attachment_Data`))
  (bind _staticmesh (`self.StaticMesh`))
  (bind _skeletalmesh (`/Game/ParallelBeam/Core/BPs/Data/DTA_Attachment.SkeletalMesh` _attachment_data))
  (`/Engine/EditorBlueprintResources/StandardMacros.IsValid` _skeletalmesh
    (:`Is Valid`
      (`ActorComponent.K2_DestroyComponent` _staticmesh)
      (bind _returnvalue (`AddComponent|NODE_AddSkeletalMeshComponent-0` :`RelativeTransform` (`KismetMathLibrary.MakeTransform` (0.0 0.0 0.0))))
      (`SceneComponent.K2_AttachToComponent` _returnvalue (`self.Scene`) "None" "SnapToTarget" "SnapToTarget" "SnapToTarget" true)
      (`SkeletalMeshComponent.SetSkeletalMeshAsset` _returnvalue _skeletalmesh)
      (set `self.SkeletalComponent` _returnvalue))
    (:`Is Not Valid`
      (`StaticMeshComponent.SetStaticMesh` _staticmesh (`/Game/ParallelBeam/Core/BPs/Data/DTA_Attachment.StaticMesh` _attachment_data)))))