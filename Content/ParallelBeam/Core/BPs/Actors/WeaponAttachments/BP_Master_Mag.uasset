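; Base magazine attachment for weapons, which sets the ammo capacity of the weapon it is equipped to.
; On equip, it casts the inventory component's owner to BP_MSK_Master_Weapon, copies its MaxAmmo onto that weapon and sets the projectile launcher's ammo count to that full amount.
; GetAttachmentReloadMontage looks up an action in the Actions map and returns its paired character and weapon montages.
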(event `self.BP_Attachment_Item.OnItemEquipped`
  (params (InventoryComponent :type "AGR_InventoryComponent Object Reference") (EquipmentSlot :type "GameplayTag Structure (by ref)"))
  (bind _asbp_msk_master_weapon (cast `/Game/ParallelBeam/Core/BPs/Actors/BP_MSK_Master_Weapon` (`ActorComponent.GetOwner` InventoryComponent)))
  (bind _output_get (set `/Game/ParallelBeam/Core/BPs/Actors/BP_MSK_Master_Weapon.MaxAmmo` (`self.Max Ammo`) _asbp_msk_master_weapon))
  (`AGR_ProjectileLauncherComponent.SetAmmoCount` (`/Game/ParallelBeam/Core/BPs/Actors/BP_MSK_Master_Weapon.BP_MSK_ProjectileLauncher` _asbp_msk_master_weapon) _output_get))

(fn `GetAttachmentReloadMontage`
  (params (Action :type "GameplayTag Structure"))
  (returns (Char :type "AnimMontage Object Reference") (Wep :type "AnimMontage Object Reference"))
  (bind (_character _weapon) (break `/Game/ParallelBeam/Core/BPs/Data/Structures/S_WepMontage` (`BlueprintMapLibrary.Map_Find` (`self.Actions`) Action)))
  (return _character _weapon))

(fn `UserConstructionScript`
  (`parent.UserConstructionScript`))