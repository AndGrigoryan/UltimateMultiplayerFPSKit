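; BP_Lazer is a laser weapon attachment that renders a beam with a light at the point it hits.
; Each Tick, a long object-type line trace runs forward from the Cylinder, ignoring itself.
; The PointLight moves to the hit location or trace end.
; The Cylinder's X scale follows the distance to that point, clamped to a maximum, to stretch the beam.
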(event `self.ReceiveTick`
  (params (DeltaSeconds :type "Float (single-precision)"))
  (bind _cylinder (`self.Cylinder`))
  (bind _returnvalue (`SceneComponent.K2_GetComponentLocation` _cylinder))
  (bind _outhit (`KismetSystemLibrary.LineTraceSingleForObjects` _returnvalue (+ _returnvalue (* (`SceneComponent.GetForwardVector` _cylinder) 100000.0)) (`|MakeArray` "ObjectTypeQuery1" "ObjectTypeQuery2" "ObjectTypeQuery3" "ObjectTypeQuery5" "ObjectTypeQuery4" :!type "EObjectTypeQuery Enum") false (`|MakeArray` self :!type "Actor Object Reference")))
  (bind (_bblockinghit _binitialoverlap _time _distance _location _impactpoint _normal _impactnormal _physmat _hitactor _hitcomponent _hitbonename _bonename _hititem _elementindex _faceindex _tracestart _traceend) (`GameplayStatics.BreakHitResult` _outhit))
  (bind _output_get (set `self.EndLocation` (select `bool` _bblockinghit :`false` _traceend :`true` _location)))
  (`SceneComponent.K2_SetWorldLocation` (`self.PointLight`) (`self.EndLocation`) false false)
  (`SceneComponent.SetRelativeScale3D` (`self.Cylinder`) (`KismetMathLibrary.MakeVector` (`KismetMathLibrary.FClamp` (`KismetMathLibrary.Vector_Distance` _output_get (`SceneComponent.K2_GetComponentLocation` (`self.Cylinder`))) 0.0 5000.0) 1.0 1.0)))

(fn `UserConstructionScript`
  (`parent.UserConstructionScript`))