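; BP_Master_Sight is a master actor Blueprint for weapon sight attachments, holding each sight's aiming configuration.
; Getter functions expose scope info (camera and weapon FOV, scope ring offset, blur amount, aim sensitivity), sway settings, an alternate scope animation flag and a force-first-person-when-aiming flag.
; It is data-only in practice: the event graph and construction script add no logic of their own.
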(fn `GetScopeInfo`
  (returns (CameraFOV :type "Map of /Game/ParallelBeam/Core/BPs/Data/Enum/E_CameraType Enum to Float (double-precision)") (WeaponFOV :type "Float (double-precision)") (ScopeRingOffset :type "Float (double-precision)") (BlurAmmount :type "Float (double-precision)") (Sensetivity :type "Float (double-precision)"))
  (return (`self.CamerFOV`) (`self.WepFOV`) (`self.InnerFishEyeRadius`) (`self.Blur Ammount`) (`self.Aiming Sensetvity`)))

(fn `GetSwaySettings`
  (returns (Sway :type "/Game/ParallelBeam/Core/BPs/Data/Structures/S_Sway Structure"))
  (return (`self.Sway`)))

(fn `ShouldForceFPview`
  (returns (ReturnValue :type Boolean))
  (return (`self.ShouldForceFPViewWhenAiming`)))

(fn `UseAlternateScopeAnim`
  (returns (`Return Value` :type Boolean))
  (locals (NewLocalVar :type Boolean :default false))
  (return (`self.UseAlternateFireAnim`)))

(fn `UserConstructionScript`
  (`parent.UserConstructionScript`))