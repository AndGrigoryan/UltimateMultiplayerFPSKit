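; BP_MSK_FieldUpgrade is a field upgrade equipment Blueprint that adds a recharge cooldown to its parent's behavior.
; A looping one-second timer started on BeginPlay counts CurrentTime up, clamped to RechargeTime.
; Interact passes to the parent only once fully charged, while UseEquipment runs the parent logic and resets the charge to zero.
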(event `self.ReceiveBeginPlay`
  (`KismetSystemLibrary.K2_SetTimerDelegate` (delegate `UpdateCurrentTime`) 1.0 true))

(event `UpdateCurrentTime`
  (set `self.CurrentTime` (`KismetMathLibrary.FClamp` (+ (`self.CurrentTime`) 1.0) 0.0 (`self.RechargeTime`))))

(event `self.Interact`
  (params (Trigger :type Boolean))
  (if (>= (`self.CurrentTime`) (`self.RechargeTime`))
    (`parent.Interact` Trigger)))

(event `self.Use_Equipment`
  (params (Action :type "GameplayTag Structure"))
  (`parent.Use_Equipment` Action)
  (set `self.CurrentTime` 0.0))

(fn `UserConstructionScript`
  (`parent.UserConstructionScript`))