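; Base skin actor that reskins an item and its attachments when ApplySkin attaches it to that item.
; It resets "Skin"-tagged meshes to default materials, then applies body materials to the item and slot materials to attachments with matching equip-slot gameplay tags.
; Named material slots get dynamic instances that carry over listed scalar, vector and texture parameters from the replaced material.
; UseFOV is set on the original materials according to local player ownership.
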(event `ApplySkin`
  (params (Actor :type "Actor Object Reference"))
  (bind _output_get (set `self.OwnerActor` Actor))
  (bind _returnvalue (`self.GetOwner` _output_get))
  (`/Engine/EditorBlueprintResources/StandardMacros.IsValid` _returnvalue
    (:`Is Valid`
      (bind _returnvalue_2 (`self.GetInstigatorController` _returnvalue))
      (`/Engine/EditorBlueprintResources/StandardMacros.IsValid` _returnvalue_2
        (:`Is Valid`
          (set `self.LocalPlayer` (`Controller.IsLocalPlayerController` _returnvalue_2)))
        (:`Is Not Valid`
          _)))
    (:`Is Not Valid`
      _))
  (`self.K2_AttachToActor` Actor "None" "SnapToTarget" "SnapToTarget" "SnapToTarget")
  (`self.ResetMaterialsToDefault` (`self.OwnerActor`))
  (bind _return_value (`/Game/ParallelBeam/Core/BPs/Components/BP_AttachmentInventory.GetAllAttachments` (`/Game/ParallelBeam/Core/BPs/FunctionLib/BFL_MSK.GetAttachmentInventory` (`self.OwnerActor`))))
  (for _array_element _return_value
    (`self.ResetMaterialsToDefault` _array_element))
  (`self.ApplyMaterial` (`self.OwnerActor`) (`self.MainBodyMaterial`))
  (for _array_element_2 (`/Game/ParallelBeam/Core/BPs/Components/BP_AttachmentInventory.AllAttachments` (`/Game/ParallelBeam/Core/BPs/FunctionLib/BFL_MSK.GetAttachmentInventory` (`self.OwnerActor`)))
    (bind _dataasset (message `/Game/ParallelBeam/Core/BPs/Interfaces/BPI_Attachment.GetDataAsset` _array_element_2))
    (for _array_element_3 (`self.AttachmentMaterial`)
      (bind (_attachmenttagstoapplyon _skinsperslot) (break `/Game/ParallelBeam/Core/BPs/Data/Structures/S_AttachmentSlotMaterial` _array_element_3))
      (if (`BlueprintGameplayTagLibrary.HasAnyTags` (`/Game/ParallelBeam/Core/BPs/Data/DTA_Attachment.EquipSlot` _dataasset) _attachmenttagstoapplyon)
        (`self.ApplyMaterial` _array_element_2 _skinsperslot)))))

(fn `ApplyMaterial`
  (params (Actor :type "Actor Object Reference") (Material :type "Array of /Game/ParallelBeam/Core/BPs/Data/Structures/S_SkinData Structure"))
  (locals (Loc_ScalarParam :type "Map of Name to Float (double-precision)") (LOC_VectorParam :type "Map of Name to LinearColor Structure") (LOC_TexParam :type "Map of Name to Texture Object Reference") (LOC_CurrentMesh :type "PrimitiveComponent Object Reference"))
  (bind _loc_currentmesh (`local.LOC_CurrentMesh`))
  (bind _loc_scalarparam (`local.Loc_ScalarParam`))
  (bind _loc_vectorparam (`local.LOC_VectorParam`))
  (bind _loc_texparam (`local.LOC_TexParam`))
  (for _array_element (`self.GetComponentsByTag` Actor "/Script/Engine.PrimitiveComponent" "Skin")
    (set `local.LOC_CurrentMesh` _array_element)
    (for _array_element_2 (`local.Material`)
      (bind (_slotstoapplyon _materialdata) (break `/Game/ParallelBeam/Core/BPs/Data/Structures/S_SkinData` _array_element_2))
      (for _array_element_3 _slotstoapplyon
        (`BlueprintMapLibrary.Map_Clear` (`local.Loc_ScalarParam`))
        (`BlueprintMapLibrary.Map_Clear` (`local.LOC_VectorParam`))
        (`BlueprintMapLibrary.Map_Clear` (`local.LOC_TexParam`))
        (bind _returnvalue (`PrimitiveComponent.GetMaterialByName` _loc_currentmesh _array_element_3))
        (`/Engine/EditorBlueprintResources/StandardMacros.IsValid` _returnvalue
          (:`Is Valid`
            (bind _returnvalue_2 (`PrimitiveComponent.GetMaterialIndex` _loc_currentmesh _array_element_3))
            (bind _returnvalue_3 (`PrimitiveComponent.CreateDynamicMaterialInstance` (`local.LOC_CurrentMesh`) _returnvalue_2 _returnvalue "None"))
            (`MaterialInstanceDynamic.SetScalarParameterValue` _returnvalue_3 "UseFOV" (`KismetMathLibrary.Conv_BoolToDouble` (`self.LocalPlayer`)))
            (for _array_element_4 (`.ParametersToCopy_7_FE35D85349002C94DE129498A7EADFDB` (break `/Game/ParallelBeam/Core/BPs/Data/Structures/S_MaterialData` _materialdata))
              (bind _returnvalue_4 (`MaterialInstanceDynamic.K2_GetScalarParameterValue` _returnvalue_3 _array_element_4))
              (`BlueprintMapLibrary.Map_Add` (`local.Loc_ScalarParam`) _array_element_4 _returnvalue_4)
              (bind _returnvalue_5 (`MaterialInstanceDynamic.K2_GetVectorParameterValue` _returnvalue_3 _array_element_4))
              (`BlueprintMapLibrary.Map_Add` (`local.LOC_VectorParam`) _array_element_4 _returnvalue_5)
              (bind _returnvalue_6 (`MaterialInstanceDynamic.K2_GetTextureParameterValue` _returnvalue_3 _array_element_4))
              (`BlueprintMapLibrary.Map_Add` (`local.LOC_TexParam`) _array_element_4 _returnvalue_6))
            (bind _returnvalue_7 (`PrimitiveComponent.CreateDynamicMaterialInstance` (`local.LOC_CurrentMesh`) _returnvalue_2 (`.MaterialToApply_2_A924C11A4E172B1BF63CF4BEC00160FE` (break `/Game/ParallelBeam/Core/BPs/Data/Structures/S_MaterialData` _materialdata)) "None"))
            (bind _keys (`BlueprintMapLibrary.Map_Keys` _loc_scalarparam))
            (bind _values (`BlueprintMapLibrary.Map_Values` _loc_scalarparam))
            (for (_array_element_5 _array_index) _keys
              (`MaterialInstanceDynamic.SetScalarParameterValue` _returnvalue_7 _array_element_5 (`|GetArrayItem` _values _array_index)))
            (bind _keys_2 (`BlueprintMapLibrary.Map_Keys` _loc_texparam))
            (bind _values_2 (`BlueprintMapLibrary.Map_Values` _loc_texparam))
            (for (_array_element_6 _array_index_2) _keys_2
              (`MaterialInstanceDynamic.SetTextureParameterValue` _returnvalue_7 _array_element_6 (`|GetArrayItem` _values_2 _array_index_2)))
            (bind _keys_3 (`BlueprintMapLibrary.Map_Keys` _loc_vectorparam))
            (bind _values_3 (`BlueprintMapLibrary.Map_Values` _loc_vectorparam))
            (for (_array_element_7 _array_index_3) _keys_3
              (`MaterialInstanceDynamic.SetVectorParameterValue` _returnvalue_7 _array_element_7 (`|GetArrayItem` _values_3 _array_index_3)))))))))

(fn `ResetMaterialsToDefault`
  (params (Actor :type "Actor Object Reference"))
  (for _array_element (`self.GetComponentsByTag` Actor "/Script/Engine.StaticMeshComponent" "Skin")
    (for _array_element_2 (`StaticMesh.StaticMaterials` (`StaticMeshComponent.StaticMesh` _array_element))
      (bind (_materialinterface _materialslotname) (break `StaticMaterial` _array_element_2))
      (`PrimitiveComponent.SetMaterialByName` _array_element _materialslotname _materialinterface))
    (`MeshComponent.SetScalarParameterValueOnMaterials` _array_element "UseFOV" (`KismetMathLibrary.Conv_BoolToDouble` (`self.LocalPlayer`))))
  (for _array_element_3 (`self.GetComponentsByTag` Actor "/Script/Engine.SkeletalMeshComponent" "Skin")
    (bind _asskeletal_mesh (cast `SkeletalMesh` (`SkinnedMeshComponent.SkinnedAsset` _array_element_3)))
    (for _array_element_4 (`SkeletalMesh.Materials` _asskeletal_mesh)
      (bind (_materialinterface_2 _materialslotname_2) (break `SkeletalMaterial` _array_element_4))
      (`PrimitiveComponent.SetMaterialByName` _array_element_3 _materialslotname_2 _materialinterface_2))
    (`MeshComponent.SetScalarParameterValueOnMaterials` _array_element_3 "UseFOV" (`KismetMathLibrary.Conv_BoolToDouble` (`self.LocalPlayer`)))))

(fn `UserConstructionScript`)