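; Match HUD that creates and drives the player's in-game UI, from pause menu and loadout to kill feed, scoreboard, killer spectator and end screens.
; A lazily created master widget hosts the score tab and a swappable per-pawn UI, which receives crosshair, fire and hit-marker events.
; Experience events update the tracker and use gameplay tags to trigger hit or kill markers with sound.
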(event `self.ReceiveBeginPlay`
  (bind _scoretabwidget (`self.ScoreTabWidget`))
  ;[0 0 0] Creating master and Score widget and adding themt oscreen
  (bind _output_get (set `self.MasterWidget` (`self.Get Master Widget`)))
  (if (`KismetSystemLibrary.IsValidClass` _scoretabwidget)
    (bind _returnvalue (`|CreateWidget` _scoretabwidget))
    (bind _returnvalue_2 (`Overlay.AddChildToOverlay` (`/Game/ParallelBeam/Core/Widgets/Game/WB_MasterHud.OV_MatchInfoContainer` _output_get) _returnvalue))
    (`OverlaySlot.SetHorizontalAlignment` _returnvalue_2 "HAlign_Fill")
    (`OverlaySlot.SetVerticalAlignment` _returnvalue_2 "VAlign_Fill")))

(event `/Game/ParallelBeam/Core/BPs/Interfaces/BPI_HUD.PauseMenu`
  (params (Add :type Boolean))
  (bind _returnvalue (`self.GetOwningPlayerController`))
  (bind _returnvalue_2 (`self.GetOwningPlayerController`))
  (bind _settingsmenu (`self.SettingsMenu`))
  ;[0 0 0] Pause Menu
  (if Add
    (`self.SettingsMenu`
      (:`then`
        _)
      (:`else`
        (bind _returnvalue_3 (`|CreateWidget` "/Game/ParallelBeam/Core/Widgets/Game/WB_PauseMenu.WB_PauseMenu_C"))
        (set `self.SettingsMenu` _returnvalue_3)))
    (set `PlayerController.bShowMouseCursor` true _returnvalue_2)
    (`WidgetBlueprintLibrary.SetInputMode_UIOnlyEx` _returnvalue_2 _settingsmenu)
    (`UserWidget.AddToViewport` _settingsmenu 0)
    (else
      (bind _settingsmenu_2 (`self.SettingsMenu`)
        (:`then`
          (`Widget.RemoveFromParent` _settingsmenu_2)
          (set `PlayerController.bShowMouseCursor` false _returnvalue :!label _label)
          (`WidgetBlueprintLibrary.SetInputMode_GameOnly` _returnvalue))
        (:`else`)))))

(event `/Game/ParallelBeam/Core/BPs/Interfaces/BPI_HUD.ShowGameUI`
  (params (Show :type Boolean))
  ;[0 0 0] Update the in game (ammo and equipment)
  (`/Game/ParallelBeam/Core/Widgets/Game/WB_MasterHud.ShowGameUI` (`self.Get Master Widget`) Show))

(event `Exit`
  ;[0 0 0] Pause Menu
  (`Widget.RemoveFromParent` (`self.SettingsMenu`))
  (goto _label))

(event `/Game/ParallelBeam/Core/BPs/Interfaces/BPI_HUD.UpdateGameUIValues`
  (bind _masterwidget (`self.MasterWidget`))
  ;[0 0 0] Update the in game (ammo and equipment)
  (`/Engine/EditorBlueprintResources/StandardMacros.IsValid` _masterwidget
    (:`Is Valid`
      (`/Game/ParallelBeam/Core/Widgets/Game/WB_MasterHud.UpdateGameUIValues` _masterwidget)
      (`/Game/ParallelBeam/Core/Widgets/Game/PawnUIs/WB_MasterPawnUI.UpdateGameUIValues` (`self.CurrentPawnUI`)))))

(event `/Game/ParallelBeam/Core/BPs/Interfaces/BPI_HUD.SetInteractionText`
  (params (Actor :type "Actor Object Reference"))
  ;[0 0 0] Show interaction text
)

(event `/Game/ParallelBeam/Core/BPs/Interfaces/BPI_HUD.AddHitMarker`
  (params (Kill :type Boolean))
  ;[0 0 0] Hit Markers
  (`/Game/ParallelBeam/Core/Widgets/Game/PawnUIs/WB_MasterPawnUI.AddHitMarker` (`self.CurrentPawnUI`) Kill)
  (`GameplayStatics.PlaySound2D` (select `bool` Kill :`false` "/Game/ParallelBeam/DEMO/EpicContent/Audio/MetaSounds/sfx_Character_DamageGiven_nl_meta.sfx_Character_DamageGiven_nl_meta" :`true` "/Game/ParallelBeam/DEMO/EpicContent/Audio/MetaSounds/sfx_Character_DamageTaken_nl_meta.sfx_Character_DamageTaken_nl_meta" :!type "SoundBase Object Reference") 0.5 1.0 0.0 null null))

(event `/Game/ParallelBeam/Core/BPs/Interfaces/BPI_HUD.ShowLoadout`
  (params (Show :type Boolean))
  (bind _masterwidget (`self.MasterWidget`))
  ;[0 0 0] Show Loadout
  (`/Engine/EditorBlueprintResources/StandardMacros.IsValid` _masterwidget
    (:`Is Valid`
      (`/Game/ParallelBeam/Core/Widgets/Game/WB_CharacterReadyScreen.ShowLoadout` (`/Game/ParallelBeam/Core/Widgets/Game/WB_MasterHud.WB_loadOutSelection` _masterwidget) Show))))

(event `/Game/ParallelBeam/Core/BPs/Interfaces/BPI_HUD.AddKillFeedElement`
  (params (Killer :type "PlayerState Object Reference") (Killed :type "PlayerState Object Reference") (DamageCauser :type "Actor Object Reference"))
  (bind _wb_killfeed (`/Game/ParallelBeam/Core/Widgets/Game/WB_MasterHud.WB_KillFeed` (`self.MasterWidget`)))
  ;[0 0 0] Add KillFeedElement
  (`/Engine/EditorBlueprintResources/StandardMacros.IsValid` DamageCauser
    (:`Is Valid`
      (bind _texture (message `/Game/ParallelBeam/Core/BPs/Interfaces/BPI_Interaction.GetIcon` DamageCauser true))
      (bind _astexture_2d (cast `Texture2D` _texture)
        (:`then`
          (`/Game/ParallelBeam/Core/Widgets/Game/Elements/WB_KillFeed.AddKillMessage` _wb_killfeed Killer Killed _astexture_2d))
        (:`CastFailed`
          (`/Game/ParallelBeam/Core/Widgets/Game/Elements/WB_KillFeed.AddKillMessage` _wb_killfeed Killer Killed null :!label _label_2))))
    (:`Is Not Valid`
      (goto _label_2))))

(event `/Game/ParallelBeam/Core/BPs/Interfaces/BPI_HUD.ShowKillerScreen`
  (params (KillerPawn :type "Pawn Object Reference") (Actor :type "Actor Object Reference") (Duration :type "Float (double-precision)"))
  ;[0 0 0] Show the Spectator Killer screen
  (`/Engine/EditorBlueprintResources/StandardMacros.IsValid` (`self.DeathSpectatorWidget`)
    (:`Is Valid`
      _)
    (:`Is Not Valid`
      (bind _returnvalue (`|CreateWidget` "/Game/ParallelBeam/Core/Widgets/Game/Elements/WB_Spectator.WB_Spectator_C"))
      (bind _output_get (set `self.DeathSpectatorWidget` _returnvalue))
      (`UserWidget.AddToViewport` _output_get 0)))
  (`/Game/ParallelBeam/Core/Widgets/Game/Elements/WB_Spectator.SetKiller` (`self.DeathSpectatorWidget`) KillerPawn Actor Duration))

(event `/Game/ParallelBeam/Core/BPs/Interfaces/BPI_HUD.MatchEndScreen`
  (params (Win :type Boolean) (Draw :type Boolean))
  ;[0 0 0] Show End Match Screen
  (bind _returnvalue (`|CreateWidget` "/Game/ParallelBeam/Core/Widgets/Game/Elements/WB_EndGameScreen.WB_EndGameScreen_C" null Win Draw))
  (`UserWidget.AddToViewport` _returnvalue 0))

(event `/Game/ParallelBeam/Core/BPs/Interfaces/BPI_HUD.ShowScoreBoard`
  (params (Show :type Boolean))
  (bind _scoreboardwidget (`self.ScoreBoardWidget`))
  ;[0 0 0] Show ScoreBoard
  (`/Engine/EditorBlueprintResources/StandardMacros.IsValid` (`self.ScoreBoard`)
    (:`Is Valid`
      (`Widget.SetVisibility` (`self.ScoreBoard`) (select `bool` Show :`false` "Collapsed" :`true` "Visible" :!type "ESlateVisibility Enum") :!label _label_3))
    (:`Is Not Valid`
      (if (`KismetSystemLibrary.IsValidClass` _scoreboardwidget)
        (bind _returnvalue (`|CreateWidget` _scoreboardwidget))
        (bind _output_get (set `self.ScoreBoard` _returnvalue))
        (`UserWidget.AddToViewport` _output_get 0)
        (goto _label_3)))))

(event `/Game/ParallelBeam/Core/BPs/Interfaces/BPI_HUD.AddExperiencePoint`
  (params (Exp :type Integer) (Reason :type "GameplayTag Structure"))
  ;[0 0 0] Add Experience points tothe HUD
  (`/Game/ParallelBeam/Core/Widgets/Game/Elements/WB_ExpTracker.Add_Score` (`/Game/ParallelBeam/Core/Widgets/Game/WB_MasterHud.WB_ExpTracker` (`self.MasterWidget`)) Reason Exp)
  (if (`BlueprintGameplayTagLibrary.MatchesTag` Reason (struct :`TagName` "Exp.Hit"))
    (`self.AddHitMarker` (`BlueprintGameplayTagLibrary.MatchesTag` Reason (struct :`TagName` "Exp.Hit.Kill")))))

(event `/Game/ParallelBeam/Core/BPs/Interfaces/BPI_HUD.UpdatePawnUI`
  (params (Widget :type "/Game/ParallelBeam/Core/Widgets/Game/PawnUIs/WB_MasterPawnUI Class Reference"))
  (bind _currentpawnui (`self.CurrentPawnUI`))
  (bind (_value _returnvalue) (`BlueprintMapLibrary.Map_Find` (`self.PawnUIStack`) Widget))
  (bind _pawnuistack (`/Game/ParallelBeam/Core/Widgets/Game/WB_MasterHud.PawnUIStack` (`self.MasterWidget`)))
  ;[0 0 0] Change Pawn UI (Character,vehicle and such)
  (if (`KismetSystemLibrary.IsValidClass` Widget)
    (if _returnvalue
      (set `self.CurrentPawnUI` _value)
      (else
        (bind _returnvalue_2 (`|CreateWidget` Widget))
        (set `self.CurrentPawnUI` _returnvalue_2)))
    (`PanelWidget.ClearChildren` _pawnuistack)
    (bind _returnvalue_3 (`Overlay.AddChildToOverlay` _pawnuistack _currentpawnui))
    (`CommonActivatableWidget.ActivateWidget` _currentpawnui)
    (`OverlaySlot.SetVerticalAlignment` _returnvalue_3 "VAlign_Fill")
    (`OverlaySlot.SetHorizontalAlignment` _returnvalue_3 "HAlign_Fill")
    (else
      (`PanelWidget.ClearChildren` (`/Game/ParallelBeam/Core/Widgets/Game/WB_MasterHud.PawnUIStack` (`self.MasterWidget`))))))

(event `/Game/ParallelBeam/Core/BPs/Interfaces/BPI_HUD.SetCrosshair`
  (params (Crosshair :type "/Game/ParallelBeam/Core/Widgets/Game/Croshairs/WB_MasterCrossHair Class Reference"))
  (`/Game/ParallelBeam/Core/Widgets/Game/PawnUIs/WB_MasterPawnUI.SetCrosshair` (`self.CurrentPawnUI`) Crosshair))

(event `/Game/ParallelBeam/Core/BPs/Interfaces/BPI_HUD.WeaponFired`
  (`/Game/ParallelBeam/Core/Widgets/Game/PawnUIs/WB_MasterPawnUI.WeaponFired` (`self.CurrentPawnUI`)))

(fn `Get Master Widget`
  (returns (ReturnValue :type "/Game/ParallelBeam/Core/Widgets/Game/WB_MasterHud Object Reference"))
  (bind _masterwidget (`self.MasterWidget`)
    (:`then`
      (return _masterwidget))
    (:`else`
      (bind _returnvalue (`|CreateWidget` "/Game/ParallelBeam/Core/Widgets/Game/WB_MasterHud.WB_MasterHud_C"))
      (`UserWidget.AddToViewport` _returnvalue 0)
      (bind _output_get (set `self.MasterWidget` _returnvalue))
      (return _output_get))))

(fn `UserConstructionScript`)