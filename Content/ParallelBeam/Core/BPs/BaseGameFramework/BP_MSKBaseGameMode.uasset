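; Base game mode for team matches, handling player flow, kill scoring and feed, round resets and match end.
; Controllers join GameState team components round-robin, AI controllers fill or free slots on login, and reaching the minimum player count starts the match.
; Pawns spawn at team-tagged PlayerStarts during play, otherwise as tagged spectators.
; Score and round-update events are empty hooks; match end destroys the session and returns to the main menu.
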(event `/Game/ParallelBeam/Core/BPs/Interfaces/BPI_Gamemode.AddKill`
  (params (Killer :type "Controller Object Reference") (Killed :type "Controller Object Reference") (DamageCauser :type "Actor Object Reference"))
  (bind _playerstate (`Controller.PlayerState` Killed))
  (bind _playerstate_2 (`Controller.PlayerState` Killer))
  ;[0.151 0.151 0.151] On Kill Achived Logic
  (`/Engine/EditorBlueprintResources/StandardMacros.IsValid` _playerstate
    (:`Is Valid`
      ;;[0 0 0] Adding Kills and deaths for score to appropriate Player States
      (`/Game/ParallelBeam/Core/BPs/Components/GameModeComponents/BP_PlayerState_PS_Component.AddKill` (`/Game/ParallelBeam/Core/BPs/FunctionLib/BFL_MSK.GetPlayerStateComponent` _playerstate_2))
      (`/Game/ParallelBeam/Core/BPs/Components/GameModeComponents/BP_PlayerState_PS_Component.AddDeath` (`/Game/ParallelBeam/Core/BPs/FunctionLib/BFL_MSK.GetPlayerStateComponent` _playerstate))
      ;;[0 0 0] Kill Feed Message
      (for _array_element (`GameStateBase.PlayerArray` (`GameplayStatics.GetGameState`))
        (`/Game/ParallelBeam/Core/BPs/Components/GameModeComponents/BP_PlayerState_PS_Component.AddKillFeedMessage` (`/Game/ParallelBeam/Core/BPs/FunctionLib/BFL_MSK.GetPlayerStateComponent` _array_element) _playerstate_2 _playerstate DamageCauser)))))

(event `/Game/ParallelBeam/Core/BPs/Interfaces/BPI_Gamemode.AddNewController`
  (params (Controller :type "Controller Object Reference"))
  (bind _return_value (`/Game/ParallelBeam/Core/BPs/FunctionLib/BFL_MSK.Get GameStateTeamComponent` (`GameplayStatics.GetGameState`) (`self.NextPlayerIndex`)))
  ;[0.151 0.151 0.151] Post Login
  ;;[0 0 0] Distributing the Players To different teams
  (`/Engine/EditorBlueprintResources/StandardMacros.IsValid` _return_value
    (:`Is Valid`
      _)
    (:`Is Not Valid`
      (set `self.NextPlayerIndex` 0)))
  (`/Game/ParallelBeam/Core/BPs/Components/GameModeComponents/BP_GameStateTeam_Component.AddPlayer` _return_value (`Controller.PlayerState` Controller))
  (`/Engine/EditorBlueprintResources/StandardMacros.IncrementInt` (`self.NextPlayerIndex`)
    (:`  `
      ;;[0 0 0] Once Required Number of players are met Starts the match and Set the Started time
      (if (>= (`GameplayStatics.GetNumPlayerControllers`) (`self.MinumumNumberOfPlayers`))
        (`/Engine/EditorBlueprintResources/StandardMacros.DoOnce` false
          (:`Completed`
            ;;;[1 1 1] RequiredDelay to make sure evenything i set
            (`KismetSystemLibrary.Delay` 1.0)
            (`/Game/ParallelBeam/Core/BPs/Components/GameModeComponents/BP_GameStateTracker.SetStartedTime` (`self.GetComponentByClass` (`GameplayStatics.GetGameState`) "/Game/ParallelBeam/Core/BPs/Components/GameModeComponents/BP_GameStateTracker.BP_GameStateTracker_C"))
            (set `self.MatchInProgress` true)))))))

(event `self.ReceiveBeginPlay`
  (bind _returnvalue (`GameplayStatics.GetGameState`))
  (bind _return_value (`/Game/ParallelBeam/Core/BPs/FunctionLib/BFL_MSK.GetGameStatTracker` _returnvalue))
  ;[0.151 0.151 0.151] Storing the TeamGameStates so we its easier to work with In Child instances
  (for _array_element (`self.K2_GetComponentsByClass` _returnvalue "/Game/ParallelBeam/Core/BPs/Components/GameModeComponents/BP_GameStateTeam_Component.BP_GameStateTeam_Component_C")
    (`BlueprintMapLibrary.Map_Add` (`self.TeamComponents`) (`/Game/ParallelBeam/Core/BPs/Components/GameModeComponents/BP_GameStateTeam_Component.TeamIndex` _array_element) _array_element))
  (`/Engine/EditorBlueprintResources/StandardMacros.IsValid` _return_value
    (:`Is Valid`
      (bind _output_get (set `self.GameStatTracker` _return_value))
      (add `/Game/ParallelBeam/Core/BPs/Components/GameModeComponents/BP_GameStateTracker.OnRoundUpdated` _output_get (`|CreateDelegate` :!event `OnRoundUpdated`)))))

(event `self.K2_PostLogin`
  (params (NewPlayer :type "PlayerController Object Reference"))
  (`parent.K2_PostLogin` NewPlayer)
  (`|ExecutionSequence`
    (:`then_0`
      (while (and (< (`GameplayStatics.GetNumPlayerStates`) (`self.MaxPlayers`)) (< (`self.AiControllersCount`) (`self.MaximumNumberOfAIs`)))
        (`|SpawnActorFromClass` (`self.AIControllerClass`) (`KismetMathLibrary.MakeTransform` (0.0 0.0 -4000.0)) "Undefined" "MultiplyWithRoot" null null)
        (bind _outactors (`GameplayStatics.GetAllActorsOfClass` "/Script/AIModule.AIController"))
        (set `self.AiControllersCount` (`KismetArrayLibrary.Array_Length` _outactors))))
    (:`then_1`
      (while (> (`GameplayStatics.GetNumPlayerStates`) (`self.MaxPlayers`))
        (bind _outactors_2 (`GameplayStatics.GetAllActorsOfClass` "/Script/AIModule.AIController"))
        (`self.K2_DestroyActor` (`|GetArrayItem` _outactors_2))
        (`self.K2_DestroyActor` (`Controller.PlayerState` (`|GetArrayItem` _outactors_2))))
      (bind _outactors_3 (`GameplayStatics.GetAllActorsOfClass` "/Script/AIModule.AIController"))
      (set `self.AiControllersCount` (`KismetArrayLibrary.Array_Length` _outactors_3)))))

(event `/Game/ParallelBeam/Core/BPs/Interfaces/BPI_Gamemode.Trigger End Match`
  (params (WiningTeamIndex :type Integer))
  ;[0.151 0.151 0.151] Trigger End game
  (`/Engine/EditorBlueprintResources/StandardMacros.DoOnce` false
    (:`Completed`
      (set `self.MatchInProgress` false)
      (`/Game/ParallelBeam/Core/BPs/Components/GameModeComponents/BP_GameStateTeam_Component.MatchEnded` (`self.K2_GetComponentsByClass` (`GameplayStatics.GetGameState`) "/Game/ParallelBeam/Core/BPs/Components/GameModeComponents/BP_GameStateTeam_Component.BP_GameStateTeam_Component_C") WiningTeamIndex)
      (`KismetSystemLibrary.Delay` 5.0)
      (`DestroySessionCallbackProxy.DestroySession` (`GameplayStatics.GetPlayerController` 0)
        (:`OnSuccess`
          _)
        (:`OnFailure`
          _))
      (`GameplayStatics.OpenLevelBySoftObjectPtr` "/Game/ParallelBeam/UltimateFPSKit/MAPs/M_MainMenu.M_MainMenu"))))

(event `/Game/ParallelBeam/Core/BPs/Interfaces/BPI_Gamemode.ScoreUpdated`
  (params (TeamComponent :type "/Game/ParallelBeam/Core/BPs/Components/GameModeComponents/BP_GameStateTeam_Component Object Reference")))

(event `/Game/ParallelBeam/Core/BPs/Interfaces/BPI_Gamemode.ResetRound`
  (bind _gamestattracker (`self.GameStatTracker`))
  (bind _outactors (`GameplayStatics.GetAllActorsOfClass` "/Script/Engine.Pawn"))
  (`self.K2_DestroyActor` _outactors)
  (bind _outactors_2 (`GameplayStatics.GetAllActorsOfClass` "/Game/ParallelBeam/Core/BPs/Actors/BP_MasterItem.BP_MasterItem_C"))
  (`self.K2_DestroyActor` _outactors_2)
  (set `self.MatchInProgress` false)
  (`KismetSystemLibrary.Delay` (`/Game/ParallelBeam/Core/BPs/Components/GameModeComponents/BP_GameStateTracker.WaitTimeBetweenRounds` (`self.GameStatTracker`)))
  (set `self.MatchInProgress` true)
  (bind _outactors_3 (`GameplayStatics.GetAllActorsOfClass` "/Script/Engine.Controller"))
  (for _array_element _outactors_3
    (`/Game/ParallelBeam/Core/BPs/Components/GameModeComponents/BP_ControllerComponent.PlayerReset` (`self.GetComponentByClass` _array_element "/Game/ParallelBeam/Core/BPs/Components/GameModeComponents/BP_ControllerComponent.BP_ControllerComponent_C")))
  (`/Game/ParallelBeam/Core/BPs/Components/GameModeComponents/BP_GameStateTracker.ResetTime` _gamestattracker (`/Game/ParallelBeam/Core/BPs/Components/GameModeComponents/BP_GameStateTracker.RoundTime` _gamestattracker)))

(event `OnRoundUpdated`)

(fn `CheckMatchInProgress`
  (returns (`Return Value` :type Boolean))
  (return (`self.MatchInProgress`)))

(fn `GetDroppableItems`
  (returns (EquipmentsToDrop :type "GameplayTagContainer Structure") (ItemsTagsToDrop :type "Array of Text"))
  (return (`self.Equipments to Drop`) (`self.Items Tags to Drop`)))

(fn `GetDroppedItemLifetime`
  (returns (LifeTime :type "Float (double-precision)"))
  (return (`self.DroppedItemLifeTime`)))

(fn `PlayerCanRestart`
  (params (Player :type "PlayerController Object Reference"))
  (returns (ReturnValue :type Boolean))
  (bind _returnvalue (`parent.PlayerCanRestart` Player))
  (return (and _returnvalue (`self.MatchInProgress`))))

(fn `SpawnDefaultPawnFor`
  (params (NewPlayer :type "Controller Object Reference") (StartSpot :type "Actor Object Reference"))
  (returns (ReturnValue :type "Pawn Object Reference"))
  (if (`self.MatchInProgress`)
    (bind _outactors (`GameplayStatics.GetAllActorsOfClassWithTag` "/Script/Engine.PlayerStart" (`KismetStringLibrary.Conv_StringToName` (`KismetStringLibrary.Conv_IntToString` (`/Game/ParallelBeam/Core/BPs/Components/GameModeComponents/BP_PlayerState_PS_Component.TeamIndex` (`/Game/ParallelBeam/Core/BPs/FunctionLib/BFL_MSK.GetPlayerStateComponent` (`Controller.PlayerState` NewPlayer))))) :!label _label))
    (bind _returnvalue (`parent.SpawnDefaultPawnFor` NewPlayer (`KismetArrayLibrary.Array_Random` _outactors)))
    (`/Engine/EditorBlueprintResources/StandardMacros.IsValid` _returnvalue
      (:`Is Valid`
        (return _returnvalue))
      (:`Is Not Valid`
        (goto _label)))
    (else
      (bind _returnvalue_2 (`|SpawnActorFromClass` "/Script/Engine.Pawn" (`self.GetTransform` (`self.K2_FindPlayerStart` NewPlayer)) "Undefined" "MultiplyWithRoot" null null))
      (`KismetArrayLibrary.Array_Add` (`Actor.Tags` _returnvalue_2) "Spectator")
      (return _returnvalue_2))))

(fn `UserConstructionScript`
  (`parent.UserConstructionScript`))