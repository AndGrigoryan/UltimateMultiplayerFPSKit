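; Map zone actor that registers itself with the BP_MapTracker on an overlapping actor's instigator controller and captures layered map textures.
; Begin and end overlaps add or remove the zone, with a delayed BeginPlay check for actors already inside.
; Capture centers each layer's orthographic scene capture on the zone, rendering only tagged actors, optionally at game start.
; It also provides layer lookup by tag and maintains additional marker layers, signaling updates.
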(event `self.ReceiveBeginPlay`
  ;[0.1927 0.1927 0.1927] InitialBinding and checking if player is already overlaping the actor
  (add `self.OnActorBeginOverlap` (delegate `OnActorBeginOverlap_Event`))
  (add `self.OnActorEndOverlap` (delegate `OnActorEndOverlap_Event`))
  (`KismetSystemLibrary.Delay` (`self.DelayForInitialCollisionCheck`))
  (for _array_element (`PrimitiveComponent.GetOverlappingActors` (`self.OverLayCube`) null)
    (`self.AddMapToTracker` true _array_element))
  (if (`self.CaptureOnGameStart`)
    (`self.Capture`)))

(event `OnActorBeginOverlap_Event` :!signature `self.OnActorBeginOverlap`
  (params (OverlappedActor :type "Actor Object Reference") (OtherActor :type "Actor Object Reference"))
  ;[0.1927 0.1927 0.1927] InitialBinding and checking if player is already overlaping the actor
  (`self.AddMapToTracker` true OtherActor))

(event `OnActorEndOverlap_Event` :!signature `self.OnActorEndOverlap`
  (params (OverlappedActor :type "Actor Object Reference") (OtherActor :type "Actor Object Reference"))
  ;[0.1927 0.1927 0.1927] InitialBinding and checking if player is already overlaping the actor
  (`self.AddMapToTracker` false OtherActor))

(event `AddMapToTracker`
  (params (Add :type Boolean) (Actor :type "Actor Object Reference"))
  (bind _returnvalue (`self.GetInstigatorController` Actor))
  (bind _returnvalue_2 (`self.GetComponentByClass` _returnvalue "/Game/ParallelBeam/UltimateMapSystem/BPs/Components/BP_MapTracker.BP_MapTracker_C"))
  ;[0.1927 0.1927 0.1927] Whenever player enters a new zone we keep a track of it, so we can always update the players map
  ; ie, If you went from z1 to z2 to z3, then exited z3 we would know to put you back in z2, if you exited z2 before exiting z3 then after leaving z3 you would be put back in z1
  (`/Engine/EditorBlueprintResources/StandardMacros.IsValid` _returnvalue
    (:`Is Valid`
      (`/Engine/EditorBlueprintResources/StandardMacros.IsValid` _returnvalue_2
        (:`Is Valid`
          (if Add
            (`/Game/ParallelBeam/UltimateMapSystem/BPs/Components/BP_MapTracker.AddMapZone` _returnvalue_2 self)
            (else
              (`/Game/ParallelBeam/UltimateMapSystem/BPs/Components/BP_MapTracker.RemoveMapZone` _returnvalue_2 self))))))))

(event `Capture`
  ;[0.1927 0.1927 0.1927] UsedToCaptureTheDifferent layers of map, can be used in editor to create textures for ur map and then place them in the Material
  ; OR can be used to capture texture at runtime once or whenever environment changing events happen
  (for _array_element (`self.MapData`)
    (bind (_scenecapture _captureactorsoftag) (break `/Game/ParallelBeam/UltimateMapSystem/Data/S_MapCaptureLayers` _array_element))
    (bind _capturecomponent2d (`SceneCapture2D.CaptureComponent2D` _scenecapture))
    (set `SceneCaptureComponent2D.OrthoWidth` (`self.Ortho Width`) _capturecomponent2d)
    (`self.K2_SetActorLocation` _scenecapture (`self.K2_GetActorLocation`) false false)
    (`SceneCaptureComponent.ClearShowOnlyComponents` _capturecomponent2d)
    (for _array_element_2 _captureactorsoftag
      (bind _outactors (`GameplayStatics.GetAllActorsWithTag` _array_element_2))
      (for _array_element_3 _outactors
        (`SceneCaptureComponent.ShowOnlyActorComponents` _capturecomponent2d _array_element_3 true)))
    (`SceneCaptureComponent2D.CaptureScene` (`SceneCapture2D.CaptureComponent2D` _scenecapture))))

(fn `GetMapLayer`
  (params (Tag :type Name))
  (returns (Value :type "/Game/ParallelBeam/UltimateMapSystem/Data/S_MapLayerData Structure"))
  (return (`BlueprintMapLibrary.Map_Find` (`self.MapLayers`) Tag)))

(fn `UpdateAdditionalLayer`
  (params (Add :type Boolean) (MarkerComponent :type "/Game/ParallelBeam/UltimateMapSystem/BPs/Components/BP_MapMarker Object Reference (by ref)"))
  (bind _additionallayers (`self.AdditionalLayers`))
  (`/Engine/EditorBlueprintResources/StandardMacros.IsValid` MarkerComponent
    (:`Is Valid`
      (if Add
        (`KismetArrayLibrary.Array_AddUnique` _additionallayers MarkerComponent)
        (else
          (`KismetArrayLibrary.Array_RemoveItem` _additionallayers MarkerComponent)))
      (`self.AdditionalLayerUpdated`))))

(fn `UserConstructionScript`
  (`KismetArrayLibrary.Array_Set` (`self.Tags`) 0 (`self.MapTag`) true))