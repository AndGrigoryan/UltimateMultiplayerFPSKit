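; BP_MapTracker is a player controller component that tracks the active map zone and feeds minimap material parameters.
; For the local controller, Tick writes pawn location and control yaw into MPC_Minimap.
; Possession changes sphere-trace for an overlapping BP_MapManager to register the pawn.
; The most recently added zone becomes current, setting capture location and ortho width, broadcasting map updates and relaying its layer changes.
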(event `self.ReceiveTick`
  (params (DeltaSeconds :type "Float (single-precision)"))
  (bind _returnvalue (`Controller.K2_GetPawn` (`self.OwnerController`)))
  (bind (_returnvalue_roll _returnvalue_pitch _returnvalue_yaw) (`KismetMathLibrary.BreakRotator` (`Pawn.GetControlRotation` _returnvalue)))
  (`/Engine/EditorBlueprintResources/StandardMacros.IsValid` _returnvalue
    (:`Is Valid`
      (`KismetMaterialLibrary.SetVectorParameterValue` "/Game/ParallelBeam/UltimateMapSystem/Material/MasterMaterial/MPC_Minimap.MPC_Minimap" "PlayerLocation" (`KismetMathLibrary.Conv_VectorToLinearColor` (`Actor.K2_GetActorLocation` _returnvalue)))
      (`KismetMaterialLibrary.SetScalarParameterValue` "/Game/ParallelBeam/UltimateMapSystem/Material/MasterMaterial/MPC_Minimap.MPC_Minimap" "PlayerRotation" (`KismetMathLibrary.MapRangeClamped` _returnvalue_yaw 0.0 360.0 1.0)))))

(event `self.ReceiveBeginPlay`
  (bind _asplayer_controller (cast `PlayerController` (`self.GetOwner`)))
  (bind _output_get (set `self.OwnerController` _asplayer_controller))
  (`self.SetComponentTickEnabled` (`Controller.IsLocalPlayerController` _output_get))
  (add `Controller.OnPossessedPawnChanged` _output_get (delegate `OnPossessedPawnChanged_Event`)))

(event `OnPossessedPawnChanged_Event`
  (params (OldPawn :type "Pawn Object Reference") (NewPawn :type "Pawn Object Reference"))
  (bind _returnvalue (`Actor.K2_GetActorLocation` NewPawn))
  (`/Engine/EditorBlueprintResources/StandardMacros.IsValid` NewPawn
    (:`Is Valid`
      (bind _outhit (`KismetSystemLibrary.SphereTraceSingleForObjects` _returnvalue _returnvalue 50.0 (`|MakeArray` "ObjectTypeQuery8" :!type "EObjectTypeQuery Enum") false (`|MakeArray` NewPawn null :!type "Actor Object Reference")))
      (bind _asbp_map_manager (cast `/Game/ParallelBeam/UltimateMapSystem/BPs/BP_MapManager` (`.HitActor` (`GameplayStatics.BreakHitResult` _outhit))))
      (`/Game/ParallelBeam/UltimateMapSystem/BPs/BP_MapManager.AddMapToTracker` _asbp_map_manager true NewPawn))))

(event `AddMapZone`
  (params (MapManager :type "/Game/ParallelBeam/UltimateMapSystem/BPs/BP_MapManager Object Reference (by ref)"))
  (bind _selfmapzones (`self.SelfMapZones`))
  (if (`KismetArrayLibrary.Array_Contains` _selfmapzones MapManager)
    ;[1 1 1] just making sure that the most recent map always is the last entry even if it already exists
    (`KismetArrayLibrary.Array_RemoveItem` _selfmapzones MapManager))
  (`KismetArrayLibrary.Array_Add` _selfmapzones MapManager)
  (`self.SetNewMap`))

(event `RemoveMapZone`
  (params (MapManager :type "/Game/ParallelBeam/UltimateMapSystem/BPs/BP_MapManager Object Reference (by ref)"))
  (`KismetArrayLibrary.Array_RemoveItem` (`self.SelfMapZones`) MapManager)
  (`self.SetNewMap`))

(fn `AdditionalLayerUpdated`
  (`self.AdditionalLayersUpdated`))

(fn `SetNewMap`
  (bind _selfmapzones (`self.SelfMapZones`))
  (bind _output (`|GetArrayItem` _selfmapzones (`KismetArrayLibrary.Array_LastIndex` _selfmapzones)))
  (if (!= _output (`self.CurrentMapZone`))
    (bind _currentmapzone (`self.CurrentMapZone`)
      (:`then`
        (clear `/Game/ParallelBeam/UltimateMapSystem/BPs/BP_MapManager.AdditionalLayerUpdated` _currentmapzone))
      (:`else`
        _))
    (bind _output_get (set `self.CurrentMapZone` _output))
    (`/Engine/EditorBlueprintResources/StandardMacros.IsValid` _output_get
      (:`Is Valid`
        (`self.UpdateMap`)
        (`KismetMaterialLibrary.SetScalarParameterValue` "/Game/ParallelBeam/UltimateMapSystem/Material/MasterMaterial/MPC_Minimap.MPC_Minimap" "CaptureOrthoWidth" (`/Game/ParallelBeam/UltimateMapSystem/BPs/BP_MapManager.Ortho Width` _output_get))
        (`KismetMaterialLibrary.SetVectorParameterValue` "/Game/ParallelBeam/UltimateMapSystem/Material/MasterMaterial/MPC_Minimap.MPC_Minimap" "CaptureLocation" (`KismetMathLibrary.Conv_VectorToLinearColor` (`Actor.K2_GetActorLocation` _output_get)))
        (add `/Game/ParallelBeam/UltimateMapSystem/BPs/BP_MapManager.AdditionalLayerUpdated` (`self.CurrentMapZone`) (`|CreateDelegate` :!event `AdditionalLayerUpdated`))))))