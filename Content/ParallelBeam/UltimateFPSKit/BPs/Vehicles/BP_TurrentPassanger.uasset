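; BP_TurrentPassanger is a vehicle turret passenger pawn that lets its controller look around and fire projectiles.
; Look input is scaled into controller yaw and pitch, then passed on through BPPawnPossesion's look rotation update.
; Primary action input drives BPMSKProjectileLauncher, which takes the pawn as owner at BeginPlay.
; The construction script attaches the camera to the skeletal mesh's turret socket.
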(event `EnhancedInput|/Game/ParallelBeam/Core/Inputs/GroundVehicle/Actions/IA_PrimaryAction_Vehicle`
  (params (ActionValue :type Boolean) (ElapsedSeconds :type "Float (double-precision)") (TriggeredSeconds :type "Float (double-precision)") (InputAction :type "InputAction Object Reference" :default "/Game/ParallelBeam/Core/Inputs/GroundVehicle/Actions/IA_PrimaryAction_Vehicle.IA_PrimaryAction_Vehicle"))
  (:`Triggered`
    (`/Game/ParallelBeam/Core/BPs/Components/BP_MSK_ProjectileLauncher.AttemptFire` (`self.BP_MSK_ProjectileLauncher`) ActionValue)))

(event `self.ReceiveBeginPlay`
  (`parent.ReceiveBeginPlay`)
  (set `/Game/ParallelBeam/Core/BPs/Components/BP_MSK_ProjectileLauncher.OwnerPawn` self (`self.BP_MSK_ProjectileLauncher`)))

(event `EnhancedInput|/Game/ParallelBeam/Core/Inputs/GroundVehicle/Actions/IA_LookAround`
  (params (ActionValue :type "Vector2D Structure") (ElapsedSeconds :type "Float (double-precision)") (TriggeredSeconds :type "Float (double-precision)") (InputAction :type "InputAction Object Reference" :default "/Game/ParallelBeam/Core/Inputs/GroundVehicle/Actions/IA_LookAround.IA_LookAround"))
  (bind (_x _y) (`KismetMathLibrary.BreakVector2D` (* ActionValue (`self.InputScaleLookAround`))))
  (:`Triggered`
    (`self.AddControllerYawInput` _x)
    (`self.AddControllerPitchInput` _y)
    (`/Game/ParallelBeam/Core/BPs/Components/BP_PawnPossesion.SetLookRotation` (`self.BP_PawnPossesion`))))

(fn `UserConstructionScript`
  (`parent.UserConstructionScript`)
  (`SceneComponent.K2_AttachToComponent` (`self.Camera`) (`self.SkeletalMesh`) "Turrent_001" "KeepRelative" "SnapToTarget" "KeepWorld" true))