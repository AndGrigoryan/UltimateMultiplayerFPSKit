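; M4 rear iron sight attachment item that also supplies the matching front sight and places it on the weapon's barrel.
; The construction script adds the front sight as a static mesh component.
; While equipped, it listens to inventory equipment slot updates and runs the handler once on equip.
; The handler snaps the front sight to the Ironsight_Socket on the item in the Barrel slot, if one exists.
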(event `self.BP_Attachment_Item.OnItemEquipped`
  (params (InventoryComponent :type "AGR_InventoryComponent Object Reference") (EquipmentSlot :type "GameplayTag Structure (by ref)"))
  (add `AGR_InventoryComponent.OnEquipmentSlotUpdated` InventoryComponent (delegate `OnEquipmentSlotUpdated`))
  (`self.OnEquipmentSlotUpdated` null))

(event `OnEquipmentSlotUpdated`
  (params (Item :type "Actor Object Reference") (SlotAction :type "EAGR_EquipmentSlotAction Enum" :default "Set") (Slot :type "GameplayTag Structure (by ref)"))
  (bind _returnvalue (`AGR_InventoryComponent.GetItemInSlot` (stale `self.BP_Attachment_Item.OnItemEquipped` InventoryComponent) (struct :`TagName` "WepAttach.Barrel")))
  (`/Engine/EditorBlueprintResources/StandardMacros.IsValid` _returnvalue
    (:`Is Valid`
      (`SceneComponent.K2_AttachToComponent` (`self.FrontSight`) (`self.GetComponentByClass` _returnvalue "/Script/Engine.PrimitiveComponent") "Ironsight_Socket" "SnapToTarget" "SnapToTarget" "SnapToTarget" true))))

(event `self.BP_Attachment_Item.OnItemUnequipped`
  (params (InventoryComponent :type "AGR_InventoryComponent Object Reference") (EquipmentSlot :type "GameplayTag Structure (by ref)"))
  (remove `AGR_InventoryComponent.OnEquipmentSlotUpdated` InventoryComponent (delegate `OnEquipmentSlotUpdated`)))

(fn `UserConstructionScript`
  (`parent.UserConstructionScript`)
  (bind _returnvalue (`AddComponent|NODE_AddStaticMeshComponent-0`))
  (set `self.FrontSight` _returnvalue))