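; M-19 slide attachment Blueprint from UltimateFPSKit, supplying the aiming and sway data for that weapon part.
; GetScopeInfo returns a uniform per-enum camera FOV map, a weapon FOV, and scope ring, blur and sensitivity values with no offset or blur.
; GetSwaySettings returns an SSway struct with all multipliers, stiffness and damping at one.
; It has no active event logic, and its construction script only calls the parent.
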(fn `GetScopeInfo`
  (returns (CameraFOV :type "Map of /Game/ParallelBeam/Core/BPs/Data/Enum/E_CameraType Enum to Float (double-precision)") (WeaponFOV :type "Float (double-precision)") (ScopeRingOffset :type "Float (double-precision)") (BlurAmmount :type "Float (double-precision)") (Sensetivity :type "Float (double-precision)"))
  (return (`|MakeMap` "NewEnumerator0" 80.0 "NewEnumerator1" 80.0 "NewEnumerator2" 80.0 :!type "/Game/ParallelBeam/Core/BPs/Data/Enum/E_CameraType Enum") 100.0 0.0 0.0 1.0))

(fn `GetSwaySettings`
  (returns (Sway :type "/Game/ParallelBeam/Core/BPs/Data/Structures/S_Sway Structure"))
  (return (make `/Game/ParallelBeam/Core/BPs/Data/Structures/S_Sway` 0.0 0.0 (1.0 1.0 1.0) (1.0 1.0 1.0) 1.0 1.0 1.0 1.0)))

(fn `UserConstructionScript`
  (`parent.UserConstructionScript`))