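; Stun status effect built as an AGR inventory item that can be picked up but not dropped, used, equipped, unequipped or destroyed through inventory checks.
; Pickup or a stack-count update switches the effect on and restarts a retriggerable delay, after which it switches off and the item expires shortly after.
; A CLT event uses a timeline to blend the Stun parameter in MPC_LocalEffects, and destruction also clears it.
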(event `self.AGR_Item.OnStackCountUpdated`
  (params (OldStackCount :type Integer64) (NewStackCount :type Integer64))
  (`self.StunStatus`))

(event `self.AGR_Item.OnItemPickedUp`
  (params (InventoryComponent :type "AGR_InventoryComponent Object Reference"))
  (set `self.Inventory Component` InventoryComponent)
  (`self.StunStatus`))

(event `StunStatus`
  (`self.CLT_AddWorldEffect` true)
  (`KismetSystemLibrary.RetriggerableDelay` 4.0)
  (`self.CLT_AddWorldEffect` false)
  (`self.SetLifeSpan` 1.0))

(event `CLT_AddWorldEffect`
  (params (Add :type Boolean))
  (bind _returnvalue (`KismetMaterialLibrary.GetScalarParameterValue` "/Game/ParallelBeam/Core/Materials/Functions/MPC_LocalEffects.MPC_LocalEffects" "Stun"))
  (bind (_direction _newtrack_0) (`Timeline|Timeline` :!via `PlayFromStart`)
    (:`Update`
      (`KismetMaterialLibrary.SetScalarParameterValue` "/Game/ParallelBeam/Core/Materials/Functions/MPC_LocalEffects.MPC_LocalEffects" "Stun" (`KismetMathLibrary.Lerp` _returnvalue (`KismetMathLibrary.Conv_BoolToDouble` Add) _newtrack_0)))))

(event `self.ReceiveDestroyed`
  (`self.CLT_AddWorldEffect` false))

(fn `CanItemBeDestroyed`
  (params (InventoryComponent :type "AGR_InventoryComponent Object Reference"))
  (returns (ReturnValue :type Boolean))
  (return false))

(fn `CanItemBeDropped`
  (params (InventoryComponent :type "AGR_InventoryComponent Object Reference"))
  (returns (ReturnValue :type Boolean))
  (return false))

(fn `CanItemBeEquipped`
  (params (InventoryComponent :type "AGR_InventoryComponent Object Reference") (Slot :type "GameplayTag Structure"))
  (returns (ReturnValue :type Boolean))
  (return false))

(fn `CanItemBePickedUp`
  (params (InventoryComponent :type "AGR_InventoryComponent Object Reference"))
  (returns (ReturnValue :type Boolean))
  (return true))

(fn `CanItemBeUnequipped`
  (params (InventoryComponent :type "AGR_InventoryComponent Object Reference") (Slot :type "GameplayTag Structure"))
  (returns (ReturnValue :type Boolean))
  (return false))

(fn `CanItemBeUsed`
  (params (InventoryComponent :type "AGR_InventoryComponent Object Reference") (ActionType :type "GameplayTag Structure"))
  (returns (ReturnValue :type Boolean))
  (return false))

(fn `UserConstructionScript`)