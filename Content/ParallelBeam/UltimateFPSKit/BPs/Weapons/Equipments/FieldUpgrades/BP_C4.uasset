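; BP_C4 is a thrown C4 equipment projectile that sticks to the surface it hits.
; On projectile bounce it attaches to the hit component and bone, keeping world transform, then destroys its projectile and rotating movement components to stop motion.
; It then orients itself from the impact normal with a 90-degree offset and snaps to the impact point.
; No detonation or damage logic is present in these graphs.
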(event `self.ProjectileMovement.OnProjectileBounce`
  (params (ImpactResult :type "HitResult Structure (by ref)") (ImpactVelocity :type "Vector Structure (by ref)"))
  (bind (_bblockinghit _binitialoverlap _time _distance _location _impactpoint _normal _impactnormal _physmat _hitactor _hitcomponent _hitbonename _bonename) (`GameplayStatics.BreakHitResult` ImpactResult))
  (`self.K2_AttachToComponent` _hitcomponent _bonename "KeepWorld" "KeepWorld" "KeepWorld")
  (`ActorComponent.K2_DestroyComponent` (`self.ProjectileMovement`))
  (`ActorComponent.K2_DestroyComponent` (`self.RotatingMovement`))
  (`self.K2_SetActorRotation` (`KismetMathLibrary.ComposeRotators` (`KismetMathLibrary.MakeRotator` (.yaw (`KismetMathLibrary.Conv_VectorToRotator` _impactnormal)) (.pitch (`KismetMathLibrary.Conv_VectorToRotator` _impactnormal)) (.roll (`KismetMathLibrary.Conv_VectorToRotator` _impactnormal))) (struct :`Pitch` -90.0)) true)
  (`self.K2_SetActorLocation` _impactpoint))

(fn `UserConstructionScript`
  (`parent.UserConstructionScript`))