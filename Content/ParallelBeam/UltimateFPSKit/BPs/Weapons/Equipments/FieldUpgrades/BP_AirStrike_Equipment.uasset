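; Air strike field upgrade equipment that lets the player aim a target area and spawn the strike there.
; While interacting, Tick traces from the player's viewpoint and moves a ground decal to the hit point, hiding it below the world on a miss.
; SpawnItem spawns the configured equipment actor at the last valid hit, resets CurrentTime and stops ticking.
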(event `self.ReceiveTick`
  (params (DeltaSeconds :type "Float (single-precision)"))
  (bind (_location _rotation) (`Controller.GetPlayerViewPoint` (`self.GetInstigatorController`)))
  (bind _returnvalue (`KismetMathLibrary.GetForwardVector` _rotation))
  (bind _outhit (`KismetSystemLibrary.LineTraceSingleForObjects` (+ _location (* _returnvalue 50.0)) (+ _location (* _returnvalue 10000.0)) (`|MakeArray` "ObjectTypeQuery1" "ObjectTypeQuery2" :!type "EObjectTypeQuery Enum")))
  (bind (_bblockinghit _binitialoverlap _time _distance _location_2) (`GameplayStatics.BreakHitResult` _outhit))
  (if _bblockinghit
    (bind _decal (`self.Decal`)
      (:`then`
        (`SceneComponent.K2_SetWorldLocation` _decal (+ _location_2 (0.0 0.0 5.0)) false false))
      (:`else`
        _))
    (set `self.SpawnLocaation` _location_2)
    (set `self.CanSpawn` true)
    (else
      (bind _decal_2 (`self.Decal`)
        (:`then`
          (`SceneComponent.K2_SetWorldLocation` _decal_2 (0.0 0.0 -5000.0) false false))
        (:`else`
          _))
      (set `self.CanSpawn` false))))

(event `self.SVR_Interact`
  (params (Action :type "GameplayTag Structure"))
  (`parent.SVR_Interact` Action)
  (`self.SetActorTickEnabled` true))

(event `self.Interact`
  (params (Trigger :type Boolean))
  (`parent.Interact` Trigger)
  (`self.SetActorTickEnabled` Trigger)
  (if Trigger
    (bind _returnvalue (`GameplayStatics.SpawnDecalAtLocation` "/Game/ParallelBeam/Core/Materials/MasterMaterials/M_AirStrikeArea_Inst.M_AirStrikeArea_Inst" (10.0 200.0 200.0)))
    (set `self.Decal` _returnvalue)
    (else
      (`ActorComponent.K2_DestroyComponent` (`self.Decal`)))))

(event `self.SpawnItem`
  (params (Action :type "GameplayTag Structure"))
  (if (`self.CanSpawn`)
    (set `self.CurrentTime` 0.0)
    (`|SpawnActorFromClass` (`self.EquipmentToSpawn`) (`KismetMathLibrary.MakeTransform` (`self.SpawnLocaation`)) "AlwaysSpawn" "MultiplyWithRoot" self (`self.GetInstigator`))
    (`self.SetActorTickEnabled` false)
    (else
      (`self.SetActorTickEnabled` false))))

(fn `UserConstructionScript`
  (`parent.UserConstructionScript`))