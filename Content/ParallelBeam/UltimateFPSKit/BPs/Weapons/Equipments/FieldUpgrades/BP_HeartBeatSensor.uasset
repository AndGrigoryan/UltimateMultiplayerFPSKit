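; Heartbeat sensor field-upgrade equipment that shows nearby pawns on a render-target radar while in use.
; Interacting starts a looping two-second timer that animates a material-collection pulse, then sphere-traces around the owner to cache pawn locations.
; Tick draws those locations as world-axis blips relative to the owner and publishes the first hit's distance as ClosestEnemy, without sorting.
; SpawnItem spawns the configured equipment and stops ticking.
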(event `self.SVR_Interact`
  (params (Action :type "GameplayTag Structure"))
  (`parent.SVR_Interact` Action))

(event `self.SpawnItem`
  (params (Action :type "GameplayTag Structure"))
  (set `self.CurrentTime` 0.0)
  (`|SpawnActorFromClass` (`self.EquipmentToSpawn`) (`KismetMathLibrary.MakeTransform` (0.0 0.0 0.0)) "AlwaysSpawn" "MultiplyWithRoot" (`self.GetInstigatorController`) (`self.GetInstigator`))
  (`self.SetActorTickEnabled` false))

(event `self.Interact`
  (params (Trigger :type Boolean))
  (`parent.Interact` Trigger)
  (if Trigger
    (bind _returnvalue (`KismetSystemLibrary.K2_SetTimerDelegate` (delegate `CaptureEnemys`) 2.0 true))
    (`self.CaptureEnemys`)
    (`self.SetActorTickEnabled` true)
    (else
      (`KismetSystemLibrary.K2_ClearAndInvalidateTimerHandle` _returnvalue)
      (`self.SetActorTickEnabled` false))))

(event `CaptureEnemys`
  (bind _returnvalue (`self.GetOwner`))
  (bind _returnvalue_2 (`self.K2_GetActorLocation` _returnvalue))
  (bind (_direction _pulse) (`Timeline|PulseProgress` :!via `PlayFromStart`)
    (:`Update`
      (`KismetMaterialLibrary.SetScalarParameterValue` "/Game/ParallelBeam/UltimateFPSKit/Material/MaterialCollection/MPC_UltimateFPSKit.MPC_UltimateFPSKit" "PulseProgress" _pulse))
    (:`Finished`
      (`KismetArrayLibrary.Array_Clear` (`self.EnemyLocations`))
      (bind _outhits (`KismetSystemLibrary.SphereTraceMultiForObjects` _returnvalue_2 _returnvalue_2 1000.0 (`|MakeArray` "ObjectTypeQuery3" :!type "EObjectTypeQuery Enum") false (`|MakeArray` _returnvalue)))
      (for _array_element _outhits
        (`KismetArrayLibrary.Array_Add` (`self.EnemyLocations`) (`self.K2_GetActorLocation` (`.HitActor` (`GameplayStatics.BreakHitResult` _array_element))))))))

(event `self.ReceiveTick`
  (params (DeltaSeconds :type "Float (single-precision)"))
  (`KismetRenderingLibrary.ClearRenderTarget2D` "/Game/ParallelBeam/UltimateFPSKit/Texture/RT_HeartBeatSensor.RT_HeartBeatSensor")
  (bind (_canvas _size _context) (`KismetRenderingLibrary.BeginDrawCanvasToRenderTarget` "/Game/ParallelBeam/UltimateFPSKit/Texture/RT_HeartBeatSensor.RT_HeartBeatSensor"))
  (for (_array_element _array_index) (`self.EnemyLocations`)
    (bind (_x _y) (`KismetMathLibrary.BreakVector2D` _size))
    (`Canvas.K2_DrawMaterial` _canvas "/Game/ParallelBeam/Core/Materials/MasterMaterials/M_EnemyLocation.M_EnemyLocation" (+ (`KismetMathLibrary.MakeVector2D` (`KismetMathLibrary.MapRangeUnclamped` (.x (- _array_element (`self.K2_GetActorLocation` (`self.GetOwner`)))) 0.0 2500.0 0.0 _x) (`KismetMathLibrary.MapRangeUnclamped` (.y (- _array_element (`self.K2_GetActorLocation` (`self.GetOwner`)))) 0.0 2500.0 0.0 _y)) (/ _size (2.0 2.0))) (50.0 50.0) (0.0 0.0) (1.0 1.0) 0.0 (1.0 1.0))
    (if (== _array_index 0)
      (`KismetMaterialLibrary.SetScalarParameterValue` "/Game/ParallelBeam/UltimateFPSKit/Material/MaterialCollection/MPC_UltimateFPSKit.MPC_UltimateFPSKit" "ClosestEnemy" (/ (`KismetMathLibrary.Abs` (`KismetMathLibrary.Vector_Distance` _array_element (`self.K2_GetActorLocation` (`self.GetOwner`)))) 100.0))))
  (`KismetRenderingLibrary.EndDrawCanvasToRenderTarget` _context)
  (if (`KismetArrayLibrary.Array_IsEmpty` (`self.EnemyLocations`))
    (`KismetMaterialLibrary.SetScalarParameterValue` "/Game/ParallelBeam/UltimateFPSKit/Material/MaterialCollection/MPC_UltimateFPSKit.MPC_UltimateFPSKit" "ClosestEnemy")))

(fn `UserConstructionScript`
  (`parent.UserConstructionScript`))