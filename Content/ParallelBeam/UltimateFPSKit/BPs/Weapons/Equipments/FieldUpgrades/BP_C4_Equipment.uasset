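; C4 field-upgrade equipment that throws explosive charges on a short press and detonates them on a longer hold.
; Interact times the press with a looping timer; throws require a completed recharge, while detonation skips that check.
; It updates the UsingEquipment state, stops weapon actions, plays the Fire or FireEmpty montage and calls SVRInteract.
; SpawnItem spawns and tracks charges on Fire, then explodes and clears them all on FireEmpty.
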(event `StartIntractTimer`
  (set `self.IntractTime` (+ (`self.IntractTime`) 0.1)))

(event `self.Interact`
  (params (Trigger :type Boolean))
  (bind _return_value (`/Game/ParallelBeam/Core/BPs/FunctionLib/BFL_MSK.GetMSKCharacterInventory` (`self.GetOwner`)))
  (bind _returnvalue (`KismetSystemLibrary.MakeLiteralBool` (< (`self.IntractTime`) 0.2)))
  (bind _returnvalue_2 (select `bool` _returnvalue :`false` (struct :`TagName` "Actions.FireEmpty") :`true` (struct :`TagName` "Actions.Fire") :!type "GameplayTag Structure"))
  ;[0 0 0] On interaction add the tag to action states And stop primary and secondary actions and play the throw montages
  (if Trigger
    (bind _returnvalue_3 (`KismetSystemLibrary.K2_SetTimerDelegate` (delegate `StartIntractTimer`) 0.1 true))
    (else
      (`KismetSystemLibrary.K2_ClearAndInvalidateTimerHandle` _returnvalue_3)
      (if _returnvalue
        (if (>= (`self.CurrentTime`) (`self.RechargeTime`))
          (bind _blocked (`/Game/ParallelBeam/Core/BPs/Components/BP_MSK_CharacterInventory.Change Action State` _return_value (struct :`TagName` "States.UsingEquipment") true :!label _label))
          (if _blocked
            (set `self.IntractTime` 0.0)
            (else
              (`/Game/ParallelBeam/Core/BPs/Components/BP_MSK_CharacterInventory.PrimaryAction` _return_value false)
              (`/Game/ParallelBeam/Core/BPs/Components/BP_MSK_CharacterInventory.SecondaryAction` _return_value false)
              (`/Game/ParallelBeam/Core/BPs/Components/BP_MSK_Montage.PlayMontage` (`/Game/ParallelBeam/Core/BPs/FunctionLib/BFL_MSK.GetMSK_MontageComponent` (`self.GetOwner`)) true false self _returnvalue_2)
              (`self.SVR_Interact` _returnvalue_2)
              (set `self.IntractTime` 0.0)))
          (else
            (set `self.IntractTime` 0.0)))
        (else
          (goto _label))))))

(event `self.SpawnItem`
  (params (Action :type "GameplayTag Structure"))
  (`|SwitchGameplayTag` Action
    (:`Actions.Fire`
      (bind _returnvalue (`|SpawnActorFromClass` (`self.EquipmentToSpawn`) (`SceneComponent.K2_GetComponentToWorld` (`self.SpawnLocation`)) "AlwaysSpawn" "MultiplyWithRoot" (`self.GetInstigatorController`) (`self.GetInstigator`)))
      (bind _asbp_explosive (cast `/Game/ParallelBeam/Core/BPs/Actors/Misc/BP_Explosive` _returnvalue))
      (`KismetArrayLibrary.Array_Add` (`self.C4s`) _asbp_explosive))
    (:`Actions.FireEmpty`
      (`/Game/ParallelBeam/Core/BPs/Actors/Misc/BP_Explosive.Explode` (`self.C4s`))
      (`KismetArrayLibrary.Array_Clear` (`self.C4s`)))))

(fn `UserConstructionScript`
  (`parent.UserConstructionScript`))