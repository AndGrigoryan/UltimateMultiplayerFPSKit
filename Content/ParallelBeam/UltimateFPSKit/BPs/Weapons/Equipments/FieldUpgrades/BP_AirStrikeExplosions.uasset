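; BP_AirStrikeExplosions is an explosive actor for an air strike field upgrade that animates a projectile mesh vertically before detonating.
; On BeginPlay, a timeline drives the mesh's relative Z height, then calls Explode when it finishes.
; The MLTEffect override runs the parent effect and adds a world camera shake at the actor's location, with radii scaled from the damage outer radius.
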(event `self.ReceiveBeginPlay`
  (bind (_direction _newtrack_0) (`Timeline|MoveMesh`)
    (:`Update`
      (`SceneComponent.K2_SetRelativeLocation` (`self.StaticMesh1`) (`KismetMathLibrary.MakeVector` 0.0 0.0 (* _newtrack_0 6000.0)) false false))
    (:`Finished`
      (`self.Explode`))))

(event `self.MLT_Effect`
  (bind _damage_outer_radius (`self.Damage Outer Radius`))
  (`parent.MLT_Effect`)
  (`GameplayStatics.PlayWorldCameraShake` "/Game/ParallelBeam/UltimateFPSKit/BPs/Data/Shakes/CS_ExplosionShake.CS_ExplosionShake_C" (`self.K2_GetActorLocation`) _damage_outer_radius (* _damage_outer_radius 4.0) 1.0 true))

(fn `UserConstructionScript`)