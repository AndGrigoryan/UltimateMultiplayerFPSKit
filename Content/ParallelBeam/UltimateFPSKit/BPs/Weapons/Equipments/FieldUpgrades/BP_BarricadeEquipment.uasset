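; Field upgrade equipment that deploys a barricade on the ground just in front of its owner.
; SpawnItem traces downward from a point ahead of the owner against WorldStatic objects to find a surface.
; On a hit it zeroes CurrentTime and spawns EquipmentToSpawn there with the owner's rotation, passing on controller and instigator.
; A DoOnce gate is reset after spawning, or after a short retriggerable delay on a miss.
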(event `self.SpawnItem`
  (params (Action :type "GameplayTag Structure"))
  (bind _returnvalue (`self.GetOwner`))
  (bind _returnvalue_2 (+ (`self.K2_GetActorLocation` _returnvalue) (* (`self.GetActorForwardVector` _returnvalue) 50.0)))
  (bind _outhit (`KismetSystemLibrary.LineTraceSingleForObjects` _returnvalue_2 (+ _returnvalue_2 (0.0 0.0 -200.0)) (`|MakeArray` "ObjectTypeQuery1" :!type "EObjectTypeQuery Enum") :!label _label))
  (bind (_bblockinghit _binitialoverlap _time _distance _location) (`GameplayStatics.BreakHitResult` _outhit))
  (if _bblockinghit
    (set `self.CurrentTime` 0.0)
    (`|SpawnActorFromClass` (`self.EquipmentToSpawn`) (`KismetMathLibrary.MakeTransform` _location (`self.K2_GetActorRotation` _returnvalue)) "AlwaysSpawn" "MultiplyWithRoot" (`self.GetInstigatorController`) (`self.GetInstigator`))
    (`/Engine/EditorBlueprintResources/StandardMacros.DoOnce` false :!via `Reset` :!label _label_2
      (:`Completed`
        (goto _label)))
    (else
      (`KismetSystemLibrary.RetriggerableDelay` 0.2)
      (goto _label_2 :!via `Reset`))))

(fn `UserConstructionScript`
  (`parent.UserConstructionScript`))