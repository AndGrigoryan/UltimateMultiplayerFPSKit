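; BP_AirStrikePoint is an air strike field upgrade actor that bombards the area around its location.
; On BeginPlay, a DoN loop spawns twelve BP_AirStrikeExplosions one second apart, passing on its owner and instigator.
; Each spawn location comes from a downward WorldStatic line trace at a random horizontal offset within 1000 units per axis.
; The actor destroys itself once the final explosion spawns.
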(event `self.ReceiveBeginPlay`
  (bind _returnvalue (`self.GetOwner`))
  (bind _returnvalue_2 (+ (`self.K2_GetActorLocation`) (`KismetMathLibrary.MakeVector` (`KismetMathLibrary.RandomFloatInRange` -1000.0 1000.0) (`KismetMathLibrary.RandomFloatInRange` -1000.0 1000.0) 2000.0)))
  (bind _counter (`/Engine/EditorBlueprintResources/StandardMacros.Do N` 12 :!label _label)
    (:`Exit`
      (`|ExecutionSequence`
        (:`then_0`
          (bind _outhit (`KismetSystemLibrary.LineTraceSingleForObjects` _returnvalue_2 (+ _returnvalue_2 (0.0 0.0 -3000.0)) (`|MakeArray` "ObjectTypeQuery1" :!type "EObjectTypeQuery Enum")))
          (`|SpawnActorFromClass` "/Game/ParallelBeam/UltimateFPSKit/BPs/Weapons/Equipments/FieldUpgrades/BP_AirStrikeExplosions.BP_AirStrikeExplosions_C" (`KismetMathLibrary.MakeTransform` (`.Location` (`GameplayStatics.BreakHitResult` _outhit))) "Undefined" "MultiplyWithRoot" _returnvalue (`self.GetInstigator` _returnvalue))
          (`KismetSystemLibrary.Delay` 1.0)
          (goto _label))
        (:`then_1`
          (if (>= _counter 12)
            (`self.K2_DestroyActor`)))))))

(fn `UserConstructionScript`)