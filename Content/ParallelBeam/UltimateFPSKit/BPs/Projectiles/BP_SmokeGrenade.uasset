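; Smoke grenade projectile that releases a Niagara smoke cloud when it explodes.
; Explode calls ApplyEffect, which attaches pooled NS_Smoke to the Sphere, resets its world rotation and stops projectile rotation following velocity.
; Explode then sets a short lifespan so the actor removes itself.
; An unconnected branch holds an alternative smoke volume built from a scaled sphere mesh with a volumetric fog material.
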(event `self.Explode`
  (`self.ApplyEffect` (0.0 0.0 0.0))
  (`self.SetLifeSpan` 10.0))

(event `self.ApplyEffect`
  (params (Location :type "Vector Structure"))
  (bind _returnvalue (`NiagaraFunctionLibrary.SpawnSystemAttached` "/Game/ParallelBeam/Core/VFX/NS_Smoke.NS_Smoke" (`self.Sphere`) "None" (0.0 0.0 0.0) (struct) "SnapToTargetIncludingScale" true true "AutoRelease"))
  (`SceneComponent.K2_SetWorldRotation` :`self` _returnvalue)
  (set `ProjectileMovementComponent.bRotationFollowsVelocity` false (`self.ProjectileMovement`)))

(fn `UserConstructionScript`
  (`parent.UserConstructionScript`))