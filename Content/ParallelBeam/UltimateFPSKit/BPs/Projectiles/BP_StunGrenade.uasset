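; BP_StunGrenade is a grenade projectile that stuns pawns caught in its blast radius.
; On Explode, a multi sphere trace gathers Pawn-type objects within DamageRadius of the grenade.
; Each hit pawn receives a stack of BP_StunItem through its inventory component, so the stun is delivered as an inventory item.
; The grenade then applies its effect at its location and destroys itself.
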(event `self.Explode`
  (bind _returnvalue (`self.K2_GetActorLocation`))
  (bind _outhits (`KismetSystemLibrary.SphereTraceMultiForObjects` _returnvalue _returnvalue (`self.Damage Radius`) (`|MakeArray` "ObjectTypeQuery3" :!type "EObjectTypeQuery Enum")))
  (for _array_element _outhits
    (bind _aspawn (cast `Pawn` (`.HitActor` (`GameplayStatics.BreakHitResult` _array_element))))
    (`AGR_InventoryComponent.AddStacks` (`AGR_InventoryFunctionLibrary.GetInventoryComponent` _aspawn) "/Game/ParallelBeam/UltimateFPSKit/BPs/Weapons/Equipments/BP_StunItem.BP_StunItem_C" 1))
  (`self.ApplyEffect` _returnvalue)
  (`self.K2_DestroyActor`))

(fn `UserConstructionScript`
  (`parent.UserConstructionScript`))