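; Armor modifier item that raises its owner's maximum health while carried, built on the MSK item pickup and drop events.
; On pickup, it adds a fraction of max health taken from the first modifier's float value, caches that bonus and fills current health to the new maximum.
; On drop, it subtracts the cached bonus and also sets current health to the restored maximum.
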(event `self.BP_MSK_Item.OnItemPickedUp`
  (params (InventoryComponent :type "AGR_InventoryComponent Object Reference"))
  (bind _return_value (`/Game/ParallelBeam/Core/BPs/FunctionLib/BFL_MSK.Get MSKHealth Component` (`ActorComponent.GetOwner` InventoryComponent)))
  (bind _maxhealth (`/Game/ParallelBeam/Core/BPs/Components/BP_HealthComponent.MaxHealth` _return_value))
  (bind _returnvalue (* _maxhealth (`.FloatValue_10_FE2B848F4014206A67501FA637D3A062` (break `/Game/ParallelBeam/Core/BPs/Data/Structures/S_GameplayTag_Value` (`|GetArrayItem` (`self.Modifiers`))))))
  (set `self.HealthIncreaseBy` _returnvalue)
  (bind _output_get (set `/Game/ParallelBeam/Core/BPs/Components/BP_HealthComponent.MaxHealth` (+ _returnvalue _maxhealth) _return_value))
  (set `/Game/ParallelBeam/Core/BPs/Components/BP_HealthComponent.CurrentHealth` _output_get _return_value))

(event `self.BP_MSK_Item.OnItemDropped`
  (params (InventoryComponent :type "AGR_InventoryComponent Object Reference") (DropLocation :type "Vector Structure (by ref)"))
  (bind _return_value (`/Game/ParallelBeam/Core/BPs/FunctionLib/BFL_MSK.Get MSKHealth Component` (`ActorComponent.GetOwner` InventoryComponent)))
  (bind _output_get (set `/Game/ParallelBeam/Core/BPs/Components/BP_HealthComponent.MaxHealth` (- (`/Game/ParallelBeam/Core/BPs/Components/BP_HealthComponent.MaxHealth` _return_value) (`self.HealthIncreaseBy`)) _return_value))
  (set `/Game/ParallelBeam/Core/BPs/Components/BP_HealthComponent.CurrentHealth` _output_get _return_value))

(fn `UserConstructionScript`
  (`parent.UserConstructionScript`))