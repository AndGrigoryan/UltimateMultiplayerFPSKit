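; Interactable ladder actor that characters climb through the MSK locomotion component.
; Interacting calls enter-ladder on that component, and overlapping the bottom hit box calls exit-ladder.
; Overlapping the top hit box while climbing sets a "LadderTop" motion warping target at the exit location, then plays the get-off montage, flagged self-only when not on the server.
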(event `self.BottomHitBox.OnComponentBeginOverlap`
  (params (OverlappedComponent :type "PrimitiveComponent Object Reference") (OtherActor :type "Actor Object Reference") (OtherComp :type "PrimitiveComponent Object Reference") (OtherBodyIndex :type Integer) (bFromSweep :type Boolean) (SweepResult :type "HitResult Structure (by ref)"))
  (`/Game/ParallelBeam/Core/BPs/Components/BP_MSK_Locomotion.CLTExitLadder` (`/Game/ParallelBeam/Core/BPs/FunctionLib/BFL_MSK.GetMSKLocomotionComponent` OtherActor)))

(event `self.TopHitBox.OnComponentBeginOverlap`
  (params (OverlappedComponent :type "PrimitiveComponent Object Reference") (OtherActor :type "Actor Object Reference") (OtherComp :type "PrimitiveComponent Object Reference") (OtherBodyIndex :type Integer) (bFromSweep :type Boolean) (SweepResult :type "HitResult Structure (by ref)"))
  (bind _return_value (`/Game/ParallelBeam/Core/BPs/FunctionLib/BFL_MSK.GetMSKLocomotionComponent` OtherActor))
  (if (`/Game/ParallelBeam/Core/BPs/Components/BP_MSK_Locomotion.IsUsingLadder` _return_value)
    (`MotionWarpingComponent.AddOrUpdateWarpTargetFromLocationAndRotation` :`self` (`self.GetComponentByClass` (`/Game/ParallelBeam/Core/BPs/Components/BP_MSK_Locomotion.As Character` _return_value) "/Script/MotionWarping.MotionWarpingComponent") :`WarpTargetName` "LadderTop" :`TargetLocation` (`SceneComponent.K2_GetComponentLocation` (`self.ExitLocation`)))
    (`/Game/ParallelBeam/Core/BPs/Components/BP_MSK_Montage.PlayMontage` (`/Game/ParallelBeam/Core/BPs/FunctionLib/BFL_MSK.GetMSK_MontageComponent` OtherActor) (not (`KismetSystemLibrary.IsServer`)) false null (struct :`TagName` "Actions.Ladder.GetOff"))))

(fn `CanGetIcon`
  (returns (ReturnValue :type Boolean))
  (return false))

(fn `CanInteract`
  (params (Actor :type "Actor Object Reference"))
  (returns (`Return Value` :type Boolean))
  (return true))

(fn `GetIcon`
  (params (Stock :type Boolean))
  (returns (Texture :type "Texture Object Reference"))
  (return null))

(fn `GetInteractionInfo`
  (params (InteractingActor :type "Actor Object Reference"))
  (returns (Item :type Text) (Type :type Text) (HoldType :type Text))
  (return "LADDER" "USE" ""))

(fn `StartInteract`
  (params (Character :type "Character Object Reference"))
  (returns (`Return Value` :type Boolean))
  (`/Game/ParallelBeam/Core/BPs/Components/BP_MSK_Locomotion.CLTEnterLadder` (`/Game/ParallelBeam/Core/BPs/FunctionLib/BFL_MSK.GetMSKLocomotionComponent` Character) self)
  (return true))

(fn `UserConstructionScript`)