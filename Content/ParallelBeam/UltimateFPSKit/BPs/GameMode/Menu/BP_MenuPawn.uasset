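; BP_MenuPawn is the pawn for the FPS kit's main menu, putting the menu on screen when play begins.
; BeginPlay shows the mouse cursor, adds WB_MainMenu to the viewport and sets Game and UI input focused on that widget.
; Disconnected leftover nodes would snap the pawn to a PlayerStart and rotate a BP_Master_Weapon with clamped mouse input, but neither runs, and Mouse2D is empty.
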(event `self.ReceiveBeginPlay`
  (bind _returnvalue (`GameplayStatics.GetPlayerController` 0))
  (set `PlayerController.bShowMouseCursor` true _returnvalue)
  (bind _returnvalue_2 (`|CreateWidget` "/Game/ParallelBeam/Core/Widgets/Menu/WB_MainMenu.WB_MainMenu_C"))
  (`UserWidget.AddToViewport` _returnvalue_2 0)
  (set `self.HUD` null)
  (`WidgetBlueprintLibrary.SetInputMode_GameAndUIEx` _returnvalue _returnvalue_2 "DoNotLock" true true))

(event `InputVectorAxis|Mouse2D`
  (params (AxisValue :type "Vector Structure")))

(fn `UserConstructionScript`)