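; Death match game mode for the Ultimate FPS Kit that turns kills into team score.
; It extends the parent AddKill event, calling it first and then comparing the team indices from the killer's and victim's player state components.
; When the teams differ, it looks up the killer's team component by index and adds one point, so same-team kills earn nothing.
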(event `/Game/ParallelBeam/Core/BPs/Interfaces/BPI_Gamemode.AddKill`
  (params (Killer :type "Controller Object Reference") (Killed :type "Controller Object Reference") (DamageCauser :type "Actor Object Reference"))
  (bind _teamindex (`/Game/ParallelBeam/Core/BPs/Components/GameModeComponents/BP_PlayerState_PS_Component.TeamIndex` (`/Game/ParallelBeam/Core/BPs/FunctionLib/BFL_MSK.GetPlayerStateComponent` (`Controller.PlayerState` Killer))))
  (`parent.AddKill` Killer Killed DamageCauser)
  (if (!= _teamindex (`/Game/ParallelBeam/Core/BPs/Components/GameModeComponents/BP_PlayerState_PS_Component.TeamIndex` (`/Game/ParallelBeam/Core/BPs/FunctionLib/BFL_MSK.GetPlayerStateComponent` (`Controller.PlayerState` Killed))))
    (`/Game/ParallelBeam/Core/BPs/Components/GameModeComponents/BP_GameStateTeam_Component.AddScore` (`BlueprintMapLibrary.Map_Find` (`self.TeamComponents`) _teamindex) 1)))

(fn `UserConstructionScript`
  (`parent.UserConstructionScript`))