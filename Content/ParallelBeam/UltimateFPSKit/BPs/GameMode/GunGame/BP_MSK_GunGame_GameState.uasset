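; Game state for a team-based Gun Game mode that upgrades each team's primary weapon as its score rises.
; On BeginPlay the authority shuffles available guns into a random progression and starts both teams on the first.
; Team score updates check kill thresholds, change that team's gun and re-equip its players.
; Possession changes, bound only for the first team component's players, also equip the current gun, spawned far below the world with matching ammo.
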(event `self.ReceiveBeginPlay`
  (bind _output (`|GetArrayItem` (`self.GunsProgression`)))
  (`/Engine/EditorBlueprintResources/ActorMacros.Switch Has Authority`
    (:`Authority`
      (`|ExecutionSequence`
        (:`then_0`
          (if (not (== (`KismetArrayLibrary.Array_Length` (`self.GunsProgression`)) (`KismetArrayLibrary.Array_Length` (`self.AvalibleGuns`)))) :!label _label
            (`KismetArrayLibrary.Array_AddUnique` (`self.GunsProgression`) (`KismetArrayLibrary.Array_Random` (`self.AvalibleGuns`)))
            (goto _label)))
        (:`then_1`
          (set `self.TeamProgressWithGuns` (`|MakeArray` _output _output)))))))

(event `self.BP_GameStateTeam_Component.TeamScoreUpdated`
  (`self.CheckIfTeamCanGetBetterGun` (`self.BP_GameStateTeam_Component`)))

(event `self.BP_GameStateTeam_Component1.TeamScoreUpdated`
  (`self.CheckIfTeamCanGetBetterGun` (`self.BP_GameStateTeam_Component1`)))

(event `UpdateGunsForAllClients`
  (params (Team :type "/Game/ParallelBeam/Core/BPs/Components/GameModeComponents/BP_GameStateTeam_Component Object Reference"))
  (for _array_element (`/Game/ParallelBeam/Core/BPs/Components/GameModeComponents/BP_GameStateTeam_Component.TeamPlayers` Team)
    (`self.EquipWeaponTOPlayer` (`PlayerState.GetPawn` _array_element))))

(event `self.BP_GameStateTeam_Component.TeamPlayerAdded`
  (params (PlayerState :type "PlayerState Object Reference"))
  (add `Controller.OnPossessedPawnChanged` (`PlayerState.GetPlayerController` PlayerState) (delegate `OnPossessedPawnChanged_Event`)))

(event `OnPossessedPawnChanged_Event`
  (params (OldPawn :type "Pawn Object Reference") (NewPawn :type "Pawn Object Reference"))
  (`self.EquipWeaponTOPlayer` NewPawn))

(fn `CheckIfTeamCanGetBetterGun`
  (params (Team :type "/Game/ParallelBeam/Core/BPs/Components/GameModeComponents/BP_GameStateTeam_Component Object Reference"))
  (bind _gunprogresskills (`self.GunProgressKills`))
  (bind _teamprogresswithguns (`self.TeamProgressWithGuns`))
  (bind _teamindex (`/Game/ParallelBeam/Core/BPs/Components/GameModeComponents/BP_GameStateTeam_Component.TeamIndex` Team))
  (for (_array_element _array_index) _gunprogresskills
    (if (< _array_element (`/Game/ParallelBeam/Core/BPs/Components/GameModeComponents/BP_GameStateTeam_Component.TeamScore` Team))
      (if (`KismetArrayLibrary.Array_IsValidIndex` (`self.GunProgressKills`) (- _array_index 1))
        (bind _output (`|GetArrayItem` (`self.GunsProgression`) (`|GetArrayItem` _gunprogresskills _array_index)))
        (if (!= (`|GetArrayItem` _teamprogresswithguns _teamindex) _output)
          (`KismetArrayLibrary.Array_Set` _teamprogresswithguns _teamindex _output true)
          (`self.UpdateGunsForAllClients` (`local.Team`))
          (`KismetSystemLibrary.PrintString` "TRUE ")
          (else
            (`KismetSystemLibrary.PrintString` "False")))))))

(fn `EquipWeaponTOPlayer`
  (params (Pawn :type "Pawn Object Reference"))
  (bind _returnvalue (`AGR_InventoryFunctionLibrary.GetInventoryComponent` Pawn))
  (bind _returnvalue_2 (`KismetMathLibrary.MakeTransform` (0.0 0.0 -1000000.0)))
  (bind _output (`|GetArrayItem` (`self.TeamProgressWithGuns`) (`/Game/ParallelBeam/Core/BPs/Components/GameModeComponents/BP_PlayerState_PS_Component.TeamIndex` (`/Game/ParallelBeam/Core/BPs/FunctionLib/BFL_MSK.GetPlayerStateComponent` (`Pawn.PlayerState` Pawn)))))
  (`/Engine/EditorBlueprintResources/StandardMacros.IsValid` Pawn
    (:`Is Valid`
      (if (not (== (`GameplayStatics.GetObjectClass` (`AGR_InventoryComponent.GetItemInSlot` _returnvalue (struct :`TagName` "CharacterSlots.Primary"))) _output))
        (bind _returnvalue_3 (`|SpawnActorFromClass` _output _returnvalue_2 "Undefined" "MultiplyWithRoot" null null))
        (`|ExecutionSequence`
          (:`then_0`
            (bind _bp_msk_item (`/Game/ParallelBeam/Core/BPs/Actors/BP_MasterItem.BP_MSK_Item` _returnvalue_3))
            (`AGR_ItemComponent.PickUpItem` _bp_msk_item _returnvalue false true true)
            (`AGR_ItemComponent.EquipItem` _bp_msk_item _returnvalue (struct :`TagName` "CharacterSlots.Primary") true))
          (:`then_1`
            (bind _return_value (message `/Game/ParallelBeam/Core/BPs/Interfaces/BPI_Weapon.GetAmmoType` _returnvalue_3))
            (bind _returnvalue_4 (`|SpawnActorFromClass` _return_value _returnvalue_2 "Undefined" "MultiplyWithRoot" null null))
            (`AGR_ItemComponent.PickUpItem` (`/Game/ParallelBeam/Core/BPs/Actors/BP_MasterItem.BP_MSK_Item` _returnvalue_4) _returnvalue true true true)))))))

(fn `UserConstructionScript`
  (`parent.UserConstructionScript`))