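; King of the Hill capture zone that awards score to the team holding it.
; On overlap changes, the server finds the team with most living pawns; server timers move capture progress and award points, pausing on ties.
; Attackers must drain rival progress before capturing, and empty hills drift back to owned or neutral.
; CaptureStatus's RepNotify broadcasts updates and tints the minimap marker by ownership, with optional debug text.
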(event `RewardPoints`
  (bind _return_value (`/Game/ParallelBeam/Core/BPs/FunctionLib/BFL_MSK.Get GameStateTeamComponent` (`GameplayStatics.GetGameState`) (`self.CurrentOccuping Team`)))
  ;[0 0 0] Reward Points
  (if (`self.CanRewardPoints`)
    (`/Engine/EditorBlueprintResources/StandardMacros.IsValid` _return_value
      (:`Is Valid`
        (`/Game/ParallelBeam/Core/BPs/Components/GameModeComponents/BP_GameStateTeam_Component.AddScore` _return_value (`self.ScoreToAwardEveryUpdate`))))))

(event `self.ReceiveBeginPlay`
  (if (`self.Show Debug info`)
    (`self.SetActorTickEnabled` true)
    (else
      (`ActorComponent.K2_DestroyComponent` (`self.TextRender`))))
  (`/Engine/EditorBlueprintResources/ActorMacros.Switch Has Authority`
    (:`Authority`
      (`KismetSystemLibrary.K2_SetTimerDelegate` (delegate `StatusUpdate`) (`self.UpdateTime`) true)
      (`KismetSystemLibrary.K2_SetTimerDelegate` (delegate `RewardPoints`) (`self.RewardTimer`) true))))

(event `StatusUpdate`
  (bind _returnvalue (select `bool` (`self.HasAnyPlayer?`) :`false` (`self.CurrentOccuping Team`) :`true` (`self.AttackingTeam`)))
  (bind _returnvalue_2 (`KismetMathLibrary.FClamp` (+ (`self.CaptureStatus`) (`self.ProgressChangeEveryUpdate`))))
  ;[0 0 0] Checking which team should the oints go to and which can capture it
  ; complicated so read slowly
  (if (>= (`self.AttackingTeam`) 0)
    (if (or (== (`self.CurrentOccuping Team`) (`self.AttackingTeam`)) (== (`self.CurrentOccuping Team`) -1))
      (if (== (`self.TryingToOccupyTeam`) (`self.AttackingTeam`))
        (if (== (`self.CaptureStatus`) 1.0) :!label _label
          (set `self.CanRewardPoints` true :!label _label_2)
          (elif (== _returnvalue_2 1.0)
            (set `self.CurrentOccuping Team` _returnvalue)
            (set `self.TryingToOccupyTeam` _returnvalue)
            (set `self.CaptureStatus` _returnvalue_2)
            (goto _label_2)
            (else
              (set `self.TryingToOccupyTeam` _returnvalue)
              (set `self.CaptureStatus` _returnvalue_2)
              (set `self.CanRewardPoints` false))))
        (else
          (if (== (`self.CaptureStatus`) 0.0) :!label _label_3
            (if (== (`self.TryingToOccupyTeam`) (`self.AttackingTeam`))
              (set `self.CanRewardPoints` false)
              (else
                (set `self.CurrentOccuping Team` -1 :!label _label_4)
                (set `self.TryingToOccupyTeam` (`self.AttackingTeam`))
                (set `self.CanRewardPoints` false)))
            (else
              (bind _output_get (set `self.CaptureStatus` (`KismetMathLibrary.FClamp` (- (`self.CaptureStatus`) (`self.ProgressChangeEveryUpdate`)))))
              (if (== _output_get 0.0)
                (goto _label_4)
                (else
                  (set `self.CanRewardPoints` false)))))))
      (else
        (goto _label_3)))
    (elif (`self.HasAnyPlayer?`)
      (set `self.CanRewardPoints` false)
      (elif (!= (`self.CurrentOccuping Team`) -1)
        (goto _label)
        (else
          (goto _label_3))))))

(event `self.ReceiveActorBeginOverlap`
  (params (OtherActor :type "Actor Object Reference"))
  ;[0 0 0] On begin and end overlap recount the players
  (`/Engine/EditorBlueprintResources/ActorMacros.Switch Has Authority` :!label _label_5
    (:`Authority`
      (bind (_teamplayervalues _maxteamindex) (`self.CheckMajorityTeam`))
      (set `self.AttackingTeam` _maxteamindex))))

(event `self.ReceiveTick`
  (params (DeltaSeconds :type "Float (single-precision)"))
  (`TextRenderComponent.K2_SetText` (`self.TextRender`) (`|FormatText` "Attacking Team: {AttackingTeam} \nTrying to Occupy Team{trying team} \nOwned by : {Owning team} \nStatis: {Status}" (`self.AttackingTeam`) (`self.TryingToOccupyTeam`) (`self.CurrentOccuping Team`) (`self.CaptureStatus`))))

(event `self.ReceiveActorEndOverlap`
  (params (OtherActor :type "Actor Object Reference"))
  ;[0 0 0] On begin and end overlap recount the players
  (goto _label_5))

(fn `CheckMajorityTeam`
  (returns (TeamPlayerValues :type "Map of Integer to Integer") (MaxTeamIndex :type Integer))
  (locals (Loc_TeamPlayerValues :type "Map of Integer to Object Object Reference") (Loc_MaxPlayerTeamIndex :type Integer :default -1))
  (bind _loc_teamplayervalues (`local.Loc_TeamPlayerValues`))
  (bind _loc_teamplayervalues_2 (`local.Loc_TeamPlayerValues`))
  (bind _value (`BlueprintMapLibrary.Map_Find` _loc_teamplayervalues_2 (`local.Loc_MaxPlayerTeamIndex`)))
  (set `self.HasAnyPlayer?` false)
  (for _array_element (`self.GetOverlappingActors` "/Script/Engine.Pawn")
    (bind _aspawn (cast `Pawn` _array_element))
    (if (> (`/Game/ParallelBeam/Core/BPs/Components/BP_HealthComponent.CurrentHealth` (`/Game/ParallelBeam/Core/BPs/FunctionLib/BFL_MSK.Get MSKHealth Component` _aspawn)) 0.0)
      (bind _teamindex (`/Game/ParallelBeam/Core/BPs/Components/GameModeComponents/BP_PlayerState_PS_Component.TeamIndex` (`/Game/ParallelBeam/Core/BPs/FunctionLib/BFL_MSK.GetPlayerStateComponent` (`Pawn.PlayerState` _aspawn))))
      (`BlueprintMapLibrary.Map_Add` _loc_teamplayervalues _teamindex (+ (`BlueprintMapLibrary.Map_Find` _loc_teamplayervalues _teamindex) 1))
      (set `self.HasAnyPlayer?` true)))
  (bind _values (`BlueprintMapLibrary.Map_Values` _loc_teamplayervalues_2))
  (for (_array_element_2 _array_index) _values
    (bind _keys (`BlueprintMapLibrary.Map_Keys` (`local.Loc_TeamPlayerValues`)))
    (if (> _array_element_2 _value)
      (set `local.Loc_MaxPlayerTeamIndex` (`|GetArrayItem` _keys _array_index))
      (else
        ;[1 1 1] This just means there are multiple teams with same ammout of people so we should stop the timer
        (if (== _array_element_2 _value)
          (set `local.Loc_MaxPlayerTeamIndex` -1)
          (return (`local.Loc_TeamPlayerValues`) (`local.Loc_MaxPlayerTeamIndex`))))))
  (return (`local.Loc_TeamPlayerValues`) (`local.Loc_MaxPlayerTeamIndex`)))

(fn `OnRep_CaptureStatus`
  (bind _returnvalue (`GameplayStatics.GetPlayerController` 0))
  (bind _currentoccuping_team (`self.CurrentOccuping Team`))
  (bind _returnvalue_2 (`self.GetComponentByClass` _returnvalue "/Game/ParallelBeam/UltimateMapSystem/BPs/Components/BP_MapTracker.BP_MapTracker_C"))
  (bind (_value _returnvalue_3) (`BlueprintMapLibrary.Map_Find` (`/Game/ParallelBeam/UltimateMapSystem/BPs/Components/BP_MapTracker.AdditionalLayerWithActors` _returnvalue_2) (`self.BP_MapMarker`)))
  (bind (_r _g _b) (`KismetMathLibrary.BreakColor` (select `bool` (== _currentoccuping_team -1) :`false` (select `bool` (== _currentoccuping_team (`/Game/ParallelBeam/Core/BPs/Components/GameModeComponents/BP_PlayerState_PS_Component.TeamIndex` (`/Game/ParallelBeam/Core/BPs/FunctionLib/BFL_MSK.GetPlayerStateComponent` (`Controller.PlayerState` _returnvalue)))) :`false` (struct :`R` 0.590619 :`B` 0.041701 :`A` 1.0) :`true` (struct :`R` 0.205191 :`G` 1.0 :`B` 0.090808 :`A` 1.0) :!type "LinearColor Structure") :`true` (struct :`R` 1.0 :`G` 1.0 :`B` 1.0 :`A` 1.0))))
  (`self.StatusUpdated`)
  (`/Engine/EditorBlueprintResources/StandardMacros.IsValid` _returnvalue_2
    (:`Is Valid`
      (if _returnvalue_3
        (bind _returnvalue_4 (`Image.GetDynamicMaterial` _value))
        (`MaterialInstanceDynamic.SetVectorParameterValue` _returnvalue_4 "PlayerIcon" (`KismetMathLibrary.MakeColor` _r _g _b 0.3))))))

(fn `UserConstructionScript`)