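; Hide-and-seek game mode that assigns the hiding team, picks pawns by team and ends rounds on kills.
; Round updates store HidingTeam in the game state, flipping from team 0 to 1 at the side-switch round.
; As wired, that team gets the parent's default pawn and others get BP_MasterHidePawn.
; After a kill, if HidingTeam still has living players, the stat tracker's EndRound receives the opposite team.
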(event `self.ReceiveBeginPlay`
  (`parent.ReceiveBeginPlay`)
  (bind _asbp_msk_hide_and_seek_game_state (cast `/Game/ParallelBeam/UltimateFPSKit/BPs/GameMode/HideAndSeek/BP_MSK_HideAndSeek_GameState` (`GameplayStatics.GetGameState`)))
  (set `self.As BP MSK Hide And Seek Game State` _asbp_msk_hide_and_seek_game_state)
  (`self.OnRoundUpdated`))

(event `/Game/ParallelBeam/Core/BPs/Interfaces/BPI_Gamemode.ScoreUpdated`
  (params (TeamComponent :type "/Game/ParallelBeam/Core/BPs/Components/GameModeComponents/BP_GameStateTeam_Component Object Reference")))

(event `self.AddKill`
  (params (Killer :type "Controller Object Reference") (Killed :type "Controller Object Reference") (DamageCauser :type "Actor Object Reference"))
  (bind _returnvalue (`GameplayStatics.GetGameState`))
  (bind _hidingteam (`/Game/ParallelBeam/UltimateFPSKit/BPs/GameMode/HideAndSeek/BP_MSK_HideAndSeek_GameState.HidingTeam` (`self.As BP MSK Hide And Seek Game State`)))
  (`parent.AddKill` Killer Killed DamageCauser)
  (if (`/Game/ParallelBeam/Core/BPs/Components/GameModeComponents/BP_GameStateTeam_Component.DoesTeamHaveAnyPlayerAlive` (`/Game/ParallelBeam/Core/BPs/FunctionLib/BFL_MSK.Get GameStateTeamComponent` _returnvalue _hidingteam))
    (`/Game/ParallelBeam/Core/BPs/Components/GameModeComponents/BP_GameStateTracker.EndRound` (`/Game/ParallelBeam/Core/BPs/FunctionLib/BFL_MSK.GetGameStatTracker` _returnvalue) (select `int` _hidingteam :`0` 1 :`1` 0))))

(event `self.OnRoundUpdated`
  (bind _gamestattracker (`self.GameStatTracker`))
  (set `/Game/ParallelBeam/UltimateFPSKit/BPs/GameMode/HideAndSeek/BP_MSK_HideAndSeek_GameState.HidingTeam` (`KismetMathLibrary.Conv_BoolToInt` (>= (`/Game/ParallelBeam/Core/BPs/Components/GameModeComponents/BP_GameStateTracker.CurrentRound` _gamestattracker) (`/Game/ParallelBeam/Core/BPs/Components/GameModeComponents/BP_GameStateTracker.NumberOfRoundsToSwitchSides` _gamestattracker))) (`self.As BP MSK Hide And Seek Game State`)))

(fn `GetDefaultPawnClassForController`
  (params (InController :type "Controller Object Reference"))
  (returns (ReturnValue :type "Object Class Reference"))
  (bind _returnvalue (`parent.GetDefaultPawnClassForController` InController))
  (if (== (`/Game/ParallelBeam/Core/BPs/Components/GameModeComponents/BP_PlayerState_PS_Component.TeamIndex` (`/Game/ParallelBeam/Core/BPs/FunctionLib/BFL_MSK.GetPlayerStateComponent` (`Controller.PlayerState` InController))) (`/Game/ParallelBeam/UltimateFPSKit/BPs/GameMode/HideAndSeek/BP_MSK_HideAndSeek_GameState.HidingTeam` (`self.As BP MSK Hide And Seek Game State`)))
    (return _returnvalue)
    (else
      (return "/Game/ParallelBeam/UltimateFPSKit/BPs/GameMode/HideAndSeek/HidePawns/BP_MasterHidePawn.BP_MasterHidePawn_C"))))

(fn `UserConstructionScript`
  (`parent.UserConstructionScript`))